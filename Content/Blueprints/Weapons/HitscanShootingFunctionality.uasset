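; Hitscan shooting logic for weapons, firing one or more camera-based line traces per shot with random spread around the max-range endpoint.
; Each trace spawns a bullet tracer, and hits send server events to deal damage and multicast surface-based impact effects and decals.
; The server accumulates damage, headshot and kill per shot, polling by timer until all bullets register before showing UI hit feedback.
; InflictEffects is an empty hook.
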(event Custom|Server_DealDamage
  (params (Target :type Object%20Object%20Reference) (ShotData :type Shot%20Data%20Structure))
  (bind (_damagecaused _died _headshot) (Class|DestructibleBPI|GetShot(Message) Target ShotData))
  (Protected|AddtoCurrentShotStats _damagecaused _headshot _died)
  (Protected|InflictEffects Target _damagecaused _died _headshot))

(event Custom|Server_ShowHitEffects
  (params (Hit :type Hit%20Result%20Structure))
  ;[0 0 0] Shooting Impact visual effects
  (CallFunction|MulticastShowHitEffects Hit))

(event Custom|Multicast_ShowHitEffects
  (params (Hit :type Hit%20Result%20Structure))
  (bind (_bblockinghit _binitialoverlap _time _distance _location _impactpoint _normal _impactnormal _physmat) (Collision|BreakHitResult Hit))
  (bind (_bblockinghit_2 _binitialoverlap_2 _time_2 _distance_2 _location_2 _impactpoint_2 _normal_2 _impactnormal_2 _physmat_2) (Collision|BreakHitResult Hit))
  ;[0 0 0] Shooting Impact visual effects
  (Niagara|SpawnSystematLocation (Utilities|Select :Index (Variables|/Script/PhysicsCore.PhysicalMaterial|GetSurfaceType _physmat) :SurfaceType_Default "/Game/Assets/ParticleSystems/ShootingFeedback/DefaultShootingFeedback.DefaultShootingFeedback" :SurfaceType1 "/Game/Assets/ParticleSystems/ShootingFeedback/FleshShootingFeedback.FleshShootingFeedback") _location (Math|Rotator|MakeRotfromZ _normal))
  (switch Utilities|FlowControl|Switch|SwitchonEPhysicalSurface (Variables|/Script/PhysicsCore.PhysicalMaterial|GetSurfaceType _physmat_2)
    (:SurfaceType_Default
      (bind _returnvalue (Rendering|Decal|SpawnDecalatLocation "/Game/Assets/Materials/Decals/BulletHoleDecal/BulletHoleDecal.BulletHoleDecal" "5.000000,5.000000,5.000000" _location_2 (Math|Conversions|RotationFromXVector _impactnormal_2) 12.0))
      (Rendering|Components|Decal|SetFadeScreenSize _returnvalue 0.0))))

(event Custom|Server_FeedbackShotStats
  ;[0 0 0] Orders to display the results of the current shot in the UI
  (if (>= (Variables|Default|GetBulletsProcessed) (Variables|Default|GetBulletsPerShot))
    (Variables|Default|SetBulletsProcessed 0)
    (if (> (Variables|CurrentShotStats|GetCurrentDamage) 0.0)
      (Default|DisplayHitFeedback (Variables|/Game/Blueprints/Player/BaseCharacter_BP.BaseCharacter_BP_C|GetPlayerControllerReference (Variables|Default|GetOwningCharacter)) (Variables|CurrentShotStats|GetCurrentDamage) (Variables|CurrentShotStats|GetCurrentHeadshot) (Variables|CurrentShotStats|GetCurrentKill))
      (Protected|ResetCurrentShotStats))
    (else
      (Utilities|Time|SetTimerbyEvent (delegate Custom|Server_FeedbackShotStats) 0.01))))

(event Custom|Server_SpawnBulletTracer
  (params (TargetPoint :type Vector))
  (Protected|SpawnBulletTracer TargetPoint))

(event Custom|Client_PlayFirstPersonMuzzleFlash
  (Niagara|SpawnSystematLocation (Variables|Default|GetMuzzleFlash) (Variables|Default|GetMuzzleLocation)))

(event EventBeginPlay
  (Variables|Default|SetCurrentBulletSpread (Variables|Default|GetUnscopedBulletSpread)))

(fn SetUpHitscan
  (params (Character :type Base%20Character%20BP%20Object%20Reference))
  (Variables|Default|SetOwningCharacter Character))

(fn ShootHitscan
  (params (MuzzleLocation :type Vector))
  (Variables|Default|SetMuzzleLocation MuzzleLocation)
  (Protected|PlayMuzzleFlash)
  (for _index (range 1 (Variables|Default|GetBulletsPerShot))
    (Protected|FireSingleShot))
  (CallFunction|ServerFeedbackShotStats))

(fn FireSingleShot
  (bind (_start _end) (Protected|FindHitscanPoints))
  (bind (_outhit _returnvalue) (Collision|LineTraceByChannel _start _end "TraceTypeQuery2" false 0 "None"))
  (if _returnvalue
    (Protected|SpawnBulletTracer (.ImpactPoint (Collision|BreakHitResult _outhit)))
    (CallFunction|ServerDealDamage (.HitActor (Collision|BreakHitResult _outhit)) (Utilities|Struct|MakeShotData (Variables|Default|GetDamageValue) (Variables|Default|GetHeadshotMultiplier) (.HitBoneName (Collision|BreakHitResult _outhit)) (Utilities|Struct|MakeDamageInstigator false (Default|GetPlayerControllerReference (Variables|Default|GetOwningCharacter)))))
    (CallFunction|ServerShowHitEffects _outhit)
    (else
      (Protected|SpawnBulletTracer _end))))

(fn FindHitscanPoints
  (bind _maxrange (Variables|Default|GetMaxRange))
  (bind _owningcharacter (Variables|Default|GetOwningCharacter))
  (bind _camera (Variables|/Game/Blueprints/Player/BaseCharacter_BP.BaseCharacter_BP_C|GetCamera _owningcharacter))
  (bind _returnvalue (Transformation|GetWorldLocation _camera))
  (bind _returnvalue_2 (Math|Vector|GetForwardVector _camera))
  (bind _returnvalue_3 (* _returnvalue_2 _maxrange))
  (bind _returnvalue_4 (+ _returnvalue _returnvalue_3))
  (bind (_x _y _z) (Math|Vector|BreakVector _returnvalue_4))
  (return _returnvalue (Math|Vector|MakeVector (+ _x (Math|Random|RandomFloatinRange (* (Variables|Default|GetCurrentBulletSpread) -1.0) (Variables|Default|GetCurrentBulletSpread))) (+ _y (Math|Random|RandomFloatinRange (* (Variables|Default|GetCurrentBulletSpread) -1.0) (Variables|Default|GetCurrentBulletSpread))) (+ _z (Math|Random|RandomFloatinRange (* (Variables|Default|GetCurrentBulletSpread) -1.0) (Variables|Default|GetCurrentBulletSpread))))))

(fn AddtoCurrentShotStats
  (params (Damage :type Float%20%28double-precision%29) (Headshot :type Boolean) (Kill :type Boolean))
  (Variables|CurrentShotStats|SetCurrentDamage (+ (Variables|CurrentShotStats|GetCurrentDamage) Damage))
  (if Headshot
    (Variables|CurrentShotStats|SetCurrentHeadshot true))
  (if Kill
    (Variables|CurrentShotStats|SetCurrentKill true))
  (Math|Integer|IncrementInt (Variables|Default|GetBulletsProcessed)))

(fn ResetCurrentShotStats
  (Variables|CurrentShotStats|SetCurrentDamage 0.0)
  (Variables|CurrentShotStats|SetCurrentHeadshot false)
  (Variables|CurrentShotStats|SetCurrentKill false))

(fn InflictEffects
  (params (Target :type Object%20Object%20Reference) (DamageDone :type Float%20%28double-precision%29) (KillDone :type Boolean) (Headshot :type Boolean)))

(fn SpawnBulletTracer
  (params (TargetPoint :type Vector))
  (bind _muzzlelocation (Variables|Default|GetMuzzleLocation))
  (Game|SpawnActorfromClass "/Game/Blueprints/Visuals/Effects/BaseBulletTracer.BaseBulletTracer_C" (Math|Transform|MakeTransform _muzzlelocation (Math|Rotator|FindLookatRotation _muzzlelocation TargetPoint) "1.000000,1.000000,1.000000") "AlwaysSpawn" 0 (- TargetPoint _muzzlelocation) (Variables|Default|GetOwningCharacter)))

(fn PlayMuzzleFlash
  (CallFunction|ClientPlayFirstPersonMuzzleFlash))