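; Blueprint interface that defines the common contract for weapons.
; It declares calls to start and stop attacking, reload or cancel reloading, and reset recoil.
; Getters expose max and current ammunition, a walking modifier and the weapon model class.
; Further functions spawn, delete, show and hide the weapon model, with most action calls returning a boolean.
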(fn StartAttacking
  (return false))

(fn StopAttacking
  (return false))

(fn Reload
  (return false))

(fn CancelReloading
  (return false))

(fn GetMaxAmmunition
  (return 0))

(fn GetCurrentAmmunition
  (return 0))

(fn GetWalkingModifier
  (return 0.0))

(fn ResetRecoil)

(fn HideWeaponModel
  (return false))

(fn ShowWeaponModel
  (return false))

(fn SpawnWeaponModel
  (params (WeaponModel :type Base%20Weapon%20Model%20BP%20Class%20Reference))
  (return false))

(fn DeleteWeaponModel
  (return false))

(fn GetWeaponModelClass
  (return 0))