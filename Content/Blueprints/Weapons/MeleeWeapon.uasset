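; Melee weapon that attacks with a cooldown-gated capsule trace from the owner's camera out to its max range.
; A hit sends server calls that apply damage, show hit feedback to the attacker and call an empty InflictEffects hook.
; The attack sound is replicated, and impact effects are multicast, with the Niagara system chosen by surface type.
; Ammo and reload functions are stubs, and model handling defers to the parent class.
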(event Custom|Multicast_ShotHitEffects
  (params (Hit :type Hit%20Result%20Structure))
  (bind (_bblockinghit _binitialoverlap _time _distance _location _impactpoint _normal _impactnormal _physmat) (Collision|BreakHitResult Hit))
  (Niagara|SpawnSystematLocation (Utilities|Select :Index (Variables|/Script/PhysicsCore.PhysicalMaterial|GetSurfaceType _physmat) :SurfaceType_Default "/Game/Assets/ParticleSystems/ShootingFeedback/DefaultShootingFeedback.DefaultShootingFeedback" :SurfaceType1 "/Game/Assets/ParticleSystems/ShootingFeedback/FleshShootingFeedback.FleshShootingFeedback") _location (Math|Rotator|MakeRotfromZ _normal)))

(event Custom|Server_DealDamage
  (params (Target :type Object%20Object%20Reference))
  (bind (_damagecaused _died) (Class|DestructibleBPI|TakeDamage(Message) Target (Variables|Default|GetDamageValue) (Utilities|Struct|MakeDamageInstigator false (Default|GetPlayerControllerReference (Variables|Default|GetOwningCharacter)))))
  (if (> _damagecaused 0.0)
    (Default|DisplayHitFeedback (Variables|/Game/Blueprints/Player/BaseCharacter_BP.BaseCharacter_BP_C|GetPlayerControllerReference (Variables|Default|GetOwningCharacter)) _damagecaused false _died))
  (Protected|InflictEffects Target _damagecaused _died))

(event Custom|Server_ShotHitEffects
  (params (Hit :type Hit%20Result%20Structure))
  (CallFunction|MulticastShotHitEffects Hit))

(event EventTick
  (params (DeltaSeconds :type Float%20%28single-precision%29))
  (Protected|UpdateCooldown DeltaSeconds))

(fn UpdateCooldown
  (params (DeltaTime :type Float%20%28double-precision%29))
  (if (>= (Variables|Default|GetCurrentCooldown) 0.0)
    (Variables|Default|SetCurrentCooldown (- (Variables|Default|GetCurrentCooldown) DeltaTime))))

(fn SetUpWeapon
  (params (OwningCharacter :type Base%20Character%20BP%20Object%20Reference) (WeaponModelClass :type Base%20Weapon%20Model%20BP%20Class%20Reference))
  (Variables|Default|SetOwningCharacter OwningCharacter)
  (CallFunction|SpawnWeaponModel WeaponModelClass)
  (CallFunction|HideWeaponModel))

(fn FindHitPoints
  (bind _owningcharacter (Variables|Default|GetOwningCharacter))
  (bind _camera (Variables|/Game/Blueprints/Player/BaseCharacter_BP.BaseCharacter_BP_C|GetCamera _owningcharacter))
  (bind _returnvalue (Transformation|GetWorldLocation _camera))
  (return _returnvalue (+ _returnvalue (* (Math|Vector|GetForwardVector _camera) (Variables|Default|GetMaxRange)))))

(fn InflictEffects
  (params (Target :type Object%20Object%20Reference) (DamageDone :type Float%20%28double-precision%29) (KillDone :type Boolean)))

(fn GetCurrentAmmunition
  (return 0))

(fn GetMaxAmmunition
  (return 0))

(fn CancelReloading
  (return false))

(fn Reload
  (return false))

(fn StartAttacking
  (bind _hitboxsize (Variables|Default|GetHitboxSize))
  (if (<= (Variables|Default|GetCurrentCooldown) 0.0)
    (Variables|Default|SetCurrentCooldown (Variables|Default|GetMaxCooldown))
    (CallFunction|ServerPlayReplicatedSound (Variables|Default|GetAttackSound) (.location (Transformation|GetActorTransform (Variables|Default|GetOwningCharacter))))
    (bind (_start _end) (Protected|FindHitPoints))
    (bind (_outhit _returnvalue) (Collision|CapsuleTraceByChannel _start _end _hitboxsize _hitboxsize "TraceTypeQuery2" false 0 "None"))
    (if _returnvalue
      (CallFunction|ServerDealDamage (.HitActor (Collision|BreakHitResult _outhit)))
      (CallFunction|ServerShotHitEffects _outhit)
      (return true))
    (else
      (return false))))

(fn StopAttacking
  (return false))

(fn HideWeaponModel
  (bind _visible (|CallParentFunction))
  (return _visible))

(fn ShowWeaponModel
  (bind _visible (|CallParentFunction))
  (return _visible))

(fn SpawnWeaponModel
  (params (WeaponModel :type Base%20Weapon%20Model%20BP%20Class%20Reference))
  (bind _spawned (|CallParentFunction WeaponModel))
  (return _spawned))

(fn DeleteWeaponModel
  (bind _deleted (|CallParentFunction))
  (return _deleted))