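; Base weapon Blueprint that manages a character's first- and third-person weapon models and replicated weapon sounds.
; Spawn, show, hide and delete calls drive an owner-only arms model through client events and an owner-hidden body model through server-to-multicast events.
; Both models attach to the right-hand weapon socket.
; Attack, reload and ammo functions are stubs returning false or zero, while walking modifier and model class have getters.
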(event Custom|Client_Show1stPersonWeaponModel
  ;[0 0 0] 1st Person Weapon Model Replication
  (Rendering|SetVisibility (Variables|/Game/Blueprints/Weapons/WeaponModelBlueprints/BaseWeaponModel_BP.BaseWeaponModel_BP_C|GetWeaponMesh (Variables|Default|Get1stPersonWeaponModel)) true false))

(event Custom|Client_Hide1stPersonWeaponModel
  ;[0 0 0] 1st Person Weapon Model Replication
  (Rendering|SetVisibility (Variables|/Game/Blueprints/Weapons/WeaponModelBlueprints/BaseWeaponModel_BP.BaseWeaponModel_BP_C|GetWeaponMesh (Variables|Default|Get1stPersonWeaponModel)) false false))

(event Custom|Server_PlayReplicatedSound
  (params (Sound :type Sound%20Cue%20Object%20Reference) (Location :type Vector))
  ;[0 0 0] Replicated Sounds
  (CallFunction|MulticastPlayReplicatedSound Sound Location))

(event Custom|Multicast_PlayReplicatedSound
  (params (Sound :type Sound%20Cue%20Object%20Reference) (Location :type Vector))
  ;[0 0 0] Replicated Sounds
  (Audio|PlaySoundatLocation Sound Location "0, 0, 0" 1.0 1.0 0.0 0 0 0 0))

(event Custom|Server_Hide3rdPersonWeaponModel
  ;[0 0 0] 3rd Person Weapon Model Replication
  (CallFunction|MulticastHide3rdPersonWeaponModel))

(event Custom|Multicast_Hide3rdPersonWeaponModel
  ;[0 0 0] 3rd Person Weapon Model Replication
  (Rendering|SetVisibility (Variables|/Game/Blueprints/Weapons/WeaponModelBlueprints/BaseWeaponModel_BP.BaseWeaponModel_BP_C|GetWeaponMesh (Variables|Default|Get3rdPersonWeaponModel)) false false))

(event Custom|Server_Show3rdPersonWeaponModel
  ;[0 0 0] 3rd Person Weapon Model Replication
  (CallFunction|MulticastShow3rdPersonWeaponModel))

(event Custom|Multicast_Show3rdPersonWeaponModel
  ;[0 0 0] 3rd Person Weapon Model Replication
  (Rendering|SetVisibility (Variables|/Game/Blueprints/Weapons/WeaponModelBlueprints/BaseWeaponModel_BP.BaseWeaponModel_BP_C|GetWeaponMesh (Variables|Default|Get3rdPersonWeaponModel)) true false))

(event Custom|Server_Spawn3rdPersonWeaponModel
  (params (WeaponModel :type Base%20Weapon%20Model%20BP%20Class%20Reference))
  ;[0 0 0] 3rd Person Weapon Model Replication
  (CallFunction|MulticastSpawn3rdPersonWeaponModel WeaponModel))

(event Custom|Multicast_Spawn3rdPersonWeaponModel
  (params (WeaponModel :type Base%20Weapon%20Model%20BP%20Class%20Reference))
  (bind _owningcharacter (Variables|Default|GetOwningCharacter))
  ;[0 0 0] 3rd Person Weapon Model Replication
  (bind _returnvalue (Game|SpawnActorfromClass WeaponModel (Transformation|GetSocketTransform (Variables|/Script/Engine.Character|GetMesh _owningcharacter) "hand_r_WeaponSocket" "RTS_World") "Undefined" _owningcharacter _owningcharacter))
  (Variables|Default|Set3rdPersonWeaponModel _returnvalue)
  (Class|PrimitiveComponent|SetOwnerNoSee (Variables|/Game/Blueprints/Weapons/WeaponModelBlueprints/BaseWeaponModel_BP.BaseWeaponModel_BP_C|GetWeaponMesh _returnvalue) true)
  (Transformation|AttachComponentToComponent _returnvalue (Variables|/Script/Engine.Character|GetMesh (Variables|Default|GetOwningCharacter)) "hand_r_WeaponSocket" "SnapToTarget" "SnapToTarget" "SnapToTarget" true))

(event Custom|Client_Delete1stPersonWeaponModel
  ;[0 0 0] 1st Person Weapon Model Replication
  (Actor|DestroyActor (Variables|Default|Get1stPersonWeaponModel)))

(event Custom|Server_Delete3rdPersonWeaponModel
  ;[0 0 0] 3rd Person Weapon Model Replication
  (CallFunction|MulticastDelete3rdPersonWeaponModel))

(event Custom|Multicast_Delete3rdPersonWeaponModel
  ;[0 0 0] 3rd Person Weapon Model Replication
  (Actor|DestroyActor (Variables|Default|Get3rdPersonWeaponModel)))

(event Custom|Client_Spawn1stPersonWeaponModel
  (params (WeaponModel :type Base%20Weapon%20Model%20BP%20Class%20Reference))
  (bind _owningcharacter (Variables|Default|GetOwningCharacter))
  ;[0 0 0] 1st Person Weapon Model Replication
  (bind _returnvalue (Game|SpawnActorfromClass WeaponModel (Transformation|GetSocketTransform (Variables|/Game/Blueprints/Player/BaseCharacter_BP.BaseCharacter_BP_C|GetArmsMesh _owningcharacter) "hand_r_WeaponSocket" "RTS_World") "Undefined" _owningcharacter _owningcharacter))
  (Variables|Default|Set1stPersonWeaponModel _returnvalue)
  (Rendering|SetOnlyOwnerSee (Variables|/Game/Blueprints/Weapons/WeaponModelBlueprints/BaseWeaponModel_BP.BaseWeaponModel_BP_C|GetWeaponMesh _returnvalue) true :!class /Script/Engine.PrimitiveComponent)
  (Transformation|AttachComponentToComponent _returnvalue (Variables|/Game/Blueprints/Player/BaseCharacter_BP.BaseCharacter_BP_C|GetArmsMesh (Variables|Default|GetOwningCharacter)) "hand_r_WeaponSocket" "SnapToTarget" "SnapToTarget" "SnapToTarget" true))

(fn CancelReloading
  (return false))

(fn DeleteWeaponModel
  (CallFunction|ClientDelete1stPersonWeaponModel)
  (CallFunction|ServerDelete3rdPersonWeaponModel)
  (return true))

(fn GetCurrentAmmunition
  (return 0))

(fn GetMaxAmmunition
  (return 0))

(fn GetWalkingModifier
  (return (Variables|Default|GetWalkingModifier)))

(fn GetWeaponModelClass
  (return (Variables|Default|GetWeaponModelClass)))

(fn HideWeaponModel
  (CallFunction|ClientHide1stPersonWeaponModel)
  (CallFunction|ServerHide3rdPersonWeaponModel)
  (return false))

(fn Reload
  (return false))

(fn ShowWeaponModel
  (CallFunction|ClientShow1stPersonWeaponModel)
  (CallFunction|ServerShow3rdPersonWeaponModel)
  (return true))

(fn SpawnWeaponModel
  (params (WeaponModel :type Base%20Weapon%20Model%20BP%20Class%20Reference))
  (bind _output_get (Variables|Default|SetWeaponModelClass WeaponModel))
  (CallFunction|ClientSpawn1stPersonWeaponModel _output_get)
  (CallFunction|ServerSpawn3rdPersonWeaponModel (Variables|Default|GetWeaponModelClass))
  (return true))

(fn StartAttacking
  (return false))

(fn StopAttacking
  (return false))