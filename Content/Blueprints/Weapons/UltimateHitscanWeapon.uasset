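; UltimateHitscanWeapon is a hitscan weapon Blueprint used by a character's ultimate ability, extending its parent's shoot and reload logic.
; Setup stores the owning character, shooting and ultimate references, then spawns the weapon model hidden.
; A reset function refills ammunition and clears cooldown, reload and attack state.
; Reloading works only when the weapon is reloadable; otherwise a successful shot that empties the ammunition ends the ultimate.
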(event EventResetRecoil
  (|CallParentFunction))

(event EventTick
  (params (DeltaSeconds :type Float%20%28single-precision%29))
  (|CallParentFunction DeltaSeconds) ; This node is disabled and will not be called.\nDrag off pins to build functionality.
)

(event EventBeginPlay
  (|CallParentFunction) ; This node is disabled and will not be called.\nDrag off pins to build functionality.
)

(fn Reload
  (if (Variables|Default|GetReloadable)
    (bind _isreloading (|CallParentFunction))
    (return _isreloading)
    (else
      (return false))))

(fn SetUpUltimateWeapon
  (params (OwningCharacter :type Base%20Character%20BP%20Object%20Reference) (HitscanShooting :type Hitscan%20Shooting%20Functionality%20Object%20Reference) (Ultimate :type Base%20Ultimate%20Object%20Reference) (WeaponModelClass :type Base%20Weapon%20Model%20BP%20Class%20Reference))
  (Variables|Default|SetOwningCharacter OwningCharacter)
  (Variables|Default|SetHitscanShooting HitscanShooting)
  (Variables|Default|SetUltimate Ultimate)
  (CallFunction|SpawnWeaponModel WeaponModelClass)
  (CallFunction|HideWeaponModel))

(fn ResetUltimateWeapon
  (Variables|Default|SetCurrentAmmunition (Variables|Default|GetMaxAmmunition))
  (Variables|Default|SetCurrentCooldown 0.0)
  (Variables|Default|SetCurrentReloadDuration 0.0)
  (Variables|Default|SetReloading false)
  (Variables|Default|SetAttacking false))

(fn Shoot
  (bind _wasexecuted (|CallParentFunction))
  (if (and _wasexecuted (not (Variables|Default|GetReloadable)))
    (if (<= (Variables|Default|GetCurrentAmmunition) 0)
      (Default|EndUltimate (Variables|Default|GetUltimate))))
  (return _wasexecuted))