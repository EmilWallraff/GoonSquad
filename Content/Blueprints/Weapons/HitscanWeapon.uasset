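; Hitscan firearm Blueprint for a character, handling firing, ammunition, reloading and recoil.
; Tick runs cooldown and reload timers, then fires while attacking or recovers recoil otherwise; empty magazines auto-reload.
; Each shot delegates the trace to HitscanShooting, plays a replicated sound and rotates the owner's camera along an indexed recoil pattern.
; Accumulated recoil is eased back while stepping the pattern index down, and scoping swaps bullet spread.
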(event Custom|ResetRecoil_1
  (Variables|Recoil|SetCurrentRecoilPatternPosition 0)
  (Default|RotateCamera (Variables|Default|GetOwningCharacter) (Utilities|Struct|MakeRecoil (* (.pitch (Variables|Recoil|GetInflictedRecoil)) -1.0) (* (.yaw (Variables|Recoil|GetInflictedRecoil)) -1.0)))
  (Variables|Recoil|SetInflictedRecoil ""))

(event EventTick
  (params (DeltaSeconds :type Float%20%28single-precision%29))
  (Protected|UpdateCooldown DeltaSeconds)
  (Protected|UpdateReloading DeltaSeconds)
  (if (Variables|Default|GetAttacking)
    (Protected|UpdateShooting)
    (else
      (Protected|UpdateRecoilRecovery DeltaSeconds))))

(event EventBeginPlay
  (Variables|Default|SetCurrentAmmunition (Variables|Default|GetMaxAmmunition)))

(fn CheckifAbletoAttack
  (return (Math|Boolean|ANDBoolean (<= (Variables|Default|GetCurrentCooldown) 0.0) (not (Variables|Default|GetReloading)) (not (Variables|Default|GetAttacking)))))

(fn UpdateCooldown
  (params (DeltaTime :type Float%20%28double-precision%29))
  (if (> (Variables|Default|GetCurrentCooldown) 0.0)
    (Variables|Default|SetCurrentCooldown (- (Variables|Default|GetCurrentCooldown) DeltaTime))))

(fn UpdateReloading
  (params (DeltaTime :type Float%20%28double-precision%29))
  (if (Variables|Default|GetReloading)
    (bind _output_get (Variables|Default|SetCurrentReloadDuration (- (Variables|Default|GetCurrentReloadDuration) DeltaTime)))
    (if (<= _output_get 0.0)
      (Variables|Default|SetCurrentAmmunition (Variables|Default|GetMaxAmmunition))
      (Variables|Default|SetReloading false))))

(fn SetUpWeapon
  (params (OwningCharacter :type Base%20Character%20BP%20Object%20Reference) (HitscanShooting :type Hitscan%20Shooting%20Functionality%20Object%20Reference) (WeaponModelClass :type Base%20Weapon%20Model%20BP%20Class%20Reference))
  (Variables|Default|SetOwningCharacter OwningCharacter)
  (Variables|Components|SetHitscanShooting HitscanShooting)
  (CallFunction|SpawnWeaponModel WeaponModelClass)
  (CallFunction|HideWeaponModel))

(fn UpdateShooting
  (if (<= (Variables|Default|GetCurrentCooldown) 0.0)
    (Protected|Shoot)))

(fn Shoot
  (if (> (Variables|Default|GetCurrentAmmunition) 0)
    (Math|Integer|DecrementInt (Variables|Default|GetCurrentAmmunition)
      (:%20%20
        (Variables|Default|SetCurrentCooldown (Variables|Default|GetMaxCooldown))
        (Default|ShootHitscan (Variables|Components|GetHitscanShooting) (.location (Default|GetMuzzleTransform (Variables|Default|Get1stPersonWeaponModel))))
        (Protected|ApplyRecoil)
        (CallFunction|ServerPlayReplicatedSound (Variables|Default|GetShotSound) (.location (Transformation|GetActorTransform (Variables|Default|GetOwningCharacter))))
        (if (<= (Variables|Default|GetCurrentAmmunition) 0)
          (CallFunction|StopAttacking)
          (CallFunction|Reload)
          (elif (Variables|Default|GetAutomatic)
            _
            (else
              (CallFunction|StopAttacking))))
        (return true)))
    (else
      (CallFunction|Reload)
      (return false))))

(fn UpdateRecoilRecovery
  (params (DeltaSeconds :type Float%20%28double-precision%29))
  (bind _recoilrecoveryspeed (Variables|Recoil|GetRecoilRecoverySpeed))
  (bind _returnvalue (* _recoilrecoveryspeed DeltaSeconds))
  (if (>= (Math|Float|Sqrt (+ (Math|Float|Square (.pitch (Variables|Recoil|GetInflictedRecoil))) (Math|Float|Square (.yaw (Variables|Recoil|GetInflictedRecoil))))) 0.01)
    (Variables|Recoil|SetInflictedRecoil (Utilities|Struct|MakeRecoil (- (.pitch (Variables|Recoil|GetInflictedRecoil)) (* (/ (.pitch (Variables|Recoil|GetInflictedRecoil)) (Math|Float|Sqrt (+ (Math|Float|Square (.pitch (Variables|Recoil|GetInflictedRecoil))) (Math|Float|Square (.yaw (Variables|Recoil|GetInflictedRecoil)))))) _returnvalue)) (- (.yaw (Variables|Recoil|GetInflictedRecoil)) (* (/ (.yaw (Variables|Recoil|GetInflictedRecoil)) (Math|Float|Sqrt (+ (Math|Float|Square (.pitch (Variables|Recoil|GetInflictedRecoil))) (Math|Float|Square (.yaw (Variables|Recoil|GetInflictedRecoil)))))) _returnvalue))))
    (Default|RotateCamera (Variables|Default|GetOwningCharacter) (Utilities|Struct|MakeRecoil (* (* (/ (.pitch (Variables|Recoil|GetInflictedRecoil)) (Math|Float|Sqrt (+ (Math|Float|Square (.pitch (Variables|Recoil|GetInflictedRecoil))) (Math|Float|Square (.yaw (Variables|Recoil|GetInflictedRecoil)))))) _returnvalue) -1.0) (* (* (/ (.yaw (Variables|Recoil|GetInflictedRecoil)) (Math|Float|Sqrt (+ (Math|Float|Square (.pitch (Variables|Recoil|GetInflictedRecoil))) (Math|Float|Square (.yaw (Variables|Recoil|GetInflictedRecoil)))))) _returnvalue) -1.0)))
    (if (> (Variables|Recoil|GetCurrentRecoilPatternPosition) 0)
      (if (<= (Variables|Recoil|GetCurrentRecoilPatternResetDuration) 0.0)
        (Math|Integer|DecrementInt (Variables|Recoil|GetCurrentRecoilPatternPosition)
          (:%20%20
            (Variables|Recoil|SetCurrentRecoilPatternResetDuration (Variables|Recoil|GetMaxRecoilPatternResetDuration))))
        (else
          (Variables|Recoil|SetCurrentRecoilPatternResetDuration (- (Variables|Recoil|GetCurrentRecoilPatternResetDuration) DeltaSeconds)))))))

(fn ApplyRecoil
  (bind _recoilpatternposition (Protected|CheckedRecoilPatternPosition))
  (bind _recoilpattern (Variables|Recoil|GetRecoilPattern))
  (bind _output (Utilities|Array|Get(acopy) _recoilpattern _recoilpatternposition))
  (bind (_pitch _yaw) (Utilities|Struct|BreakRecoil _output))
  (Default|RotateCamera (Variables|Default|GetOwningCharacter) _output)
  (Variables|Recoil|SetInflictedRecoil (Utilities|Struct|MakeRecoil (+ _pitch (.pitch (Variables|Recoil|GetInflictedRecoil))) (+ _yaw (.yaw (Variables|Recoil|GetInflictedRecoil)))))
  (Math|Integer|IncrementInt (Variables|Recoil|GetCurrentRecoilPatternPosition)
    (:%20%20
      (Variables|Recoil|SetCurrentRecoilPatternResetDuration (Variables|Recoil|GetMaxRecoilPatternResetDuration)))))

(fn CheckedRecoilPatternPosition
  (bind _currentrecoilpatternposition (Variables|Recoil|GetCurrentRecoilPatternPosition))
  (bind _recoilpattern (Variables|Recoil|GetRecoilPattern))
  (bind _returnvalue (Utilities|Array|Length _recoilpattern))
  (bind _returnvalue_2 (- _returnvalue 1))
  (if (<= _currentrecoilpatternposition _returnvalue_2)
    (return _currentrecoilpatternposition)
    (else
      (return _returnvalue_2))))

(fn StartAttacking
  (bind _abletoshoot (Protected|CheckifAbletoAttack))
  (if _abletoshoot
    (Variables|Default|SetAttacking true)
    (bind _wasexecuted (Protected|Shoot))
    (return _wasexecuted)
    (else
      (return false))))

(fn Reload
  (if (Variables|Default|GetReloading)
    (return true)
    (elif (< (Variables|Default|GetCurrentAmmunition) (Variables|Default|GetMaxAmmunition))
      (Variables|Default|SetReloading true)
      (Variables|Default|SetCurrentReloadDuration (Variables|Default|GetMaxReloadDuration))
      (Audio|PlaySoundatLocation (Variables|Default|GetReloadSound) (.location (Transformation|GetActorTransform (Variables|Default|GetOwningCharacter))) "0, 0, 0" 1.0 1.0 0.0 0 0 0 0)
      (return true)
      (else
        (return false)))))

(fn CancelReloading
  (if (Variables|Default|GetReloading)
    (Variables|Default|SetReloading false))
  (return false))

(fn GetMaxAmmunition
  (return (Variables|Default|GetMaxAmmunition)))

(fn GetCurrentAmmunition
  (return (Variables|Default|GetCurrentAmmunition)))

(fn StopAttacking
  (Variables|Default|SetAttacking false)
  (return false))

(fn HideWeaponModel
  (bind _visible (|CallParentFunction))
  (return _visible))

(fn ShowWeaponModel
  (bind _visible (|CallParentFunction))
  (return _visible))

(fn SpawnWeaponModel
  (params (WeaponModel :type Base%20Weapon%20Model%20BP%20Class%20Reference))
  (bind _spawned (|CallParentFunction WeaponModel))
  (return _spawned))

(fn DeleteWeaponModel
  (bind _deleted (|CallParentFunction))
  (return _deleted))

(fn ActivateScopeEffects
  (bind _hitscanshooting (Variables|Components|GetHitscanShooting))
  (Variables|/Game/Blueprints/Weapons/HitscanShootingFunctionality.HitscanShootingFunctionality_C|SetCurrentBulletSpread _hitscanshooting (Variables|/Game/Blueprints/Weapons/HitscanShootingFunctionality.HitscanShootingFunctionality_C|GetScopedBulletSpread _hitscanshooting))
  (return true))

(fn DeactivateScopeEffects
  (bind _hitscanshooting (Variables|Components|GetHitscanShooting))
  (Variables|/Game/Blueprints/Weapons/HitscanShootingFunctionality.HitscanShootingFunctionality_C|SetCurrentBulletSpread _hitscanshooting (Variables|/Game/Blueprints/Weapons/HitscanShootingFunctionality.HitscanShootingFunctionality_C|GetUnscopedBulletSpread _hitscanshooting))
  (return false))