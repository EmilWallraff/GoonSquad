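; NullTeleportShadow is a short-lived visual effect actor that leaves a frozen shadow copy of the player character, named for a teleport.
; On BeginPlay it copies the player's skeletal mesh and current pose onto a PoseableMesh, then overrides every material slot with the shadow material.
; It sets a random material parameter for variation, drives Alpha from a timeline, and destroys itself when the timeline finishes.
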(event EventBeginPlay
  (bind _poseablemesh (Variables|Default|GetPoseableMesh))
  (bind _playercharacter (Variables|Default|GetPlayerCharacter))
  (bind _mesh (Variables|/Script/Engine.Character|GetMesh _playercharacter))
  (bind _skeletalmesh (Variables|/Script/Engine.SkinnedMeshComponent|GetSkeletalMesh _mesh))
  (Class|SkinnedMeshComponent|SetSkeletalMesh _poseablemesh _skeletalmesh true)
  (for (_ _array_index) (Variables|/Script/Engine.SkeletalMesh|GetMaterials _skeletalmesh)
    (Rendering|Material|SetMaterial _poseablemesh _array_index "/Game/Assets/Materials/EffectMaterials/NullTeleport/NullTeleportShadow_M.NullTeleportShadow_M"))
  (Rendering|Material|SetScalarParameterValueonMaterials _poseablemesh "Random" (Math|Random|RandomFloat))
  (Class|PoseableMeshComponent|CopyPosefromSkeletalComponent _poseablemesh (Variables|/Script/Engine.Character|GetMesh (Variables|Default|GetPlayerCharacter)))
  (bind _newtrack_0 (Timeline|Timeline_0 PlayFromStart)
    (:Update
      (Rendering|Material|SetScalarParameterValueonMaterials (Variables|Default|GetPoseableMesh) "Alpha" _newtrack_0))
    (:Finished
      (Actor|DestroyActor))))

(fn ConstructionScript)