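; Base Blueprint for throwable abilities that spawn a projectile actor of a configurable class when executed.
; ExecuteAbility passes the owner camera's forward vector to a server event, which spawns the throwable at the camera transform with owner, instigator and ability references.
; Spawned objects are tracked in CurrentObjects; exceeding MaxObjects destroys the oldest, and ForgetObject removes an entry from the list.
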(event Custom|Server_SpawnProjectile
  (params (Direction :type Vector))
  (bind _owningcharacter (Variables|Default|GetOwningCharacter))
  (bind _currentobjects (Variables|Default|GetCurrentObjects))
  (bind _returnvalue (Game|SpawnActorfromClass (Variables|Default|GetThrowableClass) (Transformation|GetWorldTransform (Variables|/Game/Blueprints/Player/BaseCharacter_BP.BaseCharacter_BP_C|GetCamera (Variables|Default|GetOwningCharacter))) "AlwaysSpawn" _owningcharacter Direction _owningcharacter self _owningcharacter))
  (Utilities|Array|Add _currentobjects _returnvalue)
  (if (> (Utilities|Array|Length _currentobjects) (Variables|Default|GetMaxObjects))
    (Default|DestroyThrowable (Utilities|Array|Get(acopy) (Variables|Default|GetCurrentObjects)))))

(event EventBeginPlay
  (|CallParentFunction) ; This node is disabled and will not be called.\nDrag off pins to build functionality.
)

(event EventTick
  (params (DeltaSeconds :type Float%20%28single-precision%29))
  (|CallParentFunction DeltaSeconds) ; This node is disabled and will not be called.\nDrag off pins to build functionality.
)

(fn ExecuteAbility
  (|CallParentFunction)
  (CallFunction|ServerSpawnProjectile (Math|Vector|GetForwardVector (Variables|/Game/Blueprints/Player/BaseCharacter_BP.BaseCharacter_BP_C|GetCamera (Variables|Default|GetOwningCharacter)))))

(fn ForgetObject
  (params (Object :type Base%20Throwable%20BP%20Object%20Reference))
  (Utilities|Array|RemoveItem (Variables|Default|GetCurrentObjects) Object)
  (return))