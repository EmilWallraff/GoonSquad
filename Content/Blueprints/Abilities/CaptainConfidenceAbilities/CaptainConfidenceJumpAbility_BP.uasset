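; Captain Confidence's jump ability, which triggers the character's Dash after a short wind-up.
; ExecuteAbility runs the parent logic, casts the owner to CaptainConfidence_BP, plays a 2D preparation sound and calls a custom event, or prints an error for other characters.
; That event waits out a configurable Delay, calls Dash on the captain and plays the execution sound through ServerPlayReplicatedSound at the camera's location.
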(event Custom|CallDelayedDash
  (params (CaptainConfidence :type Captain%20Confidence%20BP%20Object%20Reference))
  (Utilities|FlowControl|Delay (Variables|Default|GetDelay))
  (Default|Dash CaptainConfidence)
  (CallFunction|ServerPlayReplicatedSound (Variables|Default|GetDashExecutionSound) (Transformation|GetWorldLocation (Variables|/Game/Blueprints/Player/BaseCharacter_BP.BaseCharacter_BP_C|GetCamera CaptainConfidence))))

(event EventBeginPlay
  (|CallParentFunction) ; This node is disabled and will not be called.\nDrag off pins to build functionality.
)

(event EventTick
  (params (DeltaSeconds :type Float%20%28single-precision%29))
  (|CallParentFunction DeltaSeconds) ; This node is disabled and will not be called.\nDrag off pins to build functionality.
)

(fn ExecuteAbility
  (|CallParentFunction)
  (bind _ascaptain_confidence_bp (Utilities|Casting|CastToCaptainConfidence_BP (Variables|Default|GetOwningCharacter))
    (:then
      (Audio|PlaySound2D (Variables|Default|GetDashPreperationSound) 1.0 1.0 0.0 0 0)
      (CallFunction|CallDelayedDash _ascaptain_confidence_bp))
    (:CastFailed
      (Development|PrintString "Captain Confidence Jump used on wrong character" true true "(R=1.000000,G=0.000000,B=0.009241,A=1.000000)" 1e+01))))