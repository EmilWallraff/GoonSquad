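; Ghost teleport ability that throws teleporter objects and manages them as a linked pair.
; Server spawning launches a throwable from the owner's camera transform, destroys the oldest once over the object limit, then caches the first two as Teleporter1 and Teleporter2.
; UpdateTeleporterPreperation prepares the teleporter opposite the occupied one, or unprepares both when their occupancy matches.
; DestroyTeleporters removes both.
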(event EventBeginPlay
  (|CallParentFunction) ; This node is disabled and will not be called.\nDrag off pins to build functionality.
)

(event EventTick
  (params (DeltaSeconds :type Float%20%28single-precision%29))
  (|CallParentFunction DeltaSeconds) ; This node is disabled and will not be called.\nDrag off pins to build functionality.
)

(event EventServerSpawnProjectile
  (params (Direction :type Vector :default "0, 0, 0"))
  (bind _owningcharacter (Variables|Default|GetOwningCharacter))
  (bind _currentobjects (Variables|Default|GetCurrentObjects))
  (bind _currentobjects_2 (Variables|Default|GetCurrentObjects))
  (|CallParentFunction Direction)
  (bind _returnvalue (Game|SpawnActorfromClass (Variables|Default|GetThrowableClass) (Transformation|GetWorldTransform (Variables|/Game/Blueprints/Player/BaseCharacter_BP.BaseCharacter_BP_C|GetCamera (Variables|Default|GetOwningCharacter))) "AlwaysSpawn" _owningcharacter "0.000000,0.000000,0.000000" _owningcharacter self _owningcharacter))
  (Utilities|Array|Add _currentobjects _returnvalue)
  (if (> (Utilities|Array|Length _currentobjects) (Variables|Default|GetMaxObjects))
    (Default|DestroyThrowable (Utilities|Array|Get(acopy) (Variables|Default|GetCurrentObjects))))
  (bind _asghost_teleporter_throwable_bp (Utilities|Casting|CastToGhostTeleporterThrowable_BP (Utilities|Array|Get(acopy) _currentobjects_2)))
  (Variables|Default|SetTeleporter1 _asghost_teleporter_throwable_bp)
  (bind _asghost_teleporter_throwable_bp_2 (Utilities|Casting|CastToGhostTeleporterThrowable_BP (Utilities|Array|Get(acopy) _currentobjects_2 1)))
  (Variables|Default|SetTeleporter2 _asghost_teleporter_throwable_bp_2))

(fn ExecuteAbility
  (|CallParentFunction))

(fn ForgetObject
  (params (Object :type Base%20Throwable%20BP%20Object%20Reference))
  (|CallParentFunction Object))

(fn UpdateTeleporterPreperation
  (bind _teleporter1 (Variables|Default|GetTeleporter1))
  (bind _teleporter2 (Variables|Default|GetTeleporter2))
  (bind _playerinside (Variables|/Game/Blueprints/Interactables/Projetiles/GhostTeleporterThrowable_BP.GhostTeleporterThrowable_BP_C|GetPlayerInside _teleporter2))
  (bind _playerinside_2 (Variables|/Game/Blueprints/Interactables/Projetiles/GhostTeleporterThrowable_BP.GhostTeleporterThrowable_BP_C|GetPlayerInside _teleporter1))
  (if (and (Utilities|IsValid (Variables|Default|GetTeleporter1)) (Utilities|IsValid (Variables|Default|GetTeleporter2)))
    (if (== _playerinside_2 _playerinside)
      (Default|UnprepareTeleporter (Variables|Default|GetTeleporter1))
      (Default|UnprepareTeleporter (Variables|Default|GetTeleporter2))
      (elif _playerinside_2
        (Default|UnprepareTeleporter (Variables|Default|GetTeleporter1))
        (Default|PrepareTeleporter (Variables|Default|GetTeleporter2))
        (elif _playerinside
          (Default|UnprepareTeleporter (Variables|Default|GetTeleporter2))
          (Default|PrepareTeleporter (Variables|Default|GetTeleporter1)))))))

(fn DestroyTeleporters
  (Default|DestroyThrowable (Variables|Default|GetTeleporter1))
  (Default|DestroyThrowable (Variables|Default|GetTeleporter2)))