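; Base ability with charges and a cooldown, storing its owning character and leaving ExecuteAbility empty as an override point.
; CallAbility spends a charge, runs ExecuteAbility and reports success, while Tick restores charges one per cooldown up to the maximum.
; Cooldown helpers scale or shorten the remaining time and can grant a charge without checking that maximum.
; A server event relays sounds through a multicast to play at a location.
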(event Custom|Server_PlayReplicatedSound
  (params (Sound :type Sound%20Cue%20Object%20Reference) (Location :type Vector))
  (CallFunction|MulticastPlayReplicatedSound Sound Location))

(event Custom|Multicast_PlayReplicatedSound
  (params (Sound :type Sound%20Cue%20Object%20Reference) (Location :type Vector))
  (Audio|PlaySoundatLocation Sound Location "0, 0, 0" 1.0 1.0 0.0 0 0 0 0))

(event EventBeginPlay
  (Variables|Default|SetCurrentCharges (Variables|Default|GetMaxCharges))
  (Variables|Default|SetCurrentCooldown (Variables|Default|GetMaxCooldown)))

(event EventTick
  (params (DeltaSeconds :type Float%20%28single-precision%29))
  (if (< (Variables|Default|GetCurrentCharges) (Variables|Default|GetMaxCharges))
    (bind _output_get (Variables|Default|SetCurrentCooldown (- (Variables|Default|GetCurrentCooldown) DeltaSeconds)))
    (if (<= _output_get 0.0)
      (Math|Integer|IncrementInt (Variables|Default|GetCurrentCharges)
        (:%20%20
          (Variables|Default|SetCurrentCooldown (Variables|Default|GetMaxCooldown)))))))

(fn CallAbility
  (if (>= (Variables|Default|GetCurrentCharges) 1)
    (Protected|UseOneCharge)
    (Protected|ExecuteAbility)
    (return true)
    (else
      (return false))))

(fn SetUpAbility
  (params (Character :type Base%20Character%20BP%20Object%20Reference))
  (Variables|Default|SetOwningCharacter Character))

(fn GetMaxCooldown
  (return (Variables|Default|GetMaxCooldown)))

(fn ReduceCooldownbyPercentage
  (params (CooldownPercentage :type Float%20%28double-precision%29))
  (bind _output_get (Variables|Default|SetCurrentCooldown (* CooldownPercentage (Variables|Default|GetCurrentCooldown))))
  (if (<= _output_get 0.0)
    (Math|Integer|IncrementInt (Variables|Default|GetCurrentCharges)
      (:%20%20
        (Variables|Default|SetCurrentCooldown 0.0)))))

(fn ReduceCooldownbyFixedTime
  (params (CooldownReduction :type Float%20%28double-precision%29))
  (bind _output_get (Variables|Default|SetCurrentCooldown (- (Variables|Default|GetCurrentCooldown) CooldownReduction)))
  (if (<= _output_get 0.0)
    (Math|Integer|IncrementInt (Variables|Default|GetCurrentCharges)
      (:%20%20
        (Variables|Default|SetCurrentCooldown 0.0)))))

(fn ExecuteAbility)

(fn UseOneCharge
  (Math|Integer|DecrementInt (Variables|Default|GetCurrentCharges)))