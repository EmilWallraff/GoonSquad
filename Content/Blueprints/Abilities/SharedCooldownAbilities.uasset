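; An ability Blueprint that lets a group of abilities share one pool of charges, as a shared cooldown.
; SetAbilities stores the group, and CallOneAbility triggers a member only if a charge is available, spending one only when that ability reports success.
; Non-members are rejected with a debug message.
; Its own CallAbility prints a warning and returns false, since direct calls are discouraged.
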(event EventBeginPlay
  (|CallParentFunction) ; This node is disabled and will not be called.\nDrag off pins to build functionality.
)

(event EventTick
  (params (DeltaSeconds :type Float%20%28single-precision%29))
  (|CallParentFunction DeltaSeconds) ; This node is disabled and will not be called.\nDrag off pins to build functionality.
)

(fn SetAbilities
  (params (Abilities :type Array%20of%20Base%20Ability%20Object%20References))
  (Variables|Default|SetAbilities Abilities))

(fn CallOneAbility
  (params (Ability :type Base%20Ability%20Object%20Reference))
  (if (Utilities|Array|ContainsItem (Variables|Default|GetAbilities) Ability)
    (if (>= (Variables|Default|GetCurrentCharges) 1)
      (bind _wasexecuted (CallFunction|CallAbility Ability))
      (if _wasexecuted
        (CallFunction|UseOneCharge)
        (return true)
        (else
          (return false)))
      (else
        _))
    (else
      (Development|PrintString "This ability is not part of the shared cooldown  abilities" true true "(R=1.000000,G=0.000000,B=0.040545,A=1.000000)" 1e+01)))
  (return false))

(fn CallAbility
  (Development|PrintString "Directly Calling a shared ability is not encouraged!" true true "(R=1.000000,G=0.055935,B=0.000000,A=1.000000)" 1e+01)
  (return false))