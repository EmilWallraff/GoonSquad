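; BaseDurationAbility is a base Blueprint for charge-based abilities that stay active for a limited duration.
; CallAbility works as a toggle when at least one charge is available, activating the ability and returning true, or ending it early and returning false.
; Tick accumulates elapsed time while active and ends the ability at MaxDuration.
; The charge is spent in EndAbility rather than on activation, alongside resetting the timer.
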(event EventBeginPlay
  (|CallParentFunction) ; This node is disabled and will not be called.\nDrag off pins to build functionality.
)

(event EventTick
  (params (DeltaSeconds :type Float%20%28single-precision%29))
  (|CallParentFunction DeltaSeconds)
  (if (Variables|Default|GetActivated)
    (bind _output_get (Variables|Default|SetCurrentDuration (+ (Variables|Default|GetCurrentDuration) DeltaSeconds)))
    (if (>= _output_get (Variables|Default|GetMaxDuration))
      (Protected|EndAbility))))

(fn EndAbility
  (Variables|Default|SetActivated false)
  (CallFunction|UseOneCharge)
  (Variables|Default|SetCurrentDuration 0.0))

(fn ExecuteAbility
  (Variables|Default|SetActivated true))

(fn CallAbility
  (if (>= (Variables|Default|GetCurrentCharges) 1)
    (if (Variables|Default|GetActivated)
      (Protected|EndAbility)
      (return false)
      (else
        (CallFunction|ExecuteAbility)
        (return true)))
    (else
      (return false))))