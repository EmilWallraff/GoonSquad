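; Playable character Blueprint for Hook, a hitscan gunner with frag, smoke and molotov grenade abilities plus an ultimate weapon.
; The three grenade inputs route through a shared-cooldown component, while the ultimate input triggers HookUltimate, which is linked to its own hitscan weapon.
; Parent initialization overrides register these components and feed abilities and key bindings to the Hook ability HUD.
; Tick refreshes the third-person health and shield bars every frame.
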(event EventBeginPlay
  (|CallParentFunction))

(event EventTick
  (params (DeltaSeconds :type Float%20%28single-precision%29))
  (|CallParentFunction DeltaSeconds)
  ;[1 1 1] Don't ask...
  (CallFunction|UpdateThirdPersonHealthBar)
  (CallFunction|UpdateThirdPersonShieldBar))

(event Input|ActionEvents|InputActionSecondaryFire
  (params (Key :type Key%20Structure :default "None")))

(event Input|ActionEvents|InputActionAbility3
  (params (Key :type Key%20Structure :default "None"))
  (:Pressed
    (Default|CallOneAbility (Variables|Default|GetSharedCooldownAbilities) (Variables|Default|GetHookMolotovAbility))))

(event Input|ActionEvents|InputActionAbility2
  (params (Key :type Key%20Structure :default "None"))
  (:Pressed
    (Default|CallOneAbility (Variables|Default|GetSharedCooldownAbilities) (Variables|Default|GetHookSmokeGranadeAbility))))

(event Input|ActionEvents|InputActionAbility1
  (params (Key :type Key%20Structure :default "None"))
  (:Pressed
    (Default|CallOneAbility (Variables|Default|GetSharedCooldownAbilities) (Variables|Default|GetHookFragGrenadeAbility))))

(event Input|ActionEvents|InputActionUltimate
  (params (Key :type Key%20Structure :default "None"))
  (:Pressed
    (Default|CallUltimate (Variables|Default|GetHookUltimate))))

(fn ConstructionScript
  (|CallParentFunction))

(fn GetAbilities
  (return (Utilities|Array|MakeArray 0 0 0)))

(fn InitializeAbilities
  (bind _hookfraggrenadeability (Variables|Default|GetHookFragGrenadeAbility))
  (bind _hookmolotovability (Variables|Default|GetHookMolotovAbility))
  (bind _hooksmokegranadeability (Variables|Default|GetHookSmokeGranadeAbility))
  (|CallParentFunction)
  (Default|SetUpAbility _hooksmokegranadeability self)
  (Utilities|Array|Add (LocalVariables|GetAbilityArray) _hooksmokegranadeability)
  (Default|SetUpAbility _hookfraggrenadeability self)
  (Utilities|Array|Add (LocalVariables|GetAbilityArray) _hookfraggrenadeability)
  (Default|SetUpAbility _hookmolotovability self)
  (Utilities|Array|Add (LocalVariables|GetAbilityArray) _hookmolotovability)
  (Default|SetUpAbility (Variables|Default|GetSharedCooldownAbilities) self)
  (Default|SetAbilities (Variables|Default|GetSharedCooldownAbilities) (LocalVariables|GetAbilityArray))
  (Default|SetUpUltimate (Variables|Default|GetHookUltimate) self))

(fn InitializeWeapons
  (bind _primaryweapon (Variables|Default|GetPrimaryWeapon))
  (Default|SetUpHitscan (Variables|Default|GetPrimaryHitscanFunctionality) self)
  (Default|SetUpWeapon (Variables|Default|GetPrimaryWeapon) self (Variables|Default|GetPrimaryHitscanFunctionality) "/Game/Blueprints/Weapons/WeaponModelBlueprints/HookGunModel_BP.HookGunModel_BP_C")
  (Variables|Default|SetCurrentlyUsedWeapon _primaryweapon)
  (Utilities|Array|Add (Variables|Default|GetAllWeapons) _primaryweapon)
  (Default|SetUpHitscan (Variables|Default|GetUltimateHitscanFunctionality) self)
  (Default|SetUpUltimateWeapon (Variables|Default|GetUltimateWeapon) self (Variables|Default|GetUltimateHitscanFunctionality) (Variables|Default|GetHookUltimate) "/Game/Blueprints/Weapons/WeaponModelBlueprints/HookUltGunModel.HookUltGunModel_C")
  (|CallParentFunction))

(fn SetUpHUDs
  (params (HUD :type Base%20HUD%20WBP%20Object%20Reference) (AbilityHUD :type User%20Widget%20Object%20Reference))
  (|CallParentFunction HUD AbilityHUD)
  (bind _ashook_ability_hud_wbp (Utilities|Casting|CastToHookAbilityHUD_WBP AbilityHUD)
    (:then
      (bind _output_get (Variables|Default|SetAbilityHUD _ashook_ability_hud_wbp))
      (Default|InitializeAbilityHUD _output_get (Variables|Default|GetHookFragGrenadeAbility) (Variables|Default|GetHookMolotovAbility) (Variables|Default|GetHookSmokeGranadeAbility) (Variables|Default|GetHookUltimate)))
    (:CastFailed
      (Development|PrintString "Hook: received wrong/no abilityHUD" true true "(R=1.000000,G=0.000000,B=0.041613,A=1.000000)" 1e+01))))

(fn UpdateValuesinHUDs
  (bind _returnvalue (Class|InputSettings|GetInputSettings))
  (|CallParentFunction)
  (Default|UpdateAbilityHUD (Variables|Default|GetAbilityHUD) (Variables|Default|GetSharedCooldownAbilities) (.key (Utilities|Array|Get(acopy) (Class|InputSettings|GetActionMappingbyName _returnvalue "Ability1"))) (.key (Utilities|Array|Get(acopy) (Class|InputSettings|GetActionMappingbyName _returnvalue "Ability3"))) (.key (Utilities|Array|Get(acopy) (Class|InputSettings|GetActionMappingbyName _returnvalue "Ability2"))) (Variables|Default|GetHookUltimate) (.key (Utilities|Array|Get(acopy) (Class|InputSettings|GetActionMappingbyName _returnvalue "Ultimate")))))