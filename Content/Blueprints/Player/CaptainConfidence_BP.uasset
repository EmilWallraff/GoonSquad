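; Captain Confidence is a playable hero character with grenade, jump and teleporter abilities, an ultimate, and a hitscan primary weapon.
; Input events trigger ability components, which are set up here and shown in a dedicated ability HUD.
; Dash launches the character server-side along camera vectors, with multicast third-person effects cleared on landing.
; Second life is replicated by multicast; TakeDamage consumes it to restore full health and end the ultimate instead of dying.
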(event Custom|Server_Dash
  (params (Forward%20Vector :type Vector) (UpVector :type Vector))
  (Character|LaunchCharacter (+ (* Forward%20Vector (Variables|Default|GetDashForwardSpeed)) (* UpVector (Variables|Default|GetDashUpwardSpeed))) false false))

(event Custom|Server_SetSecondLife
  (params (SecondLife :type Boolean))
  (CallFunction|MulticastSetSecondLife SecondLife))

(event Custom|Multicast_SetSecondLife
  (params (SecondLife :type Boolean))
  (Variables|Default|SetSecondLife SecondLife))

(event Custom|Server_EndUltimate
  (CallFunction|MulticastEndUltimate))

(event Custom|Multicast_EndUltimate
  (Default|EndUltimate (Variables|Components|GetCaptainConfidenceUltimate)))

(event Custom|Server_SetDashEffectActivation
  (params (Activated :type Boolean))
  (CallFunction|MulticastSetDashEffectActivation Activated))

(event Custom|Multicast_SetDashEffectActivation
  (params (Activated :type Boolean))
  (bind _thirdpersondasheffect (Variables|Components|GetThirdPersonDashEffect))
  (if Activated
    (Components|Activation|Activate _thirdpersondasheffect false)
    (else
      (Components|Activation|Deactivate _thirdpersondasheffect))))

(event EventBeginPlay
  (|CallParentFunction))

(event EventOnLanded
  (params (Hit :type Hit%20Result%20Structure%20%28by%20ref%29))
  (Components|Activation|Deactivate (Variables|Components|GetFirstPersonDashEffect))
  (CallFunction|ServerSetDashEffectActivation false))

(event EventTick
  (params (DeltaSeconds :type Float%20%28single-precision%29))
  (|CallParentFunction DeltaSeconds)
  ;[1 1 1] Don't ask...
  (CallFunction|UpdateThirdPersonHealthBar)
  (CallFunction|UpdateThirdPersonShieldBar))

(event Input|ActionEvents|InputActionSecondaryFire
  (params (Key :type Key%20Structure)))

(event Input|ActionEvents|InputActionAbility2
  (params (Key :type Key%20Structure))
  (:Pressed
    (Default|CallAbility (Variables|Components|GetJumpAbility))))

(event Input|ActionEvents|InputActionAbility1
  (params (Key :type Key%20Structure))
  (:Pressed
    (Default|CallAbility (Variables|Components|GetGrenadeAbility))))

(event Input|ActionEvents|InputActionUltimate
  (params (Key :type Key%20Structure))
  (:Pressed
    (Default|CallUltimate (Variables|Components|GetCaptainConfidenceUltimate))))

(event Input|ActionEvents|InputActionAbility3
  (params (Key :type Key%20Structure))
  (:Pressed
    (Default|CallAbility (Variables|Components|GetTeleporterAbility))))

(fn ConstructionScript
  (|CallParentFunction))

(fn InitializeAbilities
  (|CallParentFunction)
  (Default|SetUpAbility (Variables|Components|GetJumpAbility) self)
  (Default|SetUpAbility (Variables|Components|GetGrenadeAbility) self)
  (Default|SetUpAbility (Variables|Components|GetTeleporterAbility) self)
  (Default|SetUpUltimate (Variables|Components|GetCaptainConfidenceUltimate) self))

(fn InitializeWeapons
  (bind _primaryweapon (Variables|Components|GetPrimaryWeapon))
  (Default|SetUpHitscan (Variables|Components|GetPrimaryShootingFunctionality) self)
  (Default|SetUpWeapon (Variables|Components|GetPrimaryWeapon) self (Variables|Components|GetPrimaryShootingFunctionality) "/Game/Blueprints/Weapons/WeaponModelBlueprints/CaptainConfidenceGunModel_BP.CaptainConfidenceGunModel_BP_C")
  (Variables|Default|SetCurrentlyUsedWeapon _primaryweapon)
  (Utilities|Array|Add (Variables|Default|GetAllWeapons) _primaryweapon)
  (|CallParentFunction))

(fn SetUpHUDs
  (params (HUD :type Base%20HUD%20WBP%20Object%20Reference) (AbilityHUD :type User%20Widget%20Object%20Reference))
  (|CallParentFunction HUD AbilityHUD)
  (bind _ascaptain_confidence_ability_hud_wbp (Utilities|Casting|CastToCaptainConfidenceAbilityHUD_WBP AbilityHUD)
    (:then
      (bind _output_get (Variables|Default|SetAbilityHUD _ascaptain_confidence_ability_hud_wbp))
      (Default|InitializeAbilityHUD _output_get (Variables|Components|GetJumpAbility) (Variables|Components|GetGrenadeAbility) (Variables|Components|GetTeleporterAbility) (Variables|Components|GetCaptainConfidenceUltimate)))
    (:CastFailed
      (Development|PrintString "Captain Confidence: received wrong/no abilityHUD" true true "(R=1.000000,G=0.000000,B=0.041613,A=1.000000)" 1e+01))))

(fn UpdateValuesinHUDs
  (bind _returnvalue (Class|InputSettings|GetInputSettings))
  (|CallParentFunction)
  (Default|UpdateAbilityHUD (Variables|Default|GetAbilityHUD) (Variables|Components|GetJumpAbility) (.key (Utilities|Array|Get(acopy) (Class|InputSettings|GetActionMappingbyName _returnvalue "Ability2"))) (Variables|Components|GetGrenadeAbility) (.key (Utilities|Array|Get(acopy) (Class|InputSettings|GetActionMappingbyName _returnvalue "Ability1"))) (Variables|Components|GetTeleporterAbility) (.key (Utilities|Array|Get(acopy) (Class|InputSettings|GetActionMappingbyName _returnvalue "Ability3"))) (Variables|Components|GetCaptainConfidenceUltimate) (.key (Utilities|Array|Get(acopy) (Class|InputSettings|GetActionMappingbyName _returnvalue "Ultimate")))))

(fn Dash
  (bind _camera (Variables|Default|GetCamera))
  (CallFunction|ServerDash (Math|Vector|GetForwardVector _camera) (Math|Vector|GetUpVector _camera))
  (Components|Activation|Activate (Variables|Components|GetFirstPersonDashEffect) false)
  (CallFunction|ServerSetDashEffectActivation true))

(fn ActivateSecondLife
  (CallFunction|ServerSetSecondLife true))

(fn DeactivateSecondLife
  (CallFunction|ServerSetSecondLife false))

(fn TakeDamage
  (params (DamageValue :type Float%20%28double-precision%29) (Instigator :type Damage%20Instigator%20Structure))
  (bind _playerstatereference (Variables|Default|GetPlayerStateReference))
  (bind _isenemydamage (CallFunction|CheckifEnemyDamage Instigator))
  (if _isenemydamage
    (CallFunction|ResetSelfHealCooldown)
    (bind _output_get (LocalVariables|SetModifiedDamageValue (* (Variables|Default|GetCurrentDamageMultiplier) DamageValue)))
    (CallFunction|SetCurrentHealth (- (Variables|Default|GetCurrentHealth) _output_get))
    (if (<= (Variables|Default|GetCurrentHealth) 0.0)
      (if (not (Variables|Default|GetSecondLife))
        (CallFunction|Die Instigator)
        (Default|ReportDamageReceived _playerstatereference (+ (Variables|Default|GetCurrentHealth) (LocalVariables|GetModifiedDamageValue)) true Instigator)
        (CallFunction|ServerFeedbackDamageInstigator (+ (Variables|Default|GetCurrentHealth) (LocalVariables|GetModifiedDamageValue)) true Instigator)
        (return (+ (Variables|Default|GetCurrentHealth) (LocalVariables|GetModifiedDamageValue)) true)
        (else
          (Variables|Default|SetCurrentHealth (Variables|Default|GetMaxHealth))
          (CallFunction|ServerSetSecondLife false)
          (CallFunction|ServerEndUltimate))))
    (Default|ReportDamageReceived _playerstatereference (LocalVariables|GetModifiedDamageValue) false Instigator)
    (CallFunction|ServerFeedbackDamageInstigator (LocalVariables|GetModifiedDamageValue) false Instigator)
    (return (LocalVariables|GetModifiedDamageValue) false)
    (else
      (return 0.0 false))))