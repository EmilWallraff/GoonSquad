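; StatusEffect_BP represents a player status effect such as Bleeding, Poisoned, Burning or Watched.
; Its construction script switches on Type to set the display name and icon, which GetDisplayData returns.
; UpdateStatusEffect subtracts the passed delta time from RemainingTime, but nothing happens yet when it runs out, and the event graph holds only disabled default events.
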(event EventBeginPlay)

(event Collision|EventActorBeginOverlap
  (params (OtherActor :type Actor%20Object%20Reference)))

(event EventTick
  (params (DeltaSeconds :type Float%20%28single-precision%29)))

(fn ConstructionScript
  (switch Utilities|FlowControl|Switch|SwitchonStatusEffectType (Variables|Default|GetType)
    (:NewEnumerator0
      (Variables|Default|SetDisplayName "Bleeding")
      (Variables|Default|SetDisplayIcon "/Game/Assets/2DIcons/StatusEffectIcons/GS_bleeding_icon.GS_bleeding_icon"))
    (:NewEnumerator1
      (Variables|Default|SetDisplayName "Poisoned")
      (Variables|Default|SetDisplayIcon "/Game/Assets/2DIcons/StatusEffectIcons/GS_poisoned_icon.GS_poisoned_icon"))
    (:NewEnumerator2
      (Variables|Default|SetDisplayName "Burning")
      (Variables|Default|SetDisplayIcon "/Game/Assets/2DIcons/StatusEffectIcons/GS_burning_icon.GS_burning_icon"))
    (:NewEnumerator3
      (Variables|Default|SetDisplayName "Watched")
      (Variables|Default|SetDisplayIcon "/Game/Assets/2DIcons/StatusEffectIcons/GS_watched_icon.GS_watched_icon"))))

(fn GetDisplayData
  (return (Variables|Default|GetDisplayName) (Variables|Default|GetDisplayIcon)))

(fn UpdateStatusEffect
  (params (DeltaTime :type Float%20%28double-precision%29))
  (bind _output_get (Variables|Default|SetRemainingTime (- (Variables|Default|GetRemainingTime) DeltaTime)))
  (if (<= _output_get 0.0)
    _))