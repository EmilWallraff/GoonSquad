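; Morbius player character Blueprint, extending a parent character with Bat, Orb and Impaler abilities, an ultimate, a hitscan primary weapon and claws.
; Inputs trigger the ability objects, with bat form blocking all but the Bat ability.
; Bat and ultimate form flags jointly manage weapon-switch blocking, while bat form also blocks weapon use.
; Overrides feed abilities and key bindings to the Morbius HUD; Tick refreshes third-person health and shield bars.
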(event EventBeginPlay
  (|CallParentFunction))

(event EventTick
  (params (DeltaSeconds :type Float%20%28single-precision%29))
  (|CallParentFunction DeltaSeconds)
  ;[1 1 1] Don't ask...
  (CallFunction|UpdateThirdPersonHealthBar)
  (CallFunction|UpdateThirdPersonShieldBar))

(event Input|ActionEvents|InputActionSecondaryFire
  (params (Key :type Key%20Structure))
  (:Pressed
    (if (not (Variables|Default|GetBatForm))
      (Default|CallAbility (Variables|Default|GetMorbiusOrbAbility)))))

(event Input|ActionEvents|InputActionAbility3
  (params (Key :type Key%20Structure))
  (:Pressed
    (if (not (Variables|Default|GetBatForm))
      (Default|CallAbility (Variables|Default|GetMorbiusImpalerAbility)))))

(event Input|ActionEvents|InputActionAbility2
  (params (Key :type Key%20Structure))
  (:Pressed
    (Default|CallAbility (Variables|Default|GetMorbiusBatAbility))))

(event Input|ActionEvents|InputActionAbility1
  (params (Key :type Key%20Structure))
  (:Pressed
    (if (not (Variables|Default|GetBatForm))
      (Default|CallAbility (Variables|Default|GetMorbiusOrbAbility)))))

(event Input|ActionEvents|InputActionUltimate
  (params (Key :type Key%20Structure))
  (:Pressed
    (if (not (Variables|Default|GetBatForm))
      (Default|CallUltimate (Variables|Default|GetMorbiusUltimate)))))

(fn ConstructionScript
  (|CallParentFunction))

(fn GetAbilities
  (return (Utilities|Array|MakeArray 0 0 0)))

(fn InitializeAbilities
  (|CallParentFunction)
  (Default|SetUpAbility (Variables|Default|GetMorbiusBatAbility) self)
  (Default|SetUpAbility (Variables|Default|GetMorbiusOrbAbility) self)
  (Default|SetUpAbility (Variables|Default|GetMorbiusImpalerAbility) self)
  (Default|SetUpUltimate (Variables|Default|GetMorbiusUltimate) self))

(fn InitializeWeapons
  (bind _primaryweapon (Variables|Default|GetPrimaryWeapon))
  (Default|SetUpHitscan (Variables|Default|GetPrimaryShootingFunctionality) self)
  (Default|SetUpWeapon (Variables|Default|GetPrimaryWeapon) self (Variables|Default|GetPrimaryShootingFunctionality) "/Game/Blueprints/Weapons/WeaponModelBlueprints/MorbiusGunModel_BP.MorbiusGunModel_BP_C")
  (Variables|Default|SetCurrentlyUsedWeapon _primaryweapon)
  (Utilities|Array|Add (Variables|Default|GetAllWeapons) _primaryweapon)
  (Default|SetUpWeapon (Variables|Default|GetUltimateClaws) self "/Game/Blueprints/Weapons/WeaponModelBlueprints/KnifeModel_BP.KnifeModel_BP_C")
  (|CallParentFunction))

(fn SetUpHUDs
  (params (HUD :type Base%20HUD%20WBP%20Object%20Reference) (ScopeHUD :type Scope%20WBP%20Object%20Reference) (AbilityHUD :type User%20Widget%20Object%20Reference))
  (|CallParentFunction HUD ScopeHUD AbilityHUD)
  (bind _asmorbius_ability_hud_wbp (Utilities|Casting|CastToMorbiusAbilityHUD_WBP AbilityHUD)
    (:then
      (bind _output_get (Variables|Default|SetAbilityHUD _asmorbius_ability_hud_wbp))
      (Default|InitializeAbilityHUD _output_get (Variables|Default|GetMorbiusBatAbility) (Variables|Default|GetMorbiusOrbAbility) (Variables|Default|GetMorbiusImpalerAbility) (Variables|Default|GetMorbiusUltimate)))
    (:CastFailed
      (Development|PrintString "Morbius: received wrong/no abilityHUD" true true "(R=1.000000,G=0.000000,B=0.041613,A=1.000000)" 1e+01))))

(fn UpdateValuesinHUDs
  (bind _returnvalue (Class|InputSettings|GetInputSettings))
  (|CallParentFunction)
  (Default|UpdateAbilityHUD (Variables|Default|GetAbilityHUD) (Variables|Default|GetMorbiusBatAbility) (.key (Utilities|Array|Get(acopy) (Class|InputSettings|GetActionMappingbyName _returnvalue "Ability2"))) (Variables|Default|GetMorbiusOrbAbility) (.key (Utilities|Array|Get(acopy) (Class|InputSettings|GetActionMappingbyName _returnvalue "Ability1"))) (Variables|Default|GetMorbiusImpalerAbility) (.key (Utilities|Array|Get(acopy) (Class|InputSettings|GetActionMappingbyName _returnvalue "Ability3"))) (Variables|Default|GetMorbiusUltimate) (.key (Utilities|Array|Get(acopy) (Class|InputSettings|GetActionMappingbyName _returnvalue "Ultimate")))))

(fn ToggleBatForm
  (params (Activate :type Boolean))
  (bind _output_get (Variables|Default|SetBatForm Activate))
  (CallFunction|ToggleWeaponUseBlock _output_get)
  (if (not (Variables|Default|GetUltForm))
    (CallFunction|ToggleWeaponSwitchBlock _output_get)))

(fn ToggleUltForm
  (params (Activate :type Boolean))
  (bind _output_get (Variables|Default|SetUltForm Activate))
  (if (not (Variables|Default|GetBatForm))
    (CallFunction|ToggleWeaponSwitchBlock _output_get)))