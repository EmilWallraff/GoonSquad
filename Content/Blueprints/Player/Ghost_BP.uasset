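; Ghost_BP is the playable Ghost character, with fake, teleport and smoke abilities, an ultimate and passive cloaking.
; The server cloaks it after a timer, multicasting hidden mesh, shadow and third-person weapons.
; Movement, jumping, crouching, firing, ability use or enemy damage resets the timer or decloaks.
; A per-tick camera trace selects its ready throwable nearest the aim line, which the matching ability key activates instead of calling the ability.
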(event Custom|Server_Cloak
  (CallFunction|MulticastCloak))

(event Custom|Server_Decloak
  (CallFunction|MulticastDecloak))

(event Custom|Server_SetCurrentCloakingPreperationTime
  (params (CurrentCloakingPreperationTime :type Float%20%28double-precision%29))
  (Variables|Default|SetCurrentCloakingPreperationTime CurrentCloakingPreperationTime))

(event Custom|Multicast_Cloak
  (bind _switchedtoweapon (Variables|Default|GetSwitchedToWeapon))
  (bind _mesh (Variables|Character|GetMesh))
  (Rendering|SetVisibility _mesh false false)
  (Rendering|SetCastShadow _mesh false)
  (bind _asbase_weapon_bp (Utilities|Casting|CastToBaseWeapon_BP (Variables|Default|GetCurrentlyUsedWeapon)))
  (Default|ServerHide3rdPersonWeaponModel _asbase_weapon_bp)
  (Utilities|IsValid _switchedtoweapon
    (:Is%20Valid
      (bind _asbase_weapon_bp_2 (Utilities|Casting|CastToBaseWeapon_BP _switchedtoweapon))
      (Default|ServerHide3rdPersonWeaponModel _asbase_weapon_bp_2))
    (:Is%20Not%20Valid
      _))
  (Variables|Default|SetCloaked true))

(event Custom|Server_SetSwitchingWeapon
  (params (SwitchingWeapon :type Boolean))
  ;[0 0 0] Weapon Equipment adjusted for cloaking
  (Variables|Default|SetSwitchingWeapon SwitchingWeapon))

(event Custom|Multicast_Decloak
  (bind _mesh (Variables|Character|GetMesh))
  (Rendering|SetVisibility _mesh true false)
  (Rendering|SetCastShadow _mesh true)
  (if (Variables|Default|GetSwitchingWeapon)
    (bind _asbase_weapon_bp (Utilities|Casting|CastToBaseWeapon_BP (Variables|Default|GetSwitchedToWeapon)))
    (Default|ServerShow3rdPersonWeaponModel _asbase_weapon_bp)
    (else
      (bind _asbase_weapon_bp_2 (Utilities|Casting|CastToBaseWeapon_BP (Variables|Default|GetCurrentlyUsedWeapon)))
      (Default|ServerShow3rdPersonWeaponModel _asbase_weapon_bp_2)))
  (Variables|Default|SetCloaked false))

(event EventBeginPlay
  (|CallParentFunction))

(event EventWaitandEquipWeapon
  (params (WeaponIndex :type Integer) (WeaponDrawDuration :type Float%20%28double-precision%29))
  (bind _allweapons (Variables|Default|GetAllWeapons))
  (bind _allweapons_2 (Variables|Default|GetAllWeapons))
  (bind _output (Utilities|Array|Get(acopy) _allweapons WeaponIndex))
  (bind _output_2 (Utilities|Array|Get(acopy) _allweapons_2 WeaponIndex))
  ;[0 0 0] Weapon Equipment adjusted for cloaking
  (Utilities|FlowControl|Delay (* WeaponDrawDuration 0.15))
  (Class|WeaponBPI|ShowWeaponModel(Message) _output_2)
  (if (Variables|Default|GetCloaked)
    (bind _asbase_weapon_bp (Utilities|Casting|CastToBaseWeapon_BP _output_2)
      (:then
        (Default|ServerHide3rdPersonWeaponModel _asbase_weapon_bp))
      (:CastFailed
        _)))
  (Utilities|FlowControl|Delay (* WeaponDrawDuration 0.85))
  (if (Variables|Default|GetSwitchingWeapon)
    (CallFunction|HideAllOtherWeaponModels WeaponIndex)
    (CallFunction|ServerSetCurrentlyUsedWeapon _output)
    (Variables|Default|SetCurrentlyUsedWeapon _output)
    (CallFunction|ServerSetSwitchingWeapon false)
    (bind _currentammunition (Class|WeaponBPI|GetCurrentAmmunition(Message) (Variables|Default|GetCurrentlyUsedWeapon)))
    (if (<= _currentammunition 0)
      (Class|WeaponBPI|Reload(Message) (Variables|Default|GetCurrentlyUsedWeapon)))))

(event EventTick
  (params (DeltaSeconds :type Float%20%28single-precision%29))
  (|CallParentFunction DeltaSeconds)
  (Networking|SwitchHasAuthority
    (:Authority
      (CallFunction|UpdateCloakingPreperation DeltaSeconds))
    (:Remote
      _))
  (CallFunction|UpdateSelectedThrowable)
  ;[1 1 1] Don't ask...
  (CallFunction|UpdateThirdPersonHealthBar)
  (CallFunction|UpdateThirdPersonShieldBar))

(event Input|ActionEvents|InputActionJump
  (params (Key :type Key%20Structure :default "None"))
  ;[0 0 0] Override movement and shooting to cancel cloaking
  (:Pressed
    (CallFunction|CancelCloaking)
    (Character|Jump)))

(event Input|ActionEvents|InputActionPrimaryFire
  (params (Key :type Key%20Structure :default "None"))
  (bind _currentlyusedweapon (Variables|Default|GetCurrentlyUsedWeapon))
  ;[0 0 0] Override movement and shooting to cancel cloaking
  (:Pressed
    (if (not (or (Variables|Default|GetSwitchingWeapon) (Variables|Default|GetWeaponUseBlocked)))
      (CallFunction|CancelCloaking)
      (Class|WeaponBPI|StartAttacking(Message) _currentlyusedweapon)))
  (:Released
    (Class|WeaponBPI|StopAttacking(Message) _currentlyusedweapon)))

(event Input|ActionEvents|InputActionSecondaryFire
  (params (Key :type Key%20Structure :default "None"))
  (:Pressed
    (CallFunction|Scope))
  (:Released
    (CallFunction|Unscope)))

(event Input|ActionEvents|InputActionAbility2
  (params (Key :type Key%20Structure :default "None"))
  (:Pressed
    (CallFunction|UseAbility (Variables|Default|GetGhostTeleportAbility))))

(event Input|ActionEvents|InputActionAbility1
  (params (Key :type Key%20Structure :default "None"))
  (:Pressed
    (CallFunction|UseAbility (Variables|Default|GetGhostFakeAbility))))

(event Input|ActionEvents|InputActionUltimate
  (params (Key :type Key%20Structure :default "None"))
  (:Pressed
    (Default|CallUltimate (Variables|Default|GetGhostUltimate))))

(event Input|ActionEvents|InputActionCrouch
  (params (Key :type Key%20Structure :default "None"))
  ;[0 0 0] Override movement and shooting to cancel cloaking
  (:Pressed
    (CallFunction|CancelCloaking)
    (Character|Crouch))
  (:Released
    (CallFunction|CancelCloaking)
    (Character|UnCrouch)))

(event Input|ActionEvents|InputActionAbility3
  (params (Key :type Key%20Structure :default "None"))
  (:Pressed
    (CallFunction|UseAbility (Variables|Default|GetGhostSmokeAbility))))

(event Input|AxisEvents|InputAxisMoveForwards/Backwards
  (params (AxisValue :type Float%20%28single-precision%29))
  ;[0 0 0] Override movement and shooting to cancel cloaking
  (if (!= AxisValue 0.0)
    (CallFunction|CancelCloaking))
  (Pawn|Input|AddMovementInput (Math|Vector|GetForwardVector (Variables|Default|GetCamera)) AxisValue false))

(event Input|AxisEvents|InputAxisMoveRight/Left
  (params (AxisValue :type Float%20%28single-precision%29))
  ;[0 0 0] Override movement and shooting to cancel cloaking
  (if (!= AxisValue 0.0)
    (CallFunction|CancelCloaking))
  (Pawn|Input|AddMovementInput (Math|Vector|GetRightVector (Variables|Default|GetCamera)) AxisValue false))

(fn ConstructionScript
  (|CallParentFunction))

(fn InitializeWeapons
  (bind _primaryweapon (Variables|Default|GetPrimaryWeapon))
  (Default|SetUpHitscan (Variables|Default|GetPrimaryHitscanFunctionality) self)
  (Default|SetUpWeapon (Variables|Default|GetPrimaryWeapon) self (Variables|Default|GetPrimaryHitscanFunctionality) "/Game/Blueprints/Weapons/WeaponModelBlueprints/GhostPistolModel_BP.GhostPistolModel_BP_C")
  (Variables|Default|SetCurrentlyUsedWeapon _primaryweapon)
  (Utilities|Array|Add (Variables|Default|GetAllWeapons) _primaryweapon)
  (Default|SetUpHitscan (Variables|Default|GetUltimateHitscanFunctionality) self)
  (Default|SetUpUltimateWeapon (Variables|Default|GetUltimateWeapon) self (Variables|Default|GetUltimateHitscanFunctionality) (Variables|Default|GetGhostUltimate) "/Game/Blueprints/Weapons/WeaponModelBlueprints/GhostUltModel_BP.GhostUltModel_BP_C")
  (|CallParentFunction))

(fn InitializeAbilities
  (|CallParentFunction)
  (Default|SetUpAbility (Variables|Default|GetGhostFakeAbility) self)
  (Default|SetUpAbility (Variables|Default|GetGhostSmokeAbility) self)
  (Default|SetUpAbility (Variables|Default|GetGhostTeleportAbility) self)
  (Default|SetUpUltimate (Variables|Default|GetGhostUltimate) self))

(fn SetUpHUDs
  (params (HUD :type Base%20HUD%20WBP%20Object%20Reference) (ScopeHUD :type Scope%20WBP%20Object%20Reference) (AbilityHUD :type User%20Widget%20Object%20Reference))
  (|CallParentFunction HUD ScopeHUD AbilityHUD)
  (bind _asghost_ability_hud_wbp (Utilities|Casting|CastToGhostAbilityHUD_WBP AbilityHUD)
    (:then
      (bind _output_get (Variables|Default|SetAbilityHUD _asghost_ability_hud_wbp))
      (Default|InitializeAbilityHUD _output_get (Variables|Default|GetGhostTeleportAbility) (Variables|Default|GetGhostFakeAbility) (Variables|Default|GetGhostSmokeAbility) (Variables|Default|GetGhostUltimate) (Variables|Default|GetMaxCloakingPreperationTime)))
    (:CastFailed
      (Development|PrintString "Ghost: received wrong/no abilityHUD" true true "(R=1.000000,G=0.000000,B=0.041613,A=1.000000)" 1e+01))))

(fn UpdateValuesinHUDs
  (bind _returnvalue (Class|InputSettings|GetInputSettings))
  (|CallParentFunction)
  (Default|UpdateAbilityHUD (Variables|Default|GetAbilityHUD) (Variables|Default|GetGhostTeleportAbility) (.key (Utilities|Array|Get(acopy) (Class|InputSettings|GetActionMappingbyName _returnvalue "Ability2"))) (Variables|Default|GetGhostFakeAbility) (.key (Utilities|Array|Get(acopy) (Class|InputSettings|GetActionMappingbyName _returnvalue "Ability1"))) (Variables|Default|GetGhostSmokeAbility) (.key (Utilities|Array|Get(acopy) (Class|InputSettings|GetActionMappingbyName _returnvalue "Ability3"))) (Variables|Default|GetGhostUltimate) (.key (Utilities|Array|Get(acopy) (Class|InputSettings|GetActionMappingbyName _returnvalue "Ultimate"))) (Variables|Default|GetCloaked) (Variables|Default|GetCurrentCloakingPreperationTime)))

(fn UpdateSelectedThrowable
  (bind _camera (Variables|Default|GetCamera))
  (bind _returnvalue (Transformation|GetWorldLocation _camera))
  (bind _outhits (Collision|MultiLineTraceByChannel _returnvalue (+ _returnvalue (* (Math|Vector|GetForwardVector _camera) (Variables|Default|GetMaxAbilityActivationRange))) "TraceTypeQuery3" false 0 "None"))
  (for _array_element _outhits
    (bind _asghost_throwable_bp (Utilities|Casting|CastToGhostThrowable_BP (.HitActor (Collision|BreakHitResult _array_element))))
    (if (and (== (Variables|/Game/Blueprints/Interactables/Projectiles/BaseThrowable_BP.BaseThrowable_BP_C|GetOwningCharacter _asghost_throwable_bp) self) (Variables|/Game/Blueprints/Interactables/Projectiles/GhostThrowable_BP.GhostThrowable_BP_C|GetReadyForActivation _asghost_throwable_bp))
      (if (< (Math|Vector|GetPointDistancetoLine (Transformation|GetActorLocation (.HitActor (Collision|BreakHitResult _array_element))) (.TraceStart (Collision|BreakHitResult _array_element)) (- (.TraceEnd (Collision|BreakHitResult _array_element)) (.TraceStart (Collision|BreakHitResult _array_element)))) (LocalVariables|GetClosestDistance))
        (LocalVariables|SetClosestDistance (Math|Vector|GetPointDistancetoLine (Transformation|GetActorLocation (.HitActor (Collision|BreakHitResult _array_element))) (.TraceStart (Collision|BreakHitResult _array_element)) (- (.TraceEnd (Collision|BreakHitResult _array_element)) (.TraceStart (Collision|BreakHitResult _array_element)))))
        (LocalVariables|SetClosestThrowable _asghost_throwable_bp))))
  (if (!= (LocalVariables|GetClosestThrowable) (Variables|Default|GetSelectedThrowable))
    (Utilities|IsValid (Variables|Default|GetSelectedThrowable)
      (:Is%20Valid
        (Default|Deselect (Variables|Default|GetSelectedThrowable)))
      (:Is%20Not%20Valid
        _))
    (bind _output_get (Variables|Default|SetSelectedThrowable (LocalVariables|GetClosestThrowable)))
    (Utilities|IsValid _output_get
      (:Is%20Valid
        (Default|Select _output_get)))))

(fn SwitchtoWeapon
  (params (WeaponIndex :type Integer) (ForceSwitch :type Boolean))
  (bind _currentlyusedweapon (Variables|Default|GetCurrentlyUsedWeapon))
  (bind _allweapons (Variables|Default|GetAllWeapons))
  (if (Math|Boolean|ANDBoolean (or ForceSwitch (!= WeaponIndex (Utilities|Array|FindItem _allweapons (Variables|Default|GetCurrentlyUsedWeapon)))) (>= WeaponIndex 0) (< WeaponIndex (Utilities|Array|Length _allweapons)))
    (Variables|Default|SetSwitchedToWeapon (Utilities|Array|Get(acopy) (Variables|Default|GetAllWeapons) WeaponIndex))
    (CallFunction|Unscope)
    (Class|WeaponBPI|StopAttacking(Message) _currentlyusedweapon)
    (Class|WeaponBPI|CancelReloading(Message) _currentlyusedweapon)
    (Class|WeaponBPI|ResetRecoil(Message) _currentlyusedweapon)
    (Class|WeaponBPI|HideWeaponModel(Message) _currentlyusedweapon)
    (CallFunction|HideAllOtherWeaponModels WeaponIndex)
    (CallFunction|ServerSetSwitchingWeapon true)
    (CallFunction|WaitandEquipWeapon WeaponIndex (Variables|Default|GetWeaponSwitchDuration))))

(fn CancelCloaking
  (if (Variables|Default|GetCloaked)
    (CallFunction|ServerDecloak)
    (else
      (CallFunction|ServerSetCurrentCloakingPreperationTime 0.0))))

(fn UpdateCloakingPreperation
  (params (DeltaSeconds :type Float%20%28double-precision%29))
  (if (not (Variables|Default|GetCloaked))
    (bind _output_get (Variables|Default|SetCurrentCloakingPreperationTime (+ DeltaSeconds (Variables|Default|GetCurrentCloakingPreperationTime))))
    (if (>= _output_get (Variables|Default|GetMaxCloakingPreperationTime))
      (Variables|Default|SetCurrentCloakingPreperationTime 0.0)
      (CallFunction|ServerCloak))
    (else
      (Variables|Default|SetCurrentCloakingPreperationTime 0.0))))

(fn TakeDamage
  (params (DamageValue :type Float%20%28double-precision%29) (Instigator :type Damage%20Instigator%20Structure))
  (bind _isenemydamage (CallFunction|CheckifEnemyDamage Instigator))
  (if _isenemydamage
    (CallFunction|CancelCloaking)
    (bind (_damagecaused _died) (|CallParentFunction DamageValue Instigator))
    (return _damagecaused _died)
    (else
      (return 0.0 false))))

(fn UseAbility
  (params (Ability :type Base%20Throwable%20Ability%20BP%20Object%20Reference))
  (bind _selectedthrowable (Variables|Default|GetSelectedThrowable))
  (CallFunction|UpdateSelectedThrowable)
  (Utilities|IsValid _selectedthrowable
    (:Is%20Valid
      (if (Utilities|ClassIsChildOf (Utilities|GetClass _selectedthrowable) (Variables|/Game/Blueprints/Abilities/BaseThrowableAbility_BP.BaseThrowableAbility_BP_C|GetThrowableClass Ability))
        (Default|Activate _selectedthrowable)
        (else
          (bind _wasexecuted (Default|CallAbility Ability :!label _label))
          (if _wasexecuted
            (CallFunction|CancelCloaking)))))
    (:Is%20Not%20Valid
      (goto _label))))

(fn Unscope
  (bind _currentlyusedweapon (Variables|Default|GetCurrentlyUsedWeapon))
  (bind _scopable (Class|WeaponBPI|GetScopable(Message) _currentlyusedweapon))
  (if (and _scopable (Variables|Default|GetScoped))
    (Default|HideScope (Variables|Default|GetScopeHUD))
    (if (not (Variables|Default|GetSwitchingWeapon))
      (Rendering|SetVisibility (Variables|Default|GetArmsMesh) true true))
    (Camera|SetFieldOfView (Variables|Default|GetCamera) 9e+01)
    (Class|WeaponBPI|DeactivateScopeEffects(Message) _currentlyusedweapon)
    (Variables|Default|SetScoped false)))