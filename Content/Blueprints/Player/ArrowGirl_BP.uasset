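; ArrowGirl_BP is a player Blueprint that spawns an arrow and steers it with the camera.
; Primary fire spawns an ArrowDummy, and Tick feeds it a goal point along the camera's forward vector.
; Holding primary or secondary fire moves that goal farther or nearer within limits; Reload destroys the arrow.
; A visibility trace destroys the arrow after it goes unhit for too many consecutive ticks, counted per frame rather than in seconds.
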(event EventBeginPlay
  (|CallParentFunction))

(event EventTick
  (params (DeltaSeconds :type Float%20%28single-precision%29))
  (bind _camera (Variables|Default|GetCamera))
  (|CallParentFunction 0.0)
  (if (Variables|Default|GetArrowSpawned)
    (CallFunction|UpdateArrowGoalDistance)
    (Default|SetGoal (Variables|Default|GetArrow) (+ (* (Math|Vector|GetForwardVector _camera) (Variables|Default|GetArrowGoalDistance)) (Transformation|GetWorldLocation _camera)))
    (Development|PrintString (Utilities|String|ToString(Float) (Variables|Default|GetArrowGoalDistance)))
    (CallFunction|CheckArrowView)))

(event Input|ActionEvents|InputActionPrimaryFire
  (params (Key :type Key%20Structure :default "None"))
  (:Pressed
    (Variables|Default|SetPrimaryFiring true)
    (if (not (Variables|Default|GetArrowSpawned))
      (CallFunction|SpawnArrow)))
  (:Released
    (Variables|Default|SetPrimaryFiring false)))

(event Input|ActionEvents|InputActionSecondaryFire
  (params (Key :type Key%20Structure :default "None"))
  (:Pressed
    (Variables|Default|SetSecondaryFiring true))
  (:Released
    (Variables|Default|SetSecondaryFiring false)))

(event Input|ActionEvents|InputActionReload
  (params (Key :type Key%20Structure :default "None"))
  (:Pressed
    (CallFunction|Reload)))

(fn ConstructionScript
  (|CallParentFunction))

(fn UpdateArrowGoalDistance
  (Utilities|FlowControl|Sequence
    (:then_0
      (if (Variables|Default|GetPrimaryFiring)
        (if (< (Variables|Default|GetArrowGoalDistance) (Variables|Default|GetArrowGoalMaxDistance))
          (Variables|Default|SetArrowGoalDistance (+ (Variables|Default|GetArrowGoalDistance) (Variables|Default|GetArrowGoalDistanceChangeRate))))))
    (:then_1
      (if (Variables|Default|GetSecondaryFiring)
        (if (> (Variables|Default|GetArrowGoalDistance) (Variables|Default|GetArrowGoalMinDistance))
          (Variables|Default|SetArrowGoalDistance (- (Variables|Default|GetArrowGoalDistance) (Variables|Default|GetArrowGoalDistanceChangeRate))))))))

(fn CheckArrowView
  (bind _camera (Variables|Default|GetCamera))
  (bind _returnvalue (Transformation|GetWorldLocation _camera))
  (bind _outhit (Collision|LineTraceByChannel _returnvalue (+ _returnvalue (* (Math|Vector|GetForwardVector _camera) (Variables|Default|GetArrowGoalDistance))) "TraceTypeQuery1" false 0 "None"))
  (if (!= (.HitActor (Collision|BreakHitResult _outhit)) (Variables|Default|GetArrow))
    (if (>= (Variables|Default|GetCurrentWalledTime) (Variables|Default|GetMaxWalledTime))
      (Actor|DestroyActor (Variables|Default|GetArrow))
      (Variables|Default|SetArrowSpawned false)
      (Variables|Default|SetArrowGoalDistance (Variables|Default|GetArrowGoalMinDistance))
      (Variables|Default|SetCurrentWalledTime 0.0)
      (else
        (bind _output_get (Variables|Default|SetCurrentWalledTime (+ (Variables|Default|GetCurrentWalledTime) 1.0)))))
    (Development|PrintString (Utilities|String|ToString(Float) _output_get))
    (else
      (Variables|Default|SetCurrentWalledTime 0.0))))

(fn Reload
  (Variables|Default|SetArrowGoalDistance (Variables|Default|GetArrowGoalMinDistance))
  (if (Variables|Default|GetArrowSpawned)
    (Actor|DestroyActor (Variables|Default|GetArrow))
    (Variables|Default|SetArrowSpawned false)))

(fn SpawnArrow
  (bind _camera (Variables|Default|GetCamera))
  (bind _returnvalue (Game|SpawnActorfromClass "/Game/Blueprints/Interactables/ArrowDummy.ArrowDummy_C" (Math|Conversions|ToTransform(Vector) (+ (* (Math|Vector|GetForwardVector _camera) (Variables|Default|GetArrowGoalDistance)) (Transformation|GetWorldLocation _camera))) "AlwaysSpawn" 0 0))
  (Variables|Default|SetArrow _returnvalue)
  (Variables|Default|SetArrowSpawned true))