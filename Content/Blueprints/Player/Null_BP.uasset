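; Player character Blueprint for Null, a hero with wallrunning, removal, wallhack and ultimate abilities tied to a decaying detection meter.
; Reaching maximum detection cancels the three abilities, while ultimate mode lowers the meter and alters its decay.
; Wall snapping uses two traces to teleport and reorient the capsule, leaving a shadow; on-wall movement is unwired.
; Removal redirects primary fire to a second hitscan weapon until cancelled, including on weapon switch.
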(event Custom|Server_SetMovementMode
  (params (MovementMode :type EMovementMode%20Enum :default "MOVE_None"))
  (bind _charactermovement (Variables|Character|GetCharacterMovement))
  ;[0 0 0] Server dependet Wallrunning calls
  (bind _output_get (Variables|/Script/Engine.CharacterMovementComponent|SetDefaultLandMovementMode _charactermovement MovementMode))
  (Pawn|Components|CharacterMovement|SetMovementMode _charactermovement _output_get 0))

(event Custom|Server_RotateMeshOnWall
  ;[0 0 0] Server dependet Wallrunning calls
  (Transformation|SetWorldRotation (Variables|Default|GetCapsuleComponent) (Math|Rotator|MakeRotfromZX (* (Variables|Wallrun|GetGravityDirection) (Variables|Wallrun|Get-1)) (Wallrun|GetDirectiononGravityPlane (Math|Vector|GetForwardVector (Pawn|GetControlRotation :!class /Script/Engine.Pawn)))) false false))

(event Custom|Server_SetGravityDirection
  (params (GravityDirection :type Vector))
  ;[0 0 0] Server dependet Wallrunning calls
  (Variables|Wallrun|SetGravityDirection GravityDirection))

(event Custom|Server_SetRotation
  (params (Rotation :type Rotator))
  ;[0 0 0] Server dependet Wallrunning calls
  (Transformation|SetWorldRotation (Variables|Default|GetCapsuleComponent) Rotation false false))

(event Custom|Server_SetWorldLocation
  (params (Location :type Vector))
  ;[0 0 0] Server dependet Wallrunning calls
  (Transformation|SetWorldLocation (Variables|Default|GetCapsuleComponent) Location false true))

(event Custom|Server_SetUseControllerRotationYaw
  (params (UseControlRotationYaw :type Boolean))
  ;[0 0 0] Server dependet Wallrunning calls
  (Variables|Default|SetbUseControllerRotationYaw UseControlRotationYaw))

(event Custom|Client_CancelWallhack
  (Default|CancelAbility (Variables|Default|GetNullWallhackAbility)))

(event Custom|Server_SpawnTeleportShadow
  (bind _self self)
  ;[0 0 0] Server dependet Wallrunning calls
  (Game|SpawnActorfromClass "/Game/Blueprints/Visuals/Effects/NullTeleportShadow_BP.NullTeleportShadow_BP_C" (Transformation|GetWorldTransform (Variables|Character|GetMesh)) "AlwaysSpawn" _self _self _self))

(event EventBeginPlay
  (|CallParentFunction)
  (Variables|Detection|SetCurrentDetectionDecayRate (Variables|Detection|GetBaseDetectionDecayRate)))

(event EventTick
  (params (DeltaSeconds :type Float%20%28single-precision%29))
  (|CallParentFunction DeltaSeconds)
  (Detection|UpdateDetection DeltaSeconds)
  ;[1 1 1] Don't ask...
  (CallFunction|UpdateThirdPersonHealthBar)
  (CallFunction|UpdateThirdPersonShieldBar))

(event Input|ActionEvents|InputActionJump
  (params (Key :type Key%20Structure))
  (:Pressed
    (if (Variables|Wallrun|GetWallrunningMode)
      (Wallrun|DeactivateWallrunningMode)
      (else
        (Character|Jump)))))

(event Input|ActionEvents|InputActionPrimaryFire
  (params (Key :type Key%20Structure))
  (bind _currentlyusedweapon (Variables|Default|GetCurrentlyUsedWeapon))
  (bind _primaryweapon (Variables|Default|GetPrimaryWeapon))
  (bind _currentlyusedweapon_2 (Variables|Default|GetCurrentlyUsedWeapon))
  (bind _returnvalue (== _currentlyusedweapon_2 _primaryweapon))
  ;[0 0 0] Firing Logic including removal
  (:Pressed
    (if (not (or (Variables|Default|GetSwitchingWeapon) (Variables|Default|GetWeaponUseBlocked)))
      (if _returnvalue
        (if (Variables|Default|GetRemoval)
          (Class|WeaponBPI|StartAttacking(Message) (Variables|Default|GetRemovalPrimaryWeapon))
          (else
            (Class|WeaponBPI|StartAttacking(Message) _currentlyusedweapon :!label _label)))
        (else
          (goto _label)))))
  (:Released
    (if _returnvalue
      (Class|WeaponBPI|StopAttacking(Message) _currentlyusedweapon)
      (Class|WeaponBPI|StopAttacking(Message) (Variables|Default|GetRemovalPrimaryWeapon))
      (else
        (Class|WeaponBPI|StopAttacking(Message) _currentlyusedweapon)))))

(event Input|ActionEvents|InputActionReload
  (params (Key :type Key%20Structure))
  (bind _currentlyusedweapon (Variables|Default|GetCurrentlyUsedWeapon))
  ;[0 0 0] Firing Logic including removal
  (:Pressed
    (if (not (Math|Boolean|ORBoolean (Variables|Default|GetRemoval) (Variables|Default|GetSwitchingWeapon) (Variables|Default|GetWeaponUseBlocked)))
      (Class|WeaponBPI|StopAttacking(Message) _currentlyusedweapon)
      (Class|WeaponBPI|Reload(Message) _currentlyusedweapon))))

(event Input|ActionEvents|InputActionAbility2
  (params (Key :type Key%20Structure))
  (:Pressed
    (Default|CallAbility (Variables|Default|GetNullWallrunningAbility))))

(event Input|ActionEvents|InputActionAbility1
  (params (Key :type Key%20Structure))
  (:Pressed
    (if (== (Variables|Default|GetCurrentlyUsedWeapon) (Variables|Default|GetPrimaryWeapon))
      (Default|CallAbility (Variables|Default|GetNullRemovalAbility)))))

(event Input|ActionEvents|InputActionUltimate
  (params (Key :type Key%20Structure))
  (:Pressed
    (Default|CallUltimate (Variables|Default|GetNullUltimate))))

(event Input|ActionEvents|InputActionSecondaryFire
  (params (Key :type Key%20Structure)))

(event Input|ActionEvents|InputActionAbility3
  (params (Key :type Key%20Structure))
  (:Pressed
    (Default|CallAbility (Variables|Default|GetNullWallhackAbility))))

(event Input|AxisEvents|InputAxisLookRight/Left
  (params (AxisValue :type Float%20%28single-precision%29))
  (Pawn|Input|AddControllerYawInput (* AxisValue (Variables|/Game/Blueprints/Framework/PlayerController1_BP.PlayerController1_BP_C|GetMouseSensitivity (Variables|Default|GetPlayerControllerReference))))
  (if (Variables|Wallrun|GetWallrunningMode)
    (CallFunction|ServerRotateMeshonWall)))

(event Input|AxisEvents|InputAxisLookUp/Down
  (params (AxisValue :type Float%20%28single-precision%29))
  (Pawn|Input|AddControllerPitchInput (* AxisValue (Variables|/Game/Blueprints/Framework/PlayerController1_BP.PlayerController1_BP_C|GetMouseSensitivity (Variables|Default|GetPlayerControllerReference))))
  (if (Variables|Wallrun|GetWallrunningMode)
    (CallFunction|ServerRotateMeshonWall)))

(event Input|AxisEvents|InputAxisMoveForwards/Backwards
  (params (AxisValue :type Float%20%28single-precision%29))
  (if (not (Variables|Wallrun|GetWallrunningMode))
    (Pawn|Input|AddMovementInput (Math|Vector|GetForwardVector (Variables|Default|GetCamera)) AxisValue false)))

(event Input|AxisEvents|InputAxisMoveRight/Left
  (params (AxisValue :type Float%20%28single-precision%29))
  (if (not (Variables|Wallrun|GetWallrunningMode))
    (Pawn|Input|AddMovementInput (Math|Vector|GetRightVector (Variables|Default|GetCamera)) AxisValue false)))

(fn ConstructionScript
  (|CallParentFunction))

(fn GainDetection
  (params (Detection :type Float%20%28double-precision%29))
  (Variables|Detection|SetCurrentDetection (+ Detection (Variables|Detection|GetCurrentDetection))))

(fn UpdateDetection
  (params (DeltaTime :type Float%20%28double-precision%29))
  (if (> (Variables|Detection|GetCurrentDetection) 0.0)
    (if (>= (Variables|Detection|GetCurrentDetection) (Variables|Detection|GetMaxDetection))
      (Detection|CancelAllAbilities))
    (bind _output_get (Variables|Detection|SetCurrentDetection (- (Variables|Detection|GetCurrentDetection) (* DeltaTime (Variables|Detection|GetCurrentDetectionDecayRate)))))
    (if (< _output_get 0.0)
      (Variables|Detection|SetCurrentDetection 0.0))))

(fn CheckifDetectionAvailable
  (params (Detection :type Float%20%28double-precision%29))
  (return (> (Variables|Detection|GetMaxDetection) (+ Detection (Variables|Detection|GetCurrentDetection)))))

(fn CancelAllAbilities
  (Wallrun|DeactivateWallrunningMode)
  (Default|CancelAbility (Variables|Default|GetNullRemovalAbility))
  (Default|CancelAbility (Variables|Default|GetNullWallhackAbility)))

(fn InitializeAbilities
  (|CallParentFunction)
  (Default|SetUpAbility (Variables|Default|GetNullWallrunningAbility) self)
  (Default|SetUpAbility (Variables|Default|GetNullRemovalAbility) self)
  (Default|SetUpAbility (Variables|Default|GetNullWallhackAbility) self)
  (Default|SetUpUltimate (Variables|Default|GetNullUltimate) self))

(fn InitializeWeapons
  (bind _primaryweapon (Variables|Default|GetPrimaryWeapon))
  (Default|SetUpHitscan (Variables|Default|GetPrimaryShootingFunctionality) self)
  (Default|SetUpWeapon (Variables|Default|GetPrimaryWeapon) self (Variables|Default|GetPrimaryShootingFunctionality) "/Game/Blueprints/Weapons/WeaponModelBlueprints/NullGunModel_BP.NullGunModel_BP_C")
  (Variables|Default|SetCurrentlyUsedWeapon _primaryweapon)
  (Utilities|Array|Add (Variables|Default|GetAllWeapons) _primaryweapon)
  (|CallParentFunction)
  (Default|SetUpHitscan (Variables|Default|GetRemovalPrimaryShootingFunctionality) self)
  (Default|SetUpWeapon (Variables|Default|GetRemovalPrimaryWeapon) self (Variables|Default|GetRemovalPrimaryShootingFunctionality) "/Game/Blueprints/Weapons/WeaponModelBlueprints/NullGunModel_BP.NullGunModel_BP_C"))

(fn SetUpHUDs
  (params (HUD :type Base%20HUD%20WBP%20Object%20Reference) (ScopeHUD :type Scope%20WBP%20Object%20Reference) (AbilityHUD :type User%20Widget%20Object%20Reference))
  (|CallParentFunction HUD ScopeHUD AbilityHUD)
  (bind _asnull_ability_hud_wbp (Utilities|Casting|CastToNullAbilityHUD_WBP AbilityHUD)
    (:then
      (bind _output_get (Variables|Default|SetAbilityHUD _asnull_ability_hud_wbp))
      (Default|InitializeAbilityHUD _output_get (Variables|Default|GetNullWallrunningAbility) (Variables|Default|GetNullRemovalAbility) (Variables|Default|GetNullWallhackAbility) (Variables|Default|GetNullUltimate) (Variables|Detection|GetMaxDetection)))
    (:CastFailed
      (Development|PrintString "Null: received wrong/no abilityHUD" true true "(R=1.000000,G=0.000000,B=0.041613,A=1.000000)" 1e+01))))

(fn UpdateValuesinHUDs
  (bind _returnvalue (Class|InputSettings|GetInputSettings))
  (|CallParentFunction)
  (Default|UpdateAbilityHUD (Variables|Default|GetAbilityHUD) (Variables|Default|GetNullWallrunningAbility) (.key (Utilities|Array|Get(acopy) (Class|InputSettings|GetActionMappingbyName _returnvalue "Ability2"))) (Variables|Default|GetNullRemovalAbility) (.key (Utilities|Array|Get(acopy) (Class|InputSettings|GetActionMappingbyName _returnvalue "Ability1"))) (Variables|Default|GetNullWallhackAbility) (.key (Utilities|Array|Get(acopy) (Class|InputSettings|GetActionMappingbyName _returnvalue "Ability3"))) (Variables|Default|GetNullUltimate) (.key (Utilities|Array|Get(acopy) (Class|InputSettings|GetActionMappingbyName _returnvalue "Ultimate"))) (Variables|Detection|GetCurrentDetection)))

(fn ActivateWallrunningMode
  (Variables|Wallrun|SetWallrunningMode true)
  (CallFunction|ServerSetMovementMode "MOVE_Flying")
  (Variables|Default|SetbUseControllerRotationYaw false)
  (CallFunction|ServerSetUseControllerRotationYaw false)
  (CallFunction|ServerSetGravityDirection (Math|Vector|VectorDown)))

(fn DeactivateWallrunningMode
  (Variables|Wallrun|SetWallrunningMode false)
  (CallFunction|ServerSetMovementMode "MOVE_Walking")
  (Variables|Default|SetbUseControllerRotationYaw true)
  (CallFunction|ServerSetUseControllerRotationYaw true)
  (CallFunction|ServerSetGravityDirection (Math|Vector|VectorDown))
  (CallFunction|ServerRotateMeshonWall))

(fn MoveonWall
  (params (WorldDirection :type Vector) (ScaleValue :type Float%20%28double-precision%29))
  (bind _directiononplane (Wallrun|GetDirectiononGravityPlane WorldDirection))
  (if (!= ScaleValue 0.0)
    (if (Wallrun|CheckifDirectionWalkableGround (* _directiononplane ScaleValue))
      (Pawn|Input|AddMovementInput _directiononplane ScaleValue false)
      (else
        (Development|PrintString "Cant move")))))

(fn GetDirectiononGravityPlane
  (params (Direction :type Vector))
  (bind _gravitydirection (Variables|Wallrun|GetGravityDirection))
  (return (Math|Vector|Normalize (- Direction (* (/ (Math|Vector|DotProduct Direction _gravitydirection) (Math|Vector|DotProduct _gravitydirection _gravitydirection)) (Variables|Wallrun|GetGravityDirection))))))

(fn SnaptoNewWall
  (bind (_wallhit _hit1 _hit2) (Wallrun|CheckforNewWall))
  (if _wallhit
    (CallFunction|ServerSpawnTeleportShadow)
    (Wallrun|ActivateWallrunningMode)
    (Components|Movement|StopMovementImmediately (Variables|Character|GetCharacterMovement))
    (CallFunction|ServerSetRotation (Math|Rotator|MakeRotfromZX (.Normal (Collision|BreakHitResult _hit2)) (Math|Vector|Normalize (- (.Location (Collision|BreakHitResult _hit1)) (.Location (Collision|BreakHitResult _hit2))))))
    (CallFunction|ServerSetGravityDirection (* (.Normal (Collision|BreakHitResult _hit2)) (Variables|Wallrun|Get-1)))
    (CallFunction|ServerSetWorldLocation (+ (.Location (Collision|BreakHitResult _hit2)) (* (.Normal (Collision|BreakHitResult _hit2)) (Variables|Wallrun|GetDistanceToFeet))))
    (if (Utilities|Operators|EqualEqual (* (.Normal (Collision|BreakHitResult _hit2)) (Variables|Wallrun|Get-1)) (Math|Vector|VectorDown) 0.7)
      (Wallrun|DeactivateWallrunningMode))
    (return true)
    (else
      (return false))))

(fn CheckifDirectionWalkableGround
  (params (Direction :type Vector))
  (bind _returnvalue (Math|Vector|Normalize Direction))
  (bind _returnvalue_2 (Transformation|GetActorLocation))
  (bind _wallchecksverticaldistance (Variables|Wallrun|GetWallChecksVerticalDistance))
  (bind _returnvalue_3 (* _returnvalue _wallchecksverticaldistance))
  (bind _returnvalue_4 (+ _returnvalue_2 _returnvalue_3))
  (bind _returnvalue_5 (Collision|LineTraceByChannel _returnvalue_4 (+ _returnvalue_4 (* (Variables|Wallrun|GetGravityDirection) (Variables|Wallrun|GetDistanceToFeet))) "TraceTypeQuery1" false 0 "None" false "(R=1.000000,G=0.000000,B=0.000000,A=1.000000)" "(R=0.000000,G=1.000000,B=0.000000,A=1.000000)" 3.0))
  (return _returnvalue_5))

(fn ActivateRemoval
  (bind _primaryweapon (Variables|Default|GetPrimaryWeapon))
  (Variables|Default|SetRemoval true)
  (Variables|/Game/Blueprints/Weapons/HitscanWeapon.HitscanWeapon_C|SetInflictedRecoil _primaryweapon "")
  (Variables|/Game/Blueprints/Weapons/HitscanWeapon.HitscanWeapon_C|SetCurrentRecoilPatternPosition _primaryweapon 0)
  (if (Variables|/Game/Blueprints/Weapons/HitscanWeapon.HitscanWeapon_C|GetAttacking _primaryweapon)
    (Class|WeaponBPI|StartAttacking(Message) (Variables|Default|GetRemovalPrimaryWeapon)))
  (Class|WeaponBPI|StopAttacking(Message) (Variables|Default|GetPrimaryWeapon)))

(fn DeactivateRemoval
  (Variables|Default|SetRemoval false)
  (if (Variables|/Game/Blueprints/Weapons/HitscanWeapon.HitscanWeapon_C|GetAttacking (Variables|Default|GetRemovalPrimaryWeapon))
    (Class|WeaponBPI|StartAttacking(Message) (Variables|Default|GetPrimaryWeapon)))
  (Class|WeaponBPI|StopAttacking(Message) (Variables|Default|GetRemovalPrimaryWeapon)))

(fn SwitchtoWeapon
  (params (WeaponIndex :type Integer) (ForceSwitch :type Boolean))
  (bind _currentlyusedweapon (Variables|Default|GetCurrentlyUsedWeapon))
  (bind _allweapons (Variables|Default|GetAllWeapons))
  (if (Math|Boolean|ANDBoolean (or ForceSwitch (!= WeaponIndex (Utilities|Array|FindItem _allweapons (Variables|Default|GetCurrentlyUsedWeapon)))) (>= WeaponIndex 0) (< WeaponIndex (Utilities|Array|Length _allweapons)))
    (if (Variables|Default|GetRemoval)
      (Default|CancelAbility (Variables|Default|GetNullRemovalAbility)))
    (Variables|Default|SetSwitchedToWeapon (Utilities|Array|Get(acopy) (Variables|Default|GetAllWeapons) WeaponIndex))
    (CallFunction|Unscope)
    (Class|WeaponBPI|StopAttacking(Message) _currentlyusedweapon)
    (Class|WeaponBPI|CancelReloading(Message) _currentlyusedweapon)
    (Class|WeaponBPI|ResetRecoil(Message) _currentlyusedweapon)
    (Class|WeaponBPI|HideWeaponModel(Message) _currentlyusedweapon)
    (CallFunction|HideAllOtherWeaponModels WeaponIndex)
    (Variables|Default|SetSwitchingWeapon true)
    (CallFunction|WaitandEquipWeapon WeaponIndex (Variables|Default|GetWeaponSwitchDuration))))

(fn StartUltimateDetectionMode
  (Variables|Detection|SetCurrentDetectionDecayRate (* (Variables|Detection|GetBaseDetectionDecayRate) (Variables|Detection|GetUltimateDetectionDecayReduction)))
  (if (> (Variables|Detection|GetCurrentDetection) (* (Variables|Detection|GetMaxDetection) (Variables|Detection|GetUltimateDetectionInitialReduction)))
    (Variables|Detection|SetCurrentDetection (- (Variables|Detection|GetCurrentDetection) (* (Variables|Detection|GetMaxDetection) (Variables|Detection|GetUltimateDetectionInitialReduction))))
    (else
      (Variables|Detection|SetCurrentDetection 0.0))))

(fn EndUltimateDetectionMode
  (Variables|Detection|SetCurrentDetectionDecayRate (Variables|Detection|GetBaseDetectionDecayRate)))

(fn CheckforNewWall
  (bind _returnvalue (Pawn|GetControlRotation :!class /Script/Engine.Pawn))
  (bind _returnvalue_2 (Transformation|GetActorLocation))
  (bind _returnvalue_3 (Transformation|GetActorLocation))
  (bind _wallchecksverticaldistance (Variables|Wallrun|GetWallChecksVerticalDistance))
  (bind _returnvalue_4 (Math|Vector|GetUpVector _returnvalue))
  (bind _returnvalue_5 (* _returnvalue_4 _wallchecksverticaldistance))
  (bind _returnvalue_6 (+ _returnvalue_3 _returnvalue_5))
  (LocalVariables|SetForwardCheckVector (* (Math|Vector|GetForwardVector (Pawn|GetControlRotation :!class /Script/Engine.Pawn)) (Variables|Wallrun|GetWallCheckRange)))
  (bind (_outhit _returnvalue_7) (Collision|LineTraceByChannel _returnvalue_2 (+ _returnvalue_2 (LocalVariables|GetForwardCheckVector)) "TraceTypeQuery1" false 0 "None" true "(R=1.000000,G=0.000000,B=0.000000,A=1.000000)" "(R=0.000000,G=1.000000,B=0.000000,A=1.000000)" 2.0))
  (bind (_outhit_2 _returnvalue_8) (Collision|LineTraceByChannel _returnvalue_6 (+ _returnvalue_6 (LocalVariables|GetForwardCheckVector)) "TraceTypeQuery1" false 0 "None" true "(R=1.000000,G=0.000000,B=0.000000,A=1.000000)" "(R=0.000000,G=1.000000,B=0.000000,A=1.000000)" 2.0))
  (return (and _returnvalue_7 _returnvalue_8) _outhit _outhit_2))

(fn PlayNewWallEffects
  (bind _self self)
  (Game|SpawnActorfromClass "/Game/Blueprints/Visuals/Effects/NullTeleportShadow_BP.NullTeleportShadow_BP_C" (Transformation|GetWorldTransform (Variables|Character|GetMesh)) "AlwaysSpawn" _self _self _self))