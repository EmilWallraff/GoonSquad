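; Base ultimate ability Blueprint that manages activation and timed expiry of a character's ultimate.
; CallUltimate checks charge on the owner's PlayerState, runs the empty ExecuteUltimateAction hook, plays a voiceline and starts the ult state through server events.
; Tick counts duration until EndUltimate resets it, runs TerminateUltimateAction and ends that state.
; On BeginPlay it retries every 0.1 seconds until the owner is valid, then clears any leftover ult state.
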(event Custom|Server_StartUltState
  (Default|StartUltState (Variables|/Game/Blueprints/Player/BaseCharacter_BP.BaseCharacter_BP_C|GetPlayerStateReference (Variables|Default|GetOwningCharacter))))

(event Custom|CancelLastRoundUlt
  (Utilities|IsValid (Variables|Default|GetOwningCharacter)
    (:Is%20Valid
      (CallFunction|ServerEndUltState))
    (:Is%20Not%20Valid
      (Utilities|Time|SetTimerbyEvent (delegate Custom|CancelLastRoundUlt) 0.1))))

(event Custom|Server_EndUltState
  (Default|EndUltState (Variables|/Game/Blueprints/Player/BaseCharacter_BP.BaseCharacter_BP_C|GetPlayerStateReference (Variables|Default|GetOwningCharacter))))

(event EventTick
  (params (DeltaSeconds :type Float%20%28single-precision%29))
  (if (Variables|Default|GetActivated)
    (bind _output_get (Variables|Default|SetCurrentDuration (+ (Variables|Default|GetCurrentDuration) DeltaSeconds)))
    (if (>= _output_get (Variables|Default|GetMaxDuration))
      (Public|EndUltimate))))

(event EventBeginPlay
  (CallFunction|CancelLastRoundUlt))

(fn ExecuteUltimateAction)

(fn TerminateUltimateAction)

(fn CheckifUsable
  (return (and (not (Variables|Default|GetActivated)) (>= (CallFunction|GetCurrentUltimateCharge) (Variables|Default|GetRequiredUltimateCharge)))))

(fn CallUltimate
  (bind _usable (Protected|CheckifUsable))
  (if _usable
    (Variables|Default|SetActivated true)
    (Protected|ExecuteUltimateAction)
    (Default|PlayVoiceline (Variables|Default|GetOwningCharacter) "NewEnumerator0" true)
    (CallFunction|ServerStartUltState)
    (return true)
    (else
      (return false))))

(fn EndUltimate
  (if (Variables|Default|GetActivated)
    (Variables|Default|SetActivated false)
    (Variables|Default|SetCurrentDuration 0.0)
    (Protected|TerminateUltimateAction)
    (CallFunction|ServerEndUltState)
    (else
      (return))))

(fn SetUpUltimate
  (params (Character :type Base%20Character%20BP%20Object%20Reference))
  (Variables|Default|SetOwningCharacter Character))

(fn GetCurrentUltimateCharge
  (return (Default|GetUltimateCharge (Variables|/Game/Blueprints/Player/BaseCharacter_BP.BaseCharacter_BP_C|GetPlayerStateReference (Variables|Default|GetOwningCharacter)))))