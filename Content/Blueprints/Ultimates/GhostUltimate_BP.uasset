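; Ultimate ability Blueprint for the Ghost character that switches its ultimate weapon on and off.
; Overrides of the execute and terminate ultimate actions call the parent, then cast the owning character to Ghost_BP to activate or deactivate that weapon.
; A failed cast prints a wrong-character message.
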(event EventBeginPlay
  (|CallParentFunction) ; This node is disabled and will not be called.\nDrag off pins to build functionality.
)

(event EventTick
  (params (DeltaSeconds :type Float%20%28single-precision%29))
  (|CallParentFunction DeltaSeconds) ; This node is disabled and will not be called.\nDrag off pins to build functionality.
)

(fn TerminateUltimateAction
  (|CallParentFunction)
  (bind _asghost_bp (Utilities|Casting|CastToGhost_BP (Variables|Default|GetOwningCharacter))
    (:then
      (Default|DeactivateWeapon _asghost_bp (Variables|/Game/Blueprints/Player/Ghost_BP.Ghost_BP_C|GetUltimateWeapon _asghost_bp)))
    (:CastFailed
      (Development|PrintString "Ghost Ultimate used on wrong character" true true "(R=1.000000,G=0.000000,B=0.009241,A=1.000000)" 1e+01))))

(fn ExecuteUltimateAction
  (|CallParentFunction)
  (bind _asghost_bp (Utilities|Casting|CastToGhost_BP (Variables|Default|GetOwningCharacter))
    (:then
      (Default|ActivateWeapon _asghost_bp (Variables|/Game/Blueprints/Player/Ghost_BP.Ghost_BP_C|GetUltimateWeapon _asghost_bp)))
    (:CastFailed
      (Development|PrintString "Ghost Ultimate used on wrong character" true true "(R=1.000000,G=0.000000,B=0.009241,A=1.000000)" 1e+01))))