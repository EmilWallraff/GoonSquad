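; Morbius's ultimate ability, which switches the character into an ultimate form with claw weapons while active.
; It overrides the execute and terminate actions of its parent ultimate, casting the owning character to Morbius_BP.
; Execute activates the UltimateClaws weapon and enables the ult form, and terminate reverses both.
; A failed cast only prints a wrong-character message.
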(event EventBeginPlay)

(event EventTick
  (params (DeltaSeconds :type Float%20%28single-precision%29)))

(fn ExecuteUltimateAction
  (|CallParentFunction)
  (bind _asmorbius_bp (Utilities|Casting|CastToMorbius_BP (Variables|Default|GetOwningCharacter))
    (:then
      (Default|ActivateWeapon _asmorbius_bp (Variables|/Game/Blueprints/Player/Morbius_BP.Morbius_BP_C|GetUltimateClaws _asmorbius_bp))
      (Default|ToggleUltForm _asmorbius_bp true))
    (:CastFailed
      (Development|PrintString "Morbius Ultimate used on wrong character" true true "(R=1.000000,G=0.000000,B=0.009241,A=1.000000)" 1e+01))))

(fn TerminateUltimateAction
  (|CallParentFunction)
  (bind _asmorbius_bp (Utilities|Casting|CastToMorbius_BP (Variables|Default|GetOwningCharacter))
    (:then
      (Default|DeactivateWeapon _asmorbius_bp (Variables|/Game/Blueprints/Player/Morbius_BP.Morbius_BP_C|GetUltimateClaws _asmorbius_bp))
      (Default|ToggleUltForm _asmorbius_bp false))
    (:CastFailed
      (Development|PrintString "Morbius Ultimate used on wrong character" true true "(R=1.000000,G=0.000000,B=0.009241,A=1.000000)" 1e+01))))