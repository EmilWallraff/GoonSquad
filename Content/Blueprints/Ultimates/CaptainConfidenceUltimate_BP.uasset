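; Ultimate ability Blueprint for Captain Confidence that grants the character a second life while the ultimate runs.
; Overrides the execute and terminate actions, calling the parent first, then casting the owning character to CaptainConfidence_BP to activate or deactivate Second Life.
; The second-life logic itself lives on the character; a failed cast only prints a wrong-character message.
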(event EventBeginPlay
  (|CallParentFunction) ; This node is disabled and will not be called.\nDrag off pins to build functionality.
)

(event EventTick
  (params (DeltaSeconds :type Float%20%28single-precision%29))
  (|CallParentFunction DeltaSeconds) ; This node is disabled and will not be called.\nDrag off pins to build functionality.
)

(fn ExecuteUltimateAction
  (|CallParentFunction)
  (bind _ascaptain_confidence_bp (Utilities|Casting|CastToCaptainConfidence_BP (Variables|Default|GetOwningCharacter))
    (:then
      (Default|ActivateSecondLife _ascaptain_confidence_bp))
    (:CastFailed
      (Development|PrintString "Captain Confidence Ultimate used on wrong character" true true "(R=1.000000,G=0.000000,B=0.009241,A=1.000000)" 1e+01))))

(fn TerminateUltimateAction
  (|CallParentFunction)
  (bind _ascaptain_confidence_bp (Utilities|Casting|CastToCaptainConfidence_BP (Variables|Default|GetOwningCharacter))
    (:then
      (Default|DeactivateSecondLife _ascaptain_confidence_bp))
    (:CastFailed
      (Development|PrintString "Captain Confidence Ultimate ended on wrong character" true true "(R=1.000000,G=0.000000,B=0.009241,A=1.000000)" 1e+01))))