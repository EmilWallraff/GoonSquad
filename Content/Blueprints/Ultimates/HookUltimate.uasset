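; Ultimate ability Blueprint for the Hook character that toggles its ultimate weapon.
; Execute and terminate overrides call the parent, cast the owning character to Hook_BP, then activate or deactivate its UltimateWeapon.
; A failed cast only prints a wrong-character warning; all weapon behavior lives outside this asset.
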(event EventBeginPlay)

(event EventTick
  (params (DeltaSeconds :type Float%20%28single-precision%29)))

(fn ExecuteUltimateAction
  (|CallParentFunction)
  (bind _ashook_bp (Utilities|Casting|CastToHook_BP (Variables|Default|GetOwningCharacter))
    (:then
      (Default|ActivateWeapon _ashook_bp (Variables|/Game/Blueprints/Player/Hook_BP.Hook_BP_C|GetUltimateWeapon _ashook_bp)))
    (:CastFailed
      (Development|PrintString "Hook Ultimate used on wrong character" true true "(R=1.000000,G=0.000000,B=0.009241,A=1.000000)" 1e+01))))

(fn TerminateUltimateAction
  (|CallParentFunction)
  (bind _ashook_bp (Utilities|Casting|CastToHook_BP (Variables|Default|GetOwningCharacter))
    (:then
      (Default|DeactivateWeapon _ashook_bp (Variables|/Game/Blueprints/Player/Hook_BP.Hook_BP_C|GetUltimateWeapon _ashook_bp)))
    (:CastFailed
      (Development|PrintString "Hook Ultimate used on wrong character" true true "(R=1.000000,G=0.000000,B=0.009241,A=1.000000)" 1e+01))))