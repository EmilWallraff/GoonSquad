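; Ultimate ability for the Null character that reveals low-health enemies while active.
; Execute and terminate extend the parent ultimate, toggling detection mode on the owning Null_BP.
; While activated, every Tick calls a server event that scans all BaseCharacter_BP actors.
; It inflicts a timed status effect, credited to the owner's controller, on other-team characters at or below a fraction of max health.
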(event Custom|Server_GiveVisionOnLowHealthEnemies
  (bind _outactors (Actor|GetAllActorsOfClass "/Game/Blueprints/Player/BaseCharacter_BP.BaseCharacter_BP_C"))
  (bind _output_get (Variables|Default|SetAffectedPawns _outactors))
  (for _array_element _output_get
    (bind _sameteam (Default|CheckifonSameTeam _array_element (Variables|Default|GetOwningCharacter)))
    (if (not _sameteam)
      (if (<= (Variables|/Game/Blueprints/Player/BaseCharacter_BP.BaseCharacter_BP_C|GetCurrentHealth _array_element) (* (Variables|/Game/Blueprints/Player/BaseCharacter_BP.BaseCharacter_BP_C|GetMaxHealth _array_element) (Variables|Default|GetVisionHealthThreshold)))
        (Default|InflictStatusEffect _array_element "NewEnumerator3" (Variables|Default|GetWatchedDuration) (Utilities|Struct|MakeDamageInstigator false (Default|GetPlayerControllerReference (Variables|Default|GetOwningCharacter))))))))

(event EventBeginPlay)

(event EventTick
  (params (DeltaSeconds :type Float%20%28single-precision%29))
  (Utilities|FlowControl|Sequence
    (:then_0
      (|CallParentFunction DeltaSeconds))
    (:then_1
      (if (Variables|Default|GetActivated)
        (CallFunction|ServerGiveVisiononLowHealthEnemies)))))

(fn ExecuteUltimateAction
  (|CallParentFunction)
  (bind _asnull_bp (Utilities|Casting|CastToNull_BP (Variables|Default|GetOwningCharacter))
    (:then
      (Default|StartUltimateDetectionMode _asnull_bp))
    (:CastFailed
      (Development|PrintString "Null Ultimate used on wrong character" true true "(R=1.000000,G=0.000000,B=0.009241,A=1.000000)" 1e+01))))

(fn TerminateUltimateAction
  (|CallParentFunction)
  (bind _asnull_bp (Utilities|Casting|CastToNull_BP (Variables|Default|GetOwningCharacter))
    (:then
      (Default|EndUltimateDetectionMode _asnull_bp)
      (Utilities|Array|Clear (Variables|Default|GetAffectedPawns)))
    (:CastFailed
      (Development|PrintString "Null Ultimate used on wrong character" true true "(R=1.000000,G=0.000000,B=0.009241,A=1.000000)" 1e+01))))