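; Game mode for a round-based two-team match with character selection, an objective and score-to-win.
; Once enough players log in, it finds the objective, puts the first two players on opposing teams with spawn points and opens character selection.
; Each round resets objective and spawners and has controllers spawn pawns.
; A wiped team gives the other the round and feeds killfeeds, until a team reaches the required score and end screens show.
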(event Custom|AllPlayerLoggedIn
  (Development|PrintString "AllLoggedIn -> starting the game" true true "(R=1.000000,G=0.000000,B=0.971564,A=1.000000)" 8.0)
  (CallFunction|AssignObjective)
  (Teams|CreateTeams)
  (Spawning|AssignSpawnPoints)
  (CallFunction|StartCharacterSelection))

(event Custom|EndRound
  (params (WinningTeamNumber :type Integer))
  (Default|ResetObjective (Variables|Default|GetObjective))
  (bind _asgame_state_1_bp (Utilities|Casting|CastToGameState1_BP (Game|GetGameState))
    (:then
      (Default|EndRound _asgame_state_1_bp)
      (bind _team (Teams|FindTeambyNumber WinningTeamNumber))
      (bind _score (Default|IncrementScore _team))
      (Utilities|FlowControl|Delay 1.0)
      (if (>= _score (Variables|Default|GetRequiredScoreToWin))
        (CallFunction|EndGame _team)
        (else
          (RoundManagement|StartNewRound))))
    (:CastFailed
      (Development|PrintString "GameMode: wrong GameState" true true "(R=1.000000,G=0.000000,B=0.039016,A=1.000000)" 1e+01))))

(event Custom|AdjustUIToPlayerChanges
  (Utilities|FlowControl|Delay 0.2)
  (for _array_element (Variables|Default|GetAllPlayers)
    (bind _ascore_hud_bp (Utilities|Casting|CastToCoreHUD_BP (HUD|GetHUD _array_element)))
    (Default|ReconfigureStatisticsWidget _ascore_hud_bp)))

(event Custom|StartCharacterSelection
  (CharacterSelection|ShowCharacterSelectionUI)
  (Variables|CharacterSelection|SetCharacterSelection true))

(event Custom|EndCharacterSelection
  (if (Variables|CharacterSelection|GetCharacterSelection)
    (Variables|CharacterSelection|SetCharacterSelection false)
    (Utilities|FlowControl|Delay (Variables|CharacterSelection|GetCharacterSelectionEndingDelay))
    (CharacterSelection|HideCharacterSelectionUI)
    (CallFunction|InitializeGameModeUI)
    (RoundManagement|StartNewRound)))

(event EventBeginPlay)

(event EventTick
  (params (DeltaSeconds :type Float%20%28single-precision%29)))

(event EventPostLogin
  (params (NewPlayer :type Player%20Controller%20Object%20Reference))
  (bind _allplayers (Variables|Default|GetAllPlayers))
  ;[0 0 0] Player Connection/Disconnection
  (Development|PrintString "New Player!" true true "(R=0.000000,G=0.660000,B=1.000000,A=1.000000)" 8.0)
  (bind _asplayer_controller_1_bp (Utilities|Casting|CastToPlayerController1_BP NewPlayer))
  (Utilities|Array|Add _allplayers _asplayer_controller_1_bp)
  (CallFunction|AdjustUItoPlayerChanges)
  (if (>= (Utilities|Array|Length _allplayers) (Variables|Default|GetAmountOfPlayers))
    (CallFunction|AllPlayerLoggedin)))

(event EventOnSwapPlayerControllers
  (params (OldPC :type Player%20Controller%20Object%20Reference) (NewPC :type Player%20Controller%20Object%20Reference))
  (bind _allplayers (Variables|Default|GetAllPlayers))
  ;[0 0 0] Player Connection/Disconnection
  (Development|PrintString "PlayerControllerSwap" true true "(R=0.000000,G=0.660000,B=1.000000,A=1.000000)" 8.0)
  (bind _asplayer_controller_1_bp (Utilities|Casting|CastToPlayerController1_BP NewPC)
    (:then
      (Utilities|Array|Add (Variables|Default|GetAllPlayers) _asplayer_controller_1_bp))
    (:CastFailed
      _))
  (Utilities|IsValid OldPC
    (:Is%20Valid
      (bind _asplayer_controller_1_bp_2 (Utilities|Casting|CastToPlayerController1_BP OldPC)
        (:then
          (Utilities|Array|RemoveItem _allplayers _asplayer_controller_1_bp_2))
        (:CastFailed
          _)))
    (:Is%20Not%20Valid
      _))
  (CallFunction|AdjustUItoPlayerChanges)
  (if (>= (Utilities|Array|Length _allplayers) (Variables|Default|GetAmountOfPlayers))
    (CallFunction|AllPlayerLoggedin)))

(event EventOnLogout
  (params (ExitingController :type Controller%20Object%20Reference))
  ;[0 0 0] Player Connection/Disconnection
  (bind _asplayer_controller_1_bp (Utilities|Casting|CastToPlayerController1_BP ExitingController))
  (Utilities|Array|RemoveItem (Variables|Default|GetAllPlayers) _asplayer_controller_1_bp)
  (CallFunction|AdjustUItoPlayerChanges))

(fn ConstructionScript)

(fn OrderSpawningPlayers
  (for _array_element (Variables|Default|GetAllPlayers)
    (Default|StartSpawningPawn _array_element)))

(fn AssignSpawnPoints
  (bind _outactors (Actor|GetAllActorsOfClass "/Game/Blueprints/LevelContents/SpawnTeam0_BP.SpawnTeam0_BP_C"))
  (Default|SetSpawnPoint (Variables|Default|GetTeam0) (Transformation|GetActorTransform (Utilities|Array|Get(acopy) _outactors)))
  (bind _outactors_2 (Actor|GetAllActorsOfClass "/Game/Blueprints/LevelContents/SpawnTeam1_BP.SpawnTeam1_BP_C"))
  (Default|SetSpawnPoint (Variables|Default|GetTeam1) (Transformation|GetActorTransform (Utilities|Array|Get(acopy) _outactors_2))))

(fn SpawnPawn
  (params (PlayerController :type Player%20Controller%20Object%20Reference))
  (bind _returnvalue (Pawn|GetControlledPawn PlayerController))
  (Utilities|IsValid _returnvalue
    (:Is%20Valid
      (Actor|DestroyActor _returnvalue))
    (:Is%20Not%20Valid
      _))
  (bind _asplayer_controller_1_bp (Utilities|Casting|CastToPlayerController1_BP PlayerController))
  (bind _asplayer_state_1_bp (Utilities|Casting|CastToPlayerState1_BP (Variables|/Script/Engine.Controller|GetPlayerState _asplayer_controller_1_bp))
    (:then
      (bind _team (Teams|FindTeambyNumber (Default|GetTeam _asplayer_state_1_bp)))
      (bind _character (Class|PlayerStateInterfaceBPI|GetCharactertoSpawn(Message) (Variables|/Script/Engine.Controller|GetPlayerState PlayerController)))
      (bind _returnvalue_2 (Game|SpawnActorfromClass _character (Default|GetSpawnPoint _team) "Undefined" 0 0))
      (Pawn|Possess PlayerController _returnvalue_2))
    (:CastFailed
      (Development|PrintString "GameMode: No/Wrong Player State" true true "(R=1.000000,G=0.000000,B=0.017256,A=1.000000)" 1e+01))))

(fn CreateTeams
  (bind _allplayers (Variables|Default|GetAllPlayers))
  (for (_array_element _array_index) _allplayers
    (if (== _array_index 0)
      (bind _asplayer_state_1_bp (Utilities|Casting|CastToPlayerState1_BP (Variables|/Script/Engine.Controller|GetPlayerState _array_element)))
      (Default|SetTeam _asplayer_state_1_bp)
      (Default|AddPlayer (Variables|Default|GetTeam0) _array_element)
      (elif (== _array_index 1)
        (bind _asplayer_state_1_bp_2 (Utilities|Casting|CastToPlayerState1_BP (Variables|/Script/Engine.Controller|GetPlayerState _array_element)))
        (Default|SetTeam _asplayer_state_1_bp_2 1)
        (Default|AddPlayer (Variables|Default|GetTeam1) _array_element)
        (else
          (Development|PrintString (Utilities|String|Append (Utilities|String|ToString(Integer) (Utilities|Array|Length _allplayers)) "players here, which is more than" (Utilities|String|ToString(Integer) (Variables|Default|GetAmountOfPlayers)) "(the maximum amount) players in the lobby!") true true "(R=1.000000,G=0.032209,B=0.000000,A=1.000000)" 1e+01))))))

(fn FindTeambyNumber
  (params (TeamNumber :type Integer))
  (if (== TeamNumber 0)
    (return (Variables|Default|GetTeam0))
    (elif (== TeamNumber 1)
      (return (Variables|Default|GetTeam1))
      (else
        (Development|PrintString (Utilities|String|Append "No Team with number " (Utilities|String|ToString(Integer) TeamNumber)) true true "(R=0.000000,G=0.660000,B=1.000000,A=1.000000)" 1e+02)))))

(fn GetOtherTeam
  (params (Team :type Team%20BP%20Object%20Reference))
  (bind _team (Teams|FindTeambyNumber (- 1 (Default|GetTeamNumber Team))))
  (return _team))

(fn IsonSameTeam
  (params (Player1 :type Player%20Controller%201%20BP%20Object%20Reference) (Player2 :type Player%20Controller%201%20BP%20Object%20Reference))
  (bind _asplayer_state_1_bp (Utilities|Casting|CastToPlayerState1_BP (Variables|/Script/Engine.Controller|GetPlayerState Player1)))
  (bind _asplayer_state_1_bp_2 (Utilities|Casting|CastToPlayerState1_BP (Variables|/Script/Engine.Controller|GetPlayerState Player2)))
  (if (== (Default|GetTeam _asplayer_state_1_bp) (Default|GetTeam _asplayer_state_1_bp_2))
    (return true)
    (else
      (return false))))

(fn RegisterDeath
  (params (Dead :type Player%20Controller%201%20BP%20Object%20Reference) (Instigator :type Damage%20Instigator%20Structure))
  (Utilities|Array|Add (Variables|Default|GetDeadPlayers) Dead)
  (bind _asplayer_state_1_bp (Utilities|Casting|CastToPlayerState1_BP (Variables|/Script/Engine.Controller|GetPlayerState Dead)))
  (bind _team (Teams|FindTeambyNumber (Default|GetTeam _asplayer_state_1_bp)))
  (bind _teamdead (Default|IsTeamDead _team (Variables|Default|GetDeadPlayers)))
  (if _teamdead
    (bind _otherteam (Teams|GetOtherTeam _team))
    (CallFunction|EndRound (Default|GetTeamNumber _otherteam))
    (CallFunction|AddtoKillfeeds Dead Instigator)))

(fn StartNewRound
  (if (!= (Variables|Default|GetCurrentRound) 0)
    (RoundManagement|CleanUpRound))
  (Utilities|Array|Clear (Variables|Default|GetDeadPlayers))
  (Math|Integer|IncrementInt (Variables|Default|GetCurrentRound)
    (:%20%20
      (Default|ResetObjective (Variables|Default|GetObjective))
      (RoundManagement|PrepareSpawners)
      (Development|PrintString "New Round!")
      (Spawning|OrderSpawningPlayers)
      (bind _asgame_state_1_bp (Utilities|Casting|CastToGameState1_BP (Game|GetGameState))
        (:then
          (Default|StartRound _asgame_state_1_bp (Variables|Default|GetTimeUntilObjective)))
        (:CastFailed
          (Development|PrintString "GameMode: wrong GameState" true true "(R=1.000000,G=0.000000,B=0.039016,A=1.000000)" 1e+01))))))

(fn CleanUpRound
  (for _array_element (Variables|Default|GetAllPlayers)
    (if (not (Utilities|Array|ContainsItem (Variables|Default|GetDeadPlayers) _array_element))
      (Default|DestroyPawn _array_element)))
  (bind _outactors (Actor|GetAllActorswithInterface "/Game/Blueprints/Interactables/Interactable_BPI.Interactable_BPI_C"))
  (for _array_element_2 _outactors
    (Utilities|IsValid _array_element_2
      (:Is%20Valid
        (Actor|DestroyActor _array_element_2)))))

(fn AddtoKillfeeds
  (params (Dead :type Player%20Controller%201%20BP%20Object%20Reference) (Instigator :type Damage%20Instigator%20Structure))
  (bind _playerstate (Variables|/Script/Engine.Controller|GetPlayerState (.playercontroller Instigator)))
  (bind _playerstate_2 (Variables|/Script/Engine.Controller|GetPlayerState Dead))
  (bind _returnvalue (PlayerState|GetPlayerName _playerstate_2))
  (for _array_element (Variables|Default|GetAllPlayers)
    (bind _character (Class|PlayerStateInterfaceBPI|GetPlayerCharacter(Message) _playerstate_2))
    (if (.environmental Instigator)
      (Default|AddtoKillfeed _array_element (Utilities|Struct|MakeKillfeedEntryData (.environmental Instigator) "" 0 _returnvalue _character))
      (else
        (bind _character_2 (Class|PlayerStateInterfaceBPI|GetPlayerCharacter(Message) _playerstate))
        (Default|AddtoKillfeed _array_element (Utilities|Struct|MakeKillfeedEntryData (.environmental Instigator) (PlayerState|GetPlayerName _playerstate) _character_2 _returnvalue _character))))))

(fn EndGame
  (params (WinningTeam :type Team%20BP%20Object%20Reference))
  (for _array_element (Variables|Default|GetAllPlayers)
    (Default|DisplayEndScreen _array_element (Default|GetTeamNumber WinningTeam))
    (bind _onteam (Default|IsonTeam WinningTeam _array_element))
    (if _onteam
      (Default|PlayResultVoiceline _array_element "NewEnumerator2")
      (else
        (Default|PlayResultVoiceline _array_element "NewEnumerator3")))))

(fn GetScores
  (bind _team0 (Variables|Default|GetTeam0))
  (bind _result (LocalVariables|GetResult))
  (bind _team1 (Variables|Default|GetTeam1))
  (Utilities|Map|Add _result (Default|GetTeamNumber _team0) (Default|GetScore _team0))
  (Utilities|Map|Add _result (Default|GetTeamNumber _team1) (Default|GetScore _team1))
  (return _result))

(fn AssignObjective
  (bind _outactors (Actor|GetAllActorsOfClass "/Game/Blueprints/LevelContents/Objective_BP.Objective_BP_C"))
  (Variables|Default|SetObjective (Utilities|Array|Get(acopy) _outactors)))

(fn ShowCharacterSelectionUI
  (for _array_element (Variables|Default|GetAllPlayers)
    (Default|ClientTryShowingCharacterSelection _array_element)))

(fn HideCharacterSelectionUI
  (for _array_element (Variables|Default|GetAllPlayers)
    (Default|ClientTryHidingCharacterSelection _array_element)))

(fn ForceCharacterSelection
  (for _array_element (Variables|Default|GetAllPlayers)
    (Default|ClientTryForcingCharacterSelection _array_element)))

(fn InitializeGameModeUI
  (for _array_element (Variables|Default|GetAllPlayers)
    (Default|ClientInitializeGameModeUI _array_element)))

(fn PrepareSpawners
  (bind _outactors (Actor|GetAllActorswithInterface "/Game/Blueprints/LevelContents/Spawner_BPI.Spawner_BPI_C"))
  (for _array_element _outactors
    (Utilities|IsValid _array_element
      (:Is%20Valid
        (Class|SpawnerBPI|PrepareSpawner(Message) _array_element)))))