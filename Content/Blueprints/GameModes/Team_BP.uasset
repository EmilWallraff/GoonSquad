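; Team Blueprint that holds one team's players, score, team number and spawn point.
; Players are added to a list that backs membership checks and a team-wipe check, which is true when every member appears in a supplied dead-player list.
; Simple functions increment, read and reset the score and get or set the team number and spawn point, with no active event logic.
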(event EventBeginPlay)

(event EventTick
  (params (DeltaSeconds :type Float%20%28single-precision%29)))

(fn IsonTeam
  (params (Player :type Player%20Controller%201%20BP%20Object%20Reference))
  (return (Utilities|Array|ContainsItem (Variables|Default|GetPlayers) Player)))

(fn AddPlayer
  (params (Player :type Player%20Controller%201%20BP%20Object%20Reference))
  (Utilities|Array|Add (Variables|Default|GetPlayers) Player))

(fn IsTeamDead
  (params (DeadPlayers :type Array%20of%20Player%20Controller%201%20BP%20Object%20References))
  (for _array_element (Variables|Default|GetPlayers)
    (if (not (Utilities|Array|ContainsItem DeadPlayers _array_element))
      (return false)))
  (return true))

(fn IncrementScore
  (bind _result (Math|Integer|IncrementInt (Variables|Default|GetScore))
    (:%20%20
      (return _result))))

(fn GetScore
  (return (Variables|Default|GetScore)))

(fn ResetScore
  (Variables|Default|SetScore 0))

(fn GetTeamNumber
  (return (Variables|Default|GetTeamNumber)))

(fn SetTeamNumber
  (params (TeamNumber :type Integer))
  (Variables|Default|SetTeamNumber TeamNumber))

(fn SetSpawnPoint
  (params (SpawnPoint :type Transform))
  (Variables|Default|SetSpawnPoint SpawnPoint))

(fn GetSpawnPoint
  (return (Variables|Default|GetSpawnPoint)))