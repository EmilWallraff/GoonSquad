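; Game state for a team objective match, tracking character selection, the countdown to the objective unlock, the score and player stats.
; On Tick the authority runs the active timer, unlocks the Objective or forces selection at zero, and packs objective state and GameMode scores into GameScore.
; Player stats rebuild every tick, and selection ends early once enough players lock in.
; Lookup functions serve character display info and map images.
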(event EventBeginPlay
  (Utilities|FlowControl|Sequence
    (:then_0
      (bind _outactors (Actor|GetAllActorsOfClass "/Game/Blueprints/LevelContents/Objective_BP.Objective_BP_C"))
      (Variables|Scoring|SetObjective (Utilities|Array|Get(acopy) _outactors)))
    (:then_1
      (bind _asgame_mode_1_bp (Utilities|Casting|CastToGameMode1_BP (Game|GetGameMode)))
      (Variables|CharacterSelection|SetCurrentCharacterSelectionTime (Variables|/Game/Blueprints/GameModes/GameMode1_BP.GameMode1_BP_C|GetCharacterSelectionTime _asgame_mode_1_bp)))))

(event EventTick
  (params (DeltaSeconds :type Float%20%28single-precision%29))
  (Utilities|FlowControl|Sequence
    (:then_0
      (Networking|SwitchHasAuthority
        (:Authority
          (TimeUpdates|UpdateTime DeltaSeconds))))
    (:then_1
      ;[1 1 1] BAD CODE: keeps all player stats updated
      (PlayerUpdates|UpdatePlayers))
    (:then_2
      (Networking|SwitchHasAuthority
        (:Authority
          (CallFunction|UpdateGameScore))))))

(fn ConstructionScript)

(fn StartRound
  (params (TimeUntilObjective :type Float%20%28double-precision%29))
  (Variables|Scoring|SetCurrentTimeUntilObjective TimeUntilObjective)
  (Variables|Scoring|SetRoundTimeTicking true))

(fn EndRound
  (Variables|Scoring|SetRoundTimeTicking false))

(fn UpdateTime
  (params (DeltaSeconds :type Float%20%28double-precision%29))
  (if (Variables|Scoring|GetRoundTimeTicking)
    (TimeUpdates|UpdateRoundTime DeltaSeconds)
    (else
      (bind _asgame_mode_1_bp (Utilities|Casting|CastToGameMode1_BP (Game|GetGameMode)))
      (if (Variables|/Game/Blueprints/GameModes/GameMode1_BP.GameMode1_BP_C|GetCharacterSelection _asgame_mode_1_bp)
        (TimeUpdates|UpdateCharacterSelectionTime DeltaSeconds)))))

(fn UpdateRoundTime
  (params (DeltaSeconds :type Float%20%28double-precision%29))
  (if (>= (Variables|Scoring|GetCurrentTimeUntilObjective) 0.0)
    (bind _output_get (Variables|Scoring|SetCurrentTimeUntilObjective (- (Variables|Scoring|GetCurrentTimeUntilObjective) DeltaSeconds)))
    (if (<= _output_get 0.0)
      (Variables|Scoring|SetCurrentTimeUntilObjective 0.0)
      (Default|UnlockObjective (Variables|Scoring|GetObjective))
      (Variables|Scoring|SetRoundTimeTicking false))))

(fn UpdateCharacterSelectionTime
  (params (DeltaSeconds :type Float%20%28double-precision%29))
  (bind _output_get (Variables|CharacterSelection|SetCurrentCharacterSelectionTime (- (Variables|CharacterSelection|GetCurrentCharacterSelectionTime) DeltaSeconds)))
  (if (<= _output_get 0.0)
    (bind _asgame_mode_1_bp (Utilities|Casting|CastToGameMode1_BP (Game|GetGameMode)))
    (Default|ForceCharacterSelection _asgame_mode_1_bp)
    (Default|EndCharacterSelection _asgame_mode_1_bp)))

(fn UpdateGameScore
  (bind _objective (Variables|Scoring|GetObjective))
  (bind (_contested _owningteam _currentovertimeduration) (Default|GetObjectiveState _objective))
  (bind _asgame_mode_1_bp (Utilities|Casting|CastToGameMode1_BP (Game|GetGameMode))
    (:then
      (Variables|Scoring|SetGameScore (Utilities|Struct|MakeGameScore (Variables|Scoring|GetCurrentTimeUntilObjective) _contested _owningteam _currentovertimeduration (.Value (Utilities|Map|Find (Default|GetScores _asgame_mode_1_bp) 0)) (.Value (Utilities|Map|Find (Default|GetScores _asgame_mode_1_bp) 1)))))
    (:CastFailed
      (Development|PrintString "GameState: wrong GameMode" true true "(R=1.000000,G=0.000000,B=0.039016,A=1.000000)" 1e+01))))

(fn UpdatePlayers
  (PlayerUpdates|UpdatePlayerStats)
  (bind _asgame_mode_1_bp (Utilities|Casting|CastToGameMode1_BP (Game|GetGameMode)))
  (if (Variables|/Game/Blueprints/GameModes/GameMode1_BP.GameMode1_BP_C|GetCharacterSelection _asgame_mode_1_bp)
    (PlayerUpdates|UpdatePlayerswithSelectedCharacters)))

(fn UpdatePlayerStats
  (Utilities|Array|Clear (Variables|Default|GetAllPlayerStats))
  (for _array_element (Variables|Default|GetPlayerArray)
    (bind _asplayer_state_1_bp (Utilities|Casting|CastToPlayerState1_BP _array_element))
    (Utilities|Array|Add (Variables|Default|GetAllPlayerStats) (Default|GetPlayerStats _asplayer_state_1_bp))))

(fn UpdatePlayerswithSelectedCharacters
  (for _array_element (Variables|Default|GetPlayerArray)
    (bind _lockedin (Class|PlayerStateInterfaceBPI|GetCharacterLockedin(Message) _array_element))
    (if _lockedin
      (Math|Integer|IncrementInt (LocalVariables|GetPlayersSoFar))))
  (bind _output_get (Variables|CharacterSelection|SetPlayersWithSelectedCharacters (LocalVariables|GetPlayersSoFar)))
  (bind _asgame_mode_1_bp (Utilities|Casting|CastToGameMode1_BP (Game|GetGameMode))
    (:then
      (if (>= _output_get (Variables|/Game/Blueprints/GameModes/GameMode1_BP.GameMode1_BP_C|GetAmountOfPlayers _asgame_mode_1_bp))
        (Default|EndCharacterSelection _asgame_mode_1_bp)))
    (:CastFailed
      (Development|PrintString "f u" true true "(R=1.000000,G=0.000000,B=0.042350,A=1.000000)"))))

(fn GetCharacterDisplayInformation
  (params (Character :type Base%20Character%20BP%20Class%20Reference))
  (bind _returnvalue (Utilities|GetClassDisplayName Character))
  (bind _characterdisplayinformation (Variables|Default|GetCharacterDisplayInformation))
  (bind _returnvalue_2 (Utilities|String|Len _returnvalue))
  (bind _returnvalue_3 (- _returnvalue_2 5))
  (bind _returnvalue_4 (Utilities|String|Left _returnvalue _returnvalue_3))
  (bind (_value _returnvalue_5) (Utilities|Map|Find _characterdisplayinformation _returnvalue_4))
  (if (Utilities|IsValidClass Character)
    (if _returnvalue_5
      (return _value)
      (else
        (Development|PrintString (Utilities|String|Append "Character Display Information not found for: " _returnvalue_4) true true "(R=1.000000,G=0.008279,B=0.000000,A=1.000000)" 1e+01)
        (return "")))))

(fn GetMapImage
  (params (MapName :type String))
  (bind _mapimages (Variables|Default|GetMapImages))
  (bind (_value _returnvalue) (Utilities|Map|Find _mapimages MapName))
  (if _returnvalue
    (return _value)
    (else
      (Development|PrintString (Utilities|String|Append "Map Image not found for: " MapName) true true "(R=1.000000,G=0.008279,B=0.000000,A=1.000000)" 1e+01)
      (return 0))))