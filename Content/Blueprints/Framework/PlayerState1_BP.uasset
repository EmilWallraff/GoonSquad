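; Player state for a team-based hero game, tracking team, character selection and lock-in, combat stats and ultimate charge.
; Damage and healing reports add to totals and build charge unless the ultimate is active; selection and ultimate changes go through Server events.
; Kills advance a killstreak, reset on death, that picks a voiceline for the GetPlayerController pawn.
; Stat and character getters expose the chosen character only once locked in.
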(event Custom|Server_SetUltimateCharge
  (params (UltimateCharge :type Float%20%28double-precision%29))
  (bind _output_get (Variables|UltimateCharge|SetCurrentUltimateCharge UltimateCharge)))

(event Custom|Server_SetCharacterToSpawn
  (params (Character :type Base%20Character%20BP%20Class%20Reference))
  (Variables|CharacterSelection|SetCharacterToSpawn Character))

(event Custom|Server_SetCharacterLockedIn
  (params (LockedIn :type Boolean))
  (Variables|CharacterSelection|SetCharacterLockedIn LockedIn))

(event Custom|Server_SetUltState
  (params (UltState :type Boolean))
  (Variables|UltimateCharge|SetUltState UltState))

(event EventBeginPlay)

(event EventTick
  (params (DeltaSeconds :type Float%20%28single-precision%29)))

(event EventSetCharactertoSpawn
  (params (Character :type Base%20Character%20BP%20Class%20Reference))
  (CallFunction|ServerSetCharactertoSpawn Character))

(event EventSetCharacterLockedin
  (params (LockedIn :type Boolean))
  (CallFunction|ServerSetCharacterLockedin LockedIn))

(fn ConstructionScript)

(fn GetPlayerStats
  (if (Variables|CharacterSelection|GetCharacterLockedIn)
    (return (Utilities|Struct|MakePlayerStats (PlayerState|GetPlayerName) (Variables|CharacterSelection|GetCharacterToSpawn) (Variables|Team|GetCurrentTeam) (Variables|Stats|GetKills) (Variables|Stats|GetDeaths) (Variables|Stats|GetDamageDealt) (Variables|Stats|GetDamageReceived)))
    (else
      (return (Utilities|Struct|MakePlayerStats (PlayerState|GetPlayerName) 0 (Variables|Team|GetCurrentTeam) (Variables|Stats|GetKills) (Variables|Stats|GetDeaths) (Variables|Stats|GetDamageDealt) (Variables|Stats|GetDamageReceived))))))

(fn ReportDamageDealt
  (params (Damage :type Float%20%28double-precision%29) (Died :type Boolean) (Target :type Object%20Object%20Reference))
  (Variables|Stats|SetDamageDealt (+ Damage (Variables|Stats|GetDamageDealt)))
  (UltimateCharge|AssignUltimateCharge Damage)
  (if Died
    (Math|Integer|IncrementInt (Variables|Stats|GetKills)
      (:%20%20
        (bind _result (Math|Integer|IncrementInt (Variables|Stats|GetKillstreak))
          (:%20%20
            (switch int _result
              (:Default
                (LocalVariables|SetVoicelineType "NewEnumerator4" :!label _label))
              (:0
                (goto _label))
              (:1
                (goto _label))
              (:2
                (goto _label))
              (:3
                (LocalVariables|SetVoicelineType "NewEnumerator5" :!label _label_2))
              (:4
                (goto _label))
              (:5
                (LocalVariables|SetVoicelineType "NewEnumerator6"))
              (:6
                (goto _label_2))
              (:7
                (goto _label))
              (:8
                (goto _label_2))
              (:9
                (goto _label))
              (:10
                (goto _label_2)))
            (CallFunction|PlayVoiceline (LocalVariables|GetVoicelineType) false)))))))

(fn ReportDamageReceived
  (params (Damage :type Float%20%28double-precision%29) (Died :type Boolean) (Instigator :type Damage%20Instigator%20Structure))
  (Variables|Stats|SetDamageReceived (+ Damage (Variables|Stats|GetDamageReceived)))
  (if Died
    (Math|Integer|IncrementInt (Variables|Stats|GetDeaths)
      (:%20%20
        (Variables|Stats|SetKillstreak 0)))))

(fn ReportHealingDone
  (params (Healing :type Float%20%28double-precision%29) (Target :type Base%20Character%20BP%20Object%20Reference))
  (Variables|Stats|SetHealingDone (+ Healing (Variables|Stats|GetHealingDone)))
  (UltimateCharge|AssignUltimateCharge Healing))

(fn GetTeam
  (return (Variables|Team|GetCurrentTeam)))

(fn SetTeam
  (params (Team :type Integer))
  (Variables|Team|SetCurrentTeam Team))

(fn GetUltimateCharge
  (return (Variables|UltimateCharge|GetCurrentUltimateCharge)))

(fn AssignUltimateCharge
  (params (UltimateCharge :type Float%20%28double-precision%29))
  (if (not (Variables|UltimateCharge|GetUltState))
    (CallFunction|ServerSetUltimateCharge (+ UltimateCharge (Variables|UltimateCharge|GetCurrentUltimateCharge)))))

(fn PlayVoiceline
  (params (VoicelineType :type VoicelineType%20Enum :default "NewEnumerator0") (ForAll :type Boolean))
  (bind _asbase_character_bp (Utilities|Casting|CastToBaseCharacter_BP (Pawn|GetControlledPawn (Game|GetPlayerController))))
  (Default|PlayVoiceline _asbase_character_bp VoicelineType ForAll))

(fn StartUltState
  (CallFunction|ServerSetUltState true)
  (CallFunction|ServerSetUltimateCharge 0.0))

(fn EndUltState
  (if (Variables|UltimateCharge|GetUltState)
    (CallFunction|ServerSetUltimateCharge 0.0)
    (CallFunction|ServerSetUltState false)))

(fn GetCharacterLockedin
  (return (Variables|CharacterSelection|GetCharacterLockedIn)))

(fn GetCharactertoSpawn
  (return (Variables|CharacterSelection|GetCharacterToSpawn)))

(fn GetPlayerCharacter
  (if (Variables|CharacterSelection|GetCharacterLockedIn)
    (return (Variables|CharacterSelection|GetCharacterToSpawn))
    (else
      (return 0))))

(fn GetPlayerTeam
  (return (Variables|Team|GetCurrentTeam)))