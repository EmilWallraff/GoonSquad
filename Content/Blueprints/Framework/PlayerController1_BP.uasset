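; Player controller that links the game mode, the possessed character and the local core HUD.
; On begin play it loads saved sensitivity and crosshair settings and caches the HUD; on spawn it has the game mode create the pawn, hands it a self reference and plays a first-spawn voiceline.
; Client events and input forward UI actions to the HUD, with timer retries covering late pawn or HUD availability during setup.
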(event Custom|TryInitializingPawn
  ;[0 0 0] gives reference to pawn and spawns HUD when pawn is possessed
  (if (Utilities|IsValid (Pawn|GetControlledPawn))
    (CallFunction|GiveSelfReferencetoPawn)
    (Voicelines|OrderSpawnVoiceline)
    (else
      (Utilities|Time|SetTimerbyEvent (delegate Custom|TryInitializingPawn) 0.1))))

(event Custom|TryInitializingHUD
  ;[0 0 0] gives reference to pawn and spawns HUD when pawn is possessed
  (if (Utilities|IsValid (Variables|Default|GetCoreHUD))
    (Default|TrySettingUpGameUI (Variables|Default|GetCoreHUD))
    (else
      (Utilities|Time|SetTimerbyEvent (delegate Custom|TryInitializingHUD) 0.1))))

(event Custom|Client_TryForcingCharacterSelection
  (bind _corehud (Variables|Default|GetCoreHUD))
  ;[0 0 0] Calls Show/HideCharacterSelection locally
  (Utilities|IsValid _corehud
    (:Is%20Valid
      (Default|ForceCharacterSelection _corehud))))

(event Custom|ApplyCrosshairSettings
  (params (CrosshairData :type Crosshair%20Data%20Structure))
  ;[0 0 0] Call HUD events
  (Default|ApplyCrosshairData (Variables|Default|GetCoreHUD) CrosshairData))

(event Custom|Client_PlayResultVoiceline
  (params (Voiceline :type Sound%20Cue%20Object%20Reference))
  (Audio|PlaySound2D Voiceline 1.0 1.0 0.0 0 0))

(event Custom|StartSpawningPawn
  ;[0 0 0] on server: tells gamemode to spawn pawn
  (Utilities|FlowControl|Sequence
    (:then_0
      (bind _asgame_mode_1_bp (Utilities|Casting|CastToGameMode1_BP (Game|GetGameMode)))
      (Default|SpawnPawn _asgame_mode_1_bp self))
    (:then_1
      (CallFunction|TryInitializingPawn))
    (:then_2
      (CallFunction|ClientInitializeHUD))))

(event Custom|DisplayHitFeedback
  (params (Damage :type Float%20%28double-precision%29) (Headshot :type Boolean) (Kill :type Boolean))
  ;[0 0 0] Call HUD events
  (Default|ShowHitFeedback (Variables|Default|GetCoreHUD) Damage Headshot Kill))

(event Custom|Client_InitializeHUD
  ;[0 0 0] calls TryInitializingHUD locally
  (CallFunction|TryInitializingHUD))

(event Custom|DisplayEndScreen
  (params (WinningTeam :type Integer))
  ;[0 0 0] Call HUD events
  (Default|ShowEndScreen (Variables|Default|GetCoreHUD) WinningTeam))

(event Custom|AddToKillfeed
  (params (KillfeedEntryData :type Killfeed%20Entry%20Data%20Structure))
  ;[0 0 0] Call HUD events
  (Default|AddKillFeedEntry (Variables|Default|GetCoreHUD) KillfeedEntryData))

(event Custom|Client_InitializeGameModeUI
  ;[0 0 0] Calls TrySettingUpGameModeUI locally
  (Default|TrySettingUpGameModeUI (Variables|Default|GetCoreHUD)))

(event Custom|Client_TryShowingCharacterSelection
  (bind _corehud (Variables|Default|GetCoreHUD))
  ;[0 0 0] Calls Show/HideCharacterSelection locally
  (Utilities|IsValid _corehud
    (:Is%20Valid
      (Default|ShowCharacterSelection _corehud))
    (:Is%20Not%20Valid
      (Utilities|Time|SetTimerbyEvent (delegate Custom|Client_TryShowingCharacterSelection) 0.1))))

(event Custom|Client_TryHidingCharacterSelection
  (bind _corehud (Variables|Default|GetCoreHUD))
  ;[0 0 0] Calls Show/HideCharacterSelection locally
  (Utilities|IsValid _corehud
    (:Is%20Valid
      (Default|HideCharacterSelection _corehud))))

(event EventBeginPlay
  ;[0 0 0] locally gets reference to core HUD
  (Utilities|FlowControl|Sequence
    (:then_0
      (CallFunction|LoadPlayerSettings))
    (:then_1
      (if (Pawn|IsLocalPlayerController)
        (bind _ascore_hud_bp (Utilities|TryGettingCoreHUD 0.1 1e+01)
          (:Success
            (Variables|Default|SetCoreHUD _ascore_hud_bp))
          (:Failed
            (Development|PrintString "Failed getting HUD" true true "(R=1.000000,G=0.006938,B=0.010254,A=1.000000)" 8.0)))))))

(event Input|KeyboardEvents|Tab
  (params (Key :type Key%20Structure :default "None"))
  (bind _corehud (Variables|Default|GetCoreHUD))
  (:Pressed
    (Default|ShowStatistics _corehud))
  (:Released
    (Default|HideStatistics _corehud)))

(event Input|KeyboardEvents|Escape
  (params (Key :type Key%20Structure :default "None"))
  (:Pressed
    (Default|TogglePauseMenu (Variables|Default|GetCoreHUD))))

(fn ConstructionScript)

(fn GiveSelfReferencetoPawn
  (bind _asbase_character_bp (Utilities|Casting|CastToBaseCharacter_BP (Pawn|GetControlledPawn)))
  (Default|SetPlayerControllerReference _asbase_character_bp self))

(fn DestroyPawn
  (bind _returnvalue (Pawn|GetControlledPawn))
  (bind _asbase_character_bp (Utilities|Casting|CastToBaseCharacter_BP _returnvalue))
  (for _array_element (Variables|/Game/Blueprints/Player/BaseCharacter_BP.BaseCharacter_BP_C|GetAllWeapons _asbase_character_bp)
    (Class|WeaponBPI|DeleteWeaponModel(Message) _array_element))
  (Actor|DestroyActor _returnvalue))

(fn LoadPlayerSettings
  (bind _returnvalue (SaveGame|DoesSaveGameExist (Variables|Default|GetSettingsSaveSlotName)))
  (if _returnvalue
    (bind _returnvalue_2 (SaveGame|LoadGamefromSlot (Variables|Default|GetSettingsSaveSlotName)))
    (bind _assave_settings (Utilities|Casting|CastToSaveSettings _returnvalue_2))
    (Variables|Settings|SetMouseSensitivity (Variables|/Game/Blueprints/DataManagement/SaveSettings.SaveSettings_C|GetSensitivity _assave_settings))
    (Variables|Settings|SetCrosshairSettings (Variables|/Game/Blueprints/DataManagement/SaveSettings.SaveSettings_C|GetCrosshair _assave_settings))))

(fn ApplyPlayerSettings
  (CallFunction|ApplyCrosshairSettings (Variables|Settings|GetCrosshairSettings)))

(fn OrderSpawnVoiceline
  (if (Variables|Default|GetFirstSpawn)
    (bind _asbase_character_bp (Utilities|Casting|CastToBaseCharacter_BP (Pawn|GetControlledPawn)))
    (Default|PlayVoiceline _asbase_character_bp "NewEnumerator1" false)
    (Variables|Default|SetFirstSpawn false)
    (Variables|Voicelines|SetLastVoicelines (Variables|/Game/Blueprints/Player/BaseCharacter_BP.BaseCharacter_BP_C|GetVoicelines _asbase_character_bp))))

(fn PlayResultVoiceline
  (params (VoicelineType :type VoicelineType%20Enum :default "NewEnumerator0"))
  (CallFunction|ClientPlayResultVoiceline (.Value (Utilities|Map|Find (Variables|Voicelines|GetLastVoicelines) VoicelineType))))