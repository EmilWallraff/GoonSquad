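; Level spawner actor that places a HealthPack_BP at a height offset above itself and respawns it after removal.
; PrepareSpawner spawns the first pack only if none is present, via server events that create the actor and set the HasHealthPack flag.
; The pack receives a healing value and a reference to its spawner.
; RemoveHealthPack clears the flag and schedules a new spawn after RespawnTime.
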(event Custom|OrderNewHealthPackSpawn
  (Utilities|FlowControl|Delay (Variables|Default|GetRespawnTime))
  (CallFunction|SpawnHealthPack))

(event Custom|Server_SetHasHealthPack
  (params (HasHealthPack :type Boolean))
  (Variables|Default|SetHasHealthPack HasHealthPack))

(event Custom|Server_CreateHealthPack
  (Game|SpawnActorfromClass "/Game/Blueprints/Interactables/HealthPack_BP.HealthPack_BP_C" (CallFunction|DetermineSpawnTransform) "AlwaysSpawn" 0 (Variables|Default|GetHealingValue) self 0))

(event EventPrepareSpawner
  (CallFunction|SpawnHealthPack))

(fn ConstructionScript)

(fn SpawnHealthPack
  (if (not (Variables|Default|GetHasHealthPack))
    (CallFunction|ServerCreateHealthPack)
    (CallFunction|ServerSetHasHealthPack true)))

(fn DetermineSpawnTransform
  (bind _defaultsceneroot (Variables|Default|GetDefaultSceneRoot))
  (bind _returnvalue (Transformation|GetWorldTransform _defaultsceneroot))
  (return (Math|Transform|MakeTransform (+ (.location _returnvalue) (* (Math|Vector|VectorUp) (Variables|Default|GetHealthPackSpawnHeight))) (.rotation _returnvalue) (.scale _returnvalue))))

(fn RemoveHealthPack
  (CallFunction|ServerSetHasHealthPack false)
  (CallFunction|OrderNewHealthPackSpawn))