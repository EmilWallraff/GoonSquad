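; Capture-point objective for a two-team round mode, inactive until unlocked.
; A box overlap tracks player controllers inside; while unlocked, Tick calls a server event that compares team headcounts.
; The majority team's timer counts down while the other's refills up to the overtime maximum; a tie marks it contested and refills both.
; A timer reaching zero ends the round through GameMode1_BP and resets the objective.
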(event OnComponentEndOverlap(Box)
  (params (OverlappedComponent :type Primitive%20Component%20Object%20Reference) (OtherActor :type Actor%20Object%20Reference) (OtherComp :type Primitive%20Component%20Object%20Reference) (OtherBodyIndex :type Integer))
  ;[0 0 0] Keep PlayersInside updated
  (bind _asbase_character_bp (Utilities|Casting|CastToBaseCharacter_BP OtherActor))
  (Utilities|Array|RemoveItem (Variables|Default|GetPlayersInside) (Default|GetPlayerControllerReference _asbase_character_bp)))

(event OnComponentBeginOverlap(Box)
  (params (OverlappedComponent :type Primitive%20Component%20Object%20Reference) (OtherActor :type Actor%20Object%20Reference) (OtherComp :type Primitive%20Component%20Object%20Reference) (OtherBodyIndex :type Integer) (bFromSweep :type Boolean) (SweepResult :type Hit%20Result%20Structure%20%28by%20ref%29))
  ;[0 0 0] Keep PlayersInside updated
  (bind _asbase_character_bp (Utilities|Casting|CastToBaseCharacter_BP OtherActor))
  (Utilities|Array|Add (Variables|Default|GetPlayersInside) (Default|GetPlayerControllerReference _asbase_character_bp)))

(event Custom|Server_UpdateObjective
  (params (DeltaSeconds :type Float%20%28double-precision%29))
  ;[0 0 0] Updates objective state and overtime
  (Update|UpdateObjective DeltaSeconds))

(event Custom|Server_ResetObjective
  (bind _maxovertimeduration (Variables|Default|GetMaxOvertimeDuration))
  ;[0 0 0] Resets activity, objective state and capture time
  (Variables|Default|SetUnlocked false)
  (Variables|Default|SetContested true)
  (Variables|Default|SetCaptureTimeTeam0 _maxovertimeduration)
  (Variables|Default|SetCaptureTimeTeam1 _maxovertimeduration))

(event EventBeginPlay
  (CallFunction|ResetObjective))

(event EventTick
  (params (DeltaSeconds :type Float%20%28single-precision%29))
  ;[0 0 0] Updates objective state and overtime
  (if (Variables|Default|GetUnlocked)
    (CallFunction|ServerUpdateObjective DeltaSeconds)))

(fn ConstructionScript)

(fn UnlockObjective
  (Variables|Default|SetUnlocked true))

(fn UpdateObjective
  (params (DeltaSeconds :type Float%20%28double-precision%29))
  (bind _amountteammembers (Update|GetAmountTeamMembersonPoint))
  (bind _amountteammembers_2 (Update|GetAmountTeamMembersonPoint 1))
  (bind _returnvalue (- _amountteammembers _amountteammembers_2))
  (if (== _returnvalue 0)
    (Variables|Default|SetContested true)
    (Update|AddCaptureTime DeltaSeconds)
    (Update|AddCaptureTime DeltaSeconds 1)
    (else
      (Variables|Default|SetContested false)
      (if (> _returnvalue 0)
        (Variables|Default|SetOwningTeam 0)
        (Update|RemoveCaptureTime DeltaSeconds (Variables|Default|GetOwningTeam) :!label _label)
        (Update|AddCaptureTime DeltaSeconds (- 1 (Variables|Default|GetOwningTeam)))
        (elif (< _returnvalue 0)
          (Variables|Default|SetOwningTeam 1)
          (goto _label))))))

(fn GetAmountTeamMembersonPoint
  (params (TeamNumber :type Integer))
  (for _array_element (Variables|Default|GetPlayersInside)
    (bind _asplayer_state_1_bp (Utilities|Casting|CastToPlayerState1_BP (Variables|/Script/Engine.Controller|GetPlayerState _array_element))
      (:then
        (if (== TeamNumber (Default|GetTeam _asplayer_state_1_bp))
          (Math|Integer|IncrementInt (LocalVariables|GetResult))))
      (:CastFailed
        (Development|PrintString "Objective: wrong PlayerState!" true true "(R=1.000000,G=0.000000,B=0.039016,A=1.000000)" 1e+01))))
  (return (LocalVariables|GetResult)))

(fn ResetObjective
  (CallFunction|ServerResetObjective))

(fn GetObjectiveState
  (switch int (Variables|Default|GetOwningTeam)
    (:0
      (LocalVariables|SetCaptureTime (Variables|Default|GetCaptureTimeTeam0)))
    (:1
      (LocalVariables|SetCaptureTime (Variables|Default|GetCaptureTimeTeam1))))
  (return (Variables|Default|GetContested) (Variables|Default|GetOwningTeam) (LocalVariables|GetCaptureTime)))

(fn RemoveCaptureTime
  (params (DeltaSeconds :type Float%20%28double-precision%29) (TeamNumber :type Integer))
  (switch int TeamNumber
    (:Default
      (Development|PrintString "Objective: Invalid TeamNumber!" true true "(R=1.000000,G=0.000000,B=0.018970,A=1.000000)" 1e+01))
    (:0
      (bind _output_get (Variables|Default|SetCaptureTimeTeam0 (- (Variables|Default|GetCaptureTimeTeam0) DeltaSeconds)))
      (if (<= _output_get 0.0)
        (bind _asgame_mode_1_bp (Utilities|Casting|CastToGameMode1_BP (Game|GetGameMode) :!label _label)
          (:then
            (Default|EndRound _asgame_mode_1_bp TeamNumber)
            (CallFunction|ResetObjective))
          (:CastFailed
            (Development|PrintString "Objective: Wring GameMode!" true true "(R=1.000000,G=0.000000,B=0.018970,A=1.000000)" 1e+01)))))
    (:1
      (bind _output_get_2 (Variables|Default|SetCaptureTimeTeam1 (- (Variables|Default|GetCaptureTimeTeam1) DeltaSeconds)))
      (if (<= _output_get_2 0.0)
        (goto _label)))))

(fn AddCaptureTime
  (params (DeltaSeconds :type Float%20%28double-precision%29) (TeamNumber :type Integer))
  (bind _maxovertimeduration (Variables|Default|GetMaxOvertimeDuration))
  (bind _maxovertimeduration_2 (Variables|Default|GetMaxOvertimeDuration))
  (switch int TeamNumber
    (:Default
      (Development|PrintString "Objective: Invalid TeamNumber!" true true "(R=1.000000,G=0.000000,B=0.018970,A=1.000000)" 1e+01))
    (:0
      (bind _output_get (Variables|Default|SetCaptureTimeTeam0 (+ (Variables|Default|GetCaptureTimeTeam0) DeltaSeconds)))
      (if (>= _output_get _maxovertimeduration_2)
        (Variables|Default|SetCaptureTimeTeam0 _maxovertimeduration)))
    (:1
      (bind _output_get_2 (Variables|Default|SetCaptureTimeTeam1 (+ (Variables|Default|GetCaptureTimeTeam1) DeltaSeconds)))
      (if (>= _output_get_2 _maxovertimeduration_2)
        (Variables|Default|SetCaptureTimeTeam1 _maxovertimeduration)))))