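; ArrowDummy2 is a dummy character or pawn that moves along its capsule's axes through the forward/backward and right/left input axis events.
; Both events pass a fixed scale to AddMovementInput and ignore the axis value, so input magnitude and sign have no effect.
; SetGoal stores a CurrentGoal, but the goal-directed movement and debug print are disconnected, so the goal does not drive motion.
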(event EventBeginPlay)

(event EventTick
  (params (DeltaSeconds :type Float%20%28single-precision%29)))

(event Input|AxisEvents|InputAxisMoveForwards/Backwards
  (params (AxisValue :type Float%20%28single-precision%29))
  (Pawn|Input|AddMovementInput (Math|Vector|GetForwardVector (Variables|Collision|GetCapsuleComponent)) 1.0 false))

(event Input|AxisEvents|InputAxisMoveRight/Left
  (params (AxisValue :type Float%20%28single-precision%29))
  (Pawn|Input|AddMovementInput (Math|Vector|GetRightVector (Variables|Collision|GetCapsuleComponent)) 1.0 false))

(fn ConstructionScript)

(fn SetGoal
  (params (Input :type Vector))
  (Variables|Default|SetCurrentGoal Input))