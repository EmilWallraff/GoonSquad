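; Morbius Orb is a timed, shootable life-drain orb that damages an enemy and heals its owning character by the damage dealt.
; A range sphere tracks nearby characters, and each Tick selects the lowest-health enemy that passes a status-effect check and line-of-sight trace.
; Damage, healing and hit feedback run through a server event, while a multicast aims the red connection effect at the target.
; The orb destroys itself when its duration expires or its health runs out.
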(event OnComponentBeginOverlap(RangeCollider)
  (params (OverlappedComponent :type Primitive%20Component%20Object%20Reference) (OtherActor :type Actor%20Object%20Reference) (OtherComp :type Primitive%20Component%20Object%20Reference) (OtherBodyIndex :type Integer) (bFromSweep :type Boolean) (SweepResult :type Hit%20Result%20Structure%20%28by%20ref%29))
  (bind _asbase_character_bp (Utilities|Casting|CastToBaseCharacter_BP OtherActor))
  (Utilities|Array|AddUnique (Variables|Default|GetPlayersInRange) _asbase_character_bp))

(event OnComponentEndOverlap(RangeCollider)
  (params (OverlappedComponent :type Primitive%20Component%20Object%20Reference) (OtherActor :type Actor%20Object%20Reference) (OtherComp :type Primitive%20Component%20Object%20Reference) (OtherBodyIndex :type Integer))
  (bind _asbase_character_bp (Utilities|Casting|CastToBaseCharacter_BP OtherActor))
  (Utilities|Array|RemoveItem (Variables|Default|GetPlayersInRange) _asbase_character_bp))

(event Custom|Server_DoDamageAndHealing
  (params (Target :type Base%20Character%20BP%20Object%20Reference))
  (bind _owningcharacter (Variables|Default|GetOwningCharacter))
  (bind (_damagecaused _died) (Default|TakeDamage Target (Variables|Default|GetDamage) (Utilities|Struct|MakeDamageInstigator false (Default|GetPlayerControllerReference (Variables|Default|GetOwningCharacter)))))
  (Default|DisplayHitFeedback (Variables|/Game/Blueprints/Player/BaseCharacter_BP.BaseCharacter_BP_C|GetPlayerControllerReference (Variables|Default|GetOwningCharacter)) _damagecaused false _died)
  (Default|RestoreHealth _owningcharacter _damagecaused (Utilities|Struct|MakeDamageInstigator false (Default|GetPlayerControllerReference _owningcharacter))))

(event Custom|Multicast_DrawOrbEffects
  (params (Target :type Base%20Character%20BP%20Object%20Reference))
  (Effects|Components|ParticleSystem|SetVectorParameter (Variables|Default|GetOrbConnection) "ConnectionEnd" (Transformation|GetActorLocation Target)))

(event EventBeginPlay
  (Utilities|FlowControl|Sequence
    (:then_0
      (Variables|Default|SetCurrentHealth (Variables|Default|GetMaxHealth)))
    (:then_1
      (CallFunction|InitiateVisuals))
    (:then_2
      (Utilities|FlowControl|Delay (Variables|Default|GetDuration))
      (Actor|DestroyActor))))

(event EventTick
  (params (DeltaSeconds :type Float%20%28single-precision%29))
  (bind _targets (CallFunction|DetermineTarget))
  (Utilities|IsValid _targets
    (:Is%20Valid
      (Development|PrintString (Utilities|GetDisplayName _targets))
      (CallFunction|ShowConnection)
      (CallFunction|ServerDoDamageandHealing _targets)
      (CallFunction|MulticastDrawOrbEffects _targets))
    (:Is%20Not%20Valid
      (Development|PrintString "NOTHING HIT")
      (CallFunction|HideConnection))))

(event EventDie
  (params (Instigator :type Damage%20Instigator%20Structure))
  (Actor|DestroyActor))

(fn ConstructionScript)

(fn DetermineTarget
  (for _array_element (Variables|Default|GetPlayersInRange)
    (bind _statuseffect (Default|CheckforStatusEffect _array_element "NewEnumerator0"))
    (Utilities|IsValid _statuseffect
      (:Is%20Valid
        (bind _sameteam (Default|CheckifonSameTeam _array_element (Variables|Default|GetOwningCharacter)))
        (if (not _sameteam)
          (bind _outhit (Collision|LineTraceByChannel (Transformation|GetWorldLocation (Variables|Default|GetDefaultSceneRoot)) (.location (Transformation|GetWorldTransform (Variables|/Script/Engine.Actor|GetRootComponent _array_element))) "TraceTypeQuery2" false 0 "ForDuration" true "(R=1.000000,G=0.000000,B=0.000000,A=1.000000)" "(R=0.000000,G=1.000000,B=0.000000,A=1.000000)" 1.5))
          (if (== _array_element (.HitActor (Collision|BreakHitResult _outhit)))
            (Utilities|Array|Add (LocalVariables|GetPossibleTargets) _array_element))))))
  (for _array_element_2 (LocalVariables|GetPossibleTargets)
    (if (< (Variables|/Game/Blueprints/Player/BaseCharacter_BP.BaseCharacter_BP_C|GetCurrentHealth _array_element_2) (LocalVariables|GetLowestHealth))
      (LocalVariables|SetLowestHealthCharacter _array_element_2)
      (LocalVariables|SetLowestHealth (Variables|/Game/Blueprints/Player/BaseCharacter_BP.BaseCharacter_BP_C|GetCurrentHealth _array_element_2))))
  (return (LocalVariables|GetLowestHealthCharacter)))

(fn InitiateVisuals
  (Components|Sphere|SetSphereRadius (Variables|Default|GetRangeCollider) (Variables|Default|GetRange) true)
  (Effects|Components|ParticleSystem|SetColorParameter (Variables|Default|GetOrbConnection) "Color" "(R=1.000000,G=0.000000,B=0.000000,A=1.000000)"))

(fn ShowConnection
  (bind _orbconnection (Variables|Default|GetOrbConnection))
  (if (not (Variables|/Script/Engine.SceneComponent|GetbVisible _orbconnection))
    (Rendering|SetVisibility _orbconnection true false)))

(fn HideConnection
  (bind _orbconnection (Variables|Default|GetOrbConnection))
  (if (Variables|/Script/Engine.SceneComponent|GetbVisible _orbconnection)
    (Rendering|SetVisibility _orbconnection false false)))

(fn GetShot
  (params (ShotData :type Shot%20Data%20Structure))
  (bind (_damagecaused _died) (CallFunction|TakeDamage (.damagevalue ShotData) (.instigator ShotData)))
  (return _damagecaused _died false))

(fn TakeDamage
  (params (DamageValue :type Float%20%28double-precision%29) (Instigator :type Damage%20Instigator%20Structure))
  (bind _output_get (Variables|Default|SetCurrentHealth (- (Variables|Default|GetCurrentHealth) DamageValue)))
  (if (<= _output_get 0.0)
    (CallFunction|Die Instigator)
    (return (+ _output_get DamageValue) true)
    (else
      (return DamageValue false))))