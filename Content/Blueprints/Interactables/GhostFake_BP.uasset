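; Shootable decoy of a player character that holds a copy of the owner's current third-person weapon model in its hand socket.
; It dies when its duration expires or damage depletes its health, removing the weapon model through a server-to-multicast call.
; Shots from the opposing team make the server inflict a timed watched status effect on the shooter's pawn, credited to the owner.
; Code copying the owner's mesh and materials is present but never runs.
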(event Custom|Server_DestroyWeaponModel
  (CallFunction|MulticastDestroyWeaponModel))

(event Custom|Multicast_DestroyWeaponModel
  (Actor|DestroyActor (Variables|Default|GetWeaponModel)))

(event Custom|Server_InflictWatched
  (params (PlayerController :type Player%20Controller%201%20BP%20Object%20Reference))
  (bind _returnvalue (Pawn|GetControlledPawn PlayerController))
  (Utilities|IsValid _returnvalue
    (:Is%20Valid
      (bind _asbase_character_bp (Utilities|Casting|CastToBaseCharacter_BP _returnvalue))
      (Default|InflictStatusEffect _asbase_character_bp "NewEnumerator3" (Variables|Default|GetWatchedDuration) (Utilities|Struct|MakeDamageInstigator false (Variables|/Game/Blueprints/Player/BaseCharacter_BP.BaseCharacter_BP_C|GetPlayerControllerReference (Variables|Default|GetPlayerCharacter)))))))

(event EventBeginPlay
  (Utilities|FlowControl|Sequence
    (:then_0
      (Variables|Default|SetCurrentHealth (Variables|Default|GetMaxHealth)))
    (:then_1
      (Utilities|FlowControl|Delay (Variables|Default|GetDuration))
      (CallFunction|Die))
    (:then_2
      (CallFunction|SpawnWeaponMesh))))

(event EventDie
  (params (Instigator :type Damage%20Instigator%20Structure))
  (CallFunction|ServerDestroyWeaponModel)
  (Actor|DestroyActor))

(fn ConstructionScript)

(fn SpawnWeaponMesh
  (bind _playercharacter (Variables|Default|GetPlayerCharacter))
  (bind _asbase_weapon_bp (Utilities|Casting|CastToBaseWeapon_BP (Variables|/Game/Blueprints/Player/BaseCharacter_BP.BaseCharacter_BP_C|GetCurrentlyUsedWeapon _playercharacter)))
  (bind _returnvalue (Game|SpawnActorfromClass (Utilities|GetClass (Variables|/Game/Blueprints/Weapons/BaseWeapon_BP.BaseWeapon_BP_C|Get3rdPersonWeaponModel _asbase_weapon_bp)) (Transformation|GetSocketTransform (Variables|Default|GetSkeletalMesh) "hand_r_WeaponSocket" "RTS_World") "Undefined" _playercharacter 0))
  (Variables|Default|SetWeaponModel _returnvalue)
  (Transformation|AttachComponentToComponent _returnvalue (Variables|Default|GetSkeletalMesh) "hand_r_WeaponSocket" "SnapToTarget" "SnapToTarget" "SnapToTarget" true))

(fn CheckifEnemyShot
  (params (DamageInstigator :type Damage%20Instigator%20Structure))
  (if (.environmental DamageInstigator)
    (return false)
    (else
      (bind _team (Class|PlayerStateInterfaceBPI|GetPlayerTeam(Message) (Variables|/Script/Engine.Controller|GetPlayerState (.playercontroller DamageInstigator))))
      (bind _team_2 (Class|PlayerStateInterfaceBPI|GetPlayerTeam(Message) (Variables|/Game/Blueprints/Player/BaseCharacter_BP.BaseCharacter_BP_C|GetPlayerStateReference (Variables|Default|GetPlayerCharacter))))
      (if (!= _team _team_2)
        (return true)
        (else
          (return false))))))

(fn GetShot
  (params (ShotData :type Shot%20Data%20Structure))
  (bind _enemyshot (CallFunction|CheckifEnemyShot (.instigator ShotData)))
  (if _enemyshot
    (CallFunction|ServerInflictWatched (.PlayerController (Utilities|Struct|BreakDamageInstigator (.instigator ShotData)))))
  (bind (_damagecaused _died) (CallFunction|TakeDamage (.damagevalue ShotData) (.instigator ShotData)))
  (return _damagecaused _died false))

(fn TakeDamage
  (params (DamageValue :type Float%20%28double-precision%29) (Instigator :type Damage%20Instigator%20Structure))
  (bind _output_get (Variables|Default|SetCurrentHealth (- (Variables|Default|GetCurrentHealth) DamageValue)))
  (if (<= _output_get 0.0)
    (CallFunction|Die Instigator)
    (return (+ _output_get DamageValue) true)
    (else
      (return DamageValue false))))