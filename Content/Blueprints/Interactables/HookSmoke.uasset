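; HookSmoke is a timed smoke actor, represented by a Sphere component that expands outward and then disappears.
; BeginPlay collapses the sphere to zero scale, then starts parallel delays to snap it to FullScale after SpreadingDuration and destroy the actor after Duration.
; Tick grows the sphere linearly using DeltaSeconds, clamping any overshoot back to FullScale on a following frame.
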(event EventBeginPlay
  (bind _fullscale (Variables|Default|GetFullScale))
  (Transformation|SetWorldScale3D (Variables|Default|GetSphere) "0, 0, 0")
  (Utilities|FlowControl|Sequence
    (:then_0
      (Utilities|FlowControl|Delay (Variables|Default|GetDuration))
      (Actor|DestroyActor))
    (:then_1
      (Utilities|FlowControl|Delay (Variables|Default|GetSpreadingDuration))
      (Transformation|SetWorldScale3D (Variables|Default|GetSphere) (Math|Vector|MakeVector _fullscale _fullscale _fullscale)))))

(event EventTick
  (params (DeltaSeconds :type Float%20%28single-precision%29))
  (bind _sphere (Variables|Default|GetSphere))
  (bind _fullscale (Variables|Default|GetFullScale))
  (bind _spreadingduration (Variables|Default|GetSpreadingDuration))
  (bind _fullscale_2 (Variables|Default|GetFullScale))
  (bind _fullscale_3 (Variables|Default|GetFullScale))
  (bind _sphere_2 (Variables|Default|GetSphere))
  (bind _returnvalue (Transformation|GetWorldScale _sphere))
  (bind _returnvalue_2 (/ _spreadingduration DeltaSeconds))
  (bind _returnvalue_3 (/ _fullscale_2 _returnvalue_2))
  (if (< (.x _returnvalue) _fullscale_3)
    (Transformation|SetWorldScale3D _sphere_2 (+ (Transformation|GetWorldScale _sphere_2) (Math|Vector|MakeVector _returnvalue_3 _returnvalue_3 _returnvalue_3)))
    (elif (> (.x _returnvalue) _fullscale_3)
      (Transformation|SetWorldScale3D (Variables|Default|GetSphere) (Math|Vector|MakeVector _fullscale _fullscale _fullscale)))))

(fn ConstructionScript)