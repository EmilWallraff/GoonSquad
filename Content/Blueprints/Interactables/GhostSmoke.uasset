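; GhostSmoke is a temporary smoke actor that spreads along its Z axis, then destroys itself after Duration.
; BeginPlay flattens the Smoke component to zero Z scale, and Tick grows it linearly toward FullScale over SpreadingDuration.
; A parallel delay snaps it to full Z scale when spreading ends.
; The overshoot clamp in Tick sets all three axes to FullScale, unlike that snap, which keeps X and Y at one.
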(event EventBeginPlay
  (Transformation|SetWorldScale3D (Variables|Default|GetSmoke) "1.000000,1.000000, 0")
  (Utilities|FlowControl|Sequence
    (:then_0
      (Utilities|FlowControl|Delay (Variables|Default|GetDuration))
      (Actor|DestroyActor))
    (:then_1
      (Utilities|FlowControl|Delay (Variables|Default|GetSpreadingDuration))
      (Transformation|SetWorldScale3D (Variables|Default|GetSmoke) (Math|Vector|MakeVector 1.0 1.0 (Variables|Default|GetFullScale))))))

(event EventTick
  (params (DeltaSeconds :type Float%20%28single-precision%29))
  (bind _smoke (Variables|Default|GetSmoke))
  (bind _fullscale (Variables|Default|GetFullScale))
  (bind _fullscale_2 (Variables|Default|GetFullScale))
  (bind _smoke_2 (Variables|Default|GetSmoke))
  (bind _returnvalue (Transformation|GetWorldScale _smoke))
  (if (< (.z _returnvalue) _fullscale_2)
    (Transformation|SetWorldScale3D _smoke_2 (+ (Transformation|GetWorldScale _smoke_2) (Math|Vector|MakeVector 0.0 0.0 (/ (Variables|Default|GetFullScale) (/ (Variables|Default|GetSpreadingDuration) DeltaSeconds)))))
    (elif (> (.z _returnvalue) _fullscale_2)
      (Transformation|SetWorldScale3D (Variables|Default|GetSmoke) (Math|Vector|MakeVector _fullscale _fullscale _fullscale)))))

(fn ConstructionScript)