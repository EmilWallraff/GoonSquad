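; Captain Confidence's thrown teleporter projectile, which teleports its owning character to where it lands once a valid target is within range.
; After the projectile stops, a delay expands its range sphere from zero, and overlaps track characters inside.
; Tick checks those characters and, on a valid target, calls server events to teleport the owner, knock valid targets away and upward, and play a sound.
; The throwable destroys itself shortly afterward.
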(event OnProjectileStop(ProjectileMovement)
  (params (ImpactResult :type Hit%20Result%20Structure%20%28by%20ref%29))
  (Utilities|FlowControl|Delay (Variables|Default|GetActivationDuration))
  (Components|Sphere|SetSphereRadius (Variables|Default|GetRangeCollider) (Variables|Default|GetRange) true))

(event OnComponentBeginOverlap(RangeCollider)
  (params (OverlappedComponent :type Primitive%20Component%20Object%20Reference) (OtherActor :type Actor%20Object%20Reference) (OtherComp :type Primitive%20Component%20Object%20Reference) (OtherBodyIndex :type Integer) (bFromSweep :type Boolean) (SweepResult :type Hit%20Result%20Structure%20%28by%20ref%29))
  (bind _asbase_character_bp (Utilities|Casting|CastToBaseCharacter_BP OtherActor))
  (Utilities|Array|AddUnique (Variables|Default|GetPlayersInRange) _asbase_character_bp))

(event OnComponentEndOverlap(RangeCollider)
  (params (OverlappedComponent :type Primitive%20Component%20Object%20Reference) (OtherActor :type Actor%20Object%20Reference) (OtherComp :type Primitive%20Component%20Object%20Reference) (OtherBodyIndex :type Integer))
  (bind _asbase_character_bp (Utilities|Casting|CastToBaseCharacter_BP OtherActor))
  (Utilities|Array|RemoveItem (Variables|Default|GetPlayersInRange) _asbase_character_bp))

(event Custom|Server_ActivateTeleporter
  (bind _box (Variables|Default|GetBox))
  (bind _returnvalue (Transformation|GetWorldTransform _box))
  (Transformation|Teleport (Variables|Default|GetOwningCharacter) (+ (.location _returnvalue) "0,0,80.000000") (.rotation _returnvalue))
  (for _array_element (Variables|Default|GetPlayersInRange)
    (bind _istarget (CallFunction|IsValidTarget _array_element))
    (if _istarget
      (Character|LaunchCharacter _array_element (Math|Vector|MakeVector (* (.x (Math|Vector|Normalize (- (Transformation|GetWorldLocation (Variables|/Game/Blueprints/Player/BaseCharacter_BP.BaseCharacter_BP_C|GetCamera _array_element)) (Transformation|GetWorldLocation (Variables|Default|GetBox))))) 5e+02) (* (.y (Math|Vector|Normalize (- (Transformation|GetWorldLocation (Variables|/Game/Blueprints/Player/BaseCharacter_BP.BaseCharacter_BP_C|GetCamera _array_element)) (Transformation|GetWorldLocation (Variables|Default|GetBox))))) 5e+02) 3e+02) true true))))

(event EventBeginPlay
  (|CallParentFunction)
  (Components|Sphere|SetSphereRadius (Variables|Default|GetRangeCollider) 0.0 true))

(event EventTick
  (params (DeltaSeconds :type Float%20%28single-precision%29))
  (for _array_element (Variables|Default|GetPlayersInRange)
    (bind _istarget (CallFunction|IsValidTarget _array_element))
    (if _istarget
      (CallFunction|ServerActivateTeleporter)
      (CallFunction|ServerPlayReplicatedSound (Variables|Default|GetActivationSound) (Transformation|GetWorldLocation (Variables|Default|GetBox)))
      (Utilities|FlowControl|Delay 0.5)
      (CallFunction|DestroyThrowable))))

(fn ConstructionScript
  (|CallParentFunction))