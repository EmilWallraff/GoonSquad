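; Base throwable projectile Blueprint that launches along its Direction at the movement component's initial speed.
; A server-to-multicast event pair replicates sounds played at a location.
; Target validation rejects teammates and requires a line trace from the Box to the other character's camera to hit that character.
; DestroyThrowable destroys the actor and tells its owning ability to forget it.
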(event Custom|Server_PlayReplicatedSound
  (params (Sound :type Sound%20Cue%20Object%20Reference) (Location :type Vector))
  (CallFunction|MulticastPlayReplicatedSound Sound Location))

(event Custom|Multicast_PlayReplicatedSound
  (params (Sound :type Sound%20Cue%20Object%20Reference) (Location :type Vector))
  (Audio|PlaySoundatLocation Sound Location "0, 0, 0" 1.0 1.0 0.0 0 0 0 0))

(event EventBeginPlay
  (bind _projectilemovement (Variables|Components|GetProjectileMovement))
  (Variables|/Script/Engine.MovementComponent|SetVelocity _projectilemovement (* (Variables|Default|GetDirection) (Variables|/Script/Engine.ProjectileMovementComponent|GetInitialSpeed (Variables|Components|GetProjectileMovement))))
  (Components|Activation|Activate _projectilemovement false))

(fn ConstructionScript)

(fn DestroyThrowable
  (Actor|DestroyActor)
  (Default|ForgetObject (Variables|Components|GetOwningAbility) self))

(fn IsValidTarget
  (params (OtherCharacter :type Base%20Character%20BP%20Object%20Reference))
  (bind _sameteam (Default|CheckifonSameTeam OtherCharacter (Variables|Default|GetOwningCharacter)))
  (if _sameteam
    (return false)
    (else
      (bind _outhit (Collision|LineTraceByChannel (Transformation|GetWorldLocation (Variables|Components|GetBox)) (.location (Transformation|GetWorldTransform (Variables|/Game/Blueprints/Player/BaseCharacter_BP.BaseCharacter_BP_C|GetCamera OtherCharacter))) "TraceTypeQuery2" false 0 "None"))
      (if (== OtherCharacter (.HitActor (Collision|BreakHitResult _outhit)))
        (return true)
        (else
          (return false))))))