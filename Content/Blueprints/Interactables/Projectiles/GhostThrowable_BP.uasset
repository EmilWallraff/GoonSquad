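; Base ghost throwable projectile that becomes ready for activation once it stops moving, with an empty Activate function.
; On stop, it sets a ready flag via a server event and shows an activation icon, directly if the owning character is locally controlled, otherwise via a client event.
; The icon is a prompt widget that takes the owning ability's display icon and changes background opacity on Select and Deselect.
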(event OnProjectileStop(ProjectileMovement)
  (params (ImpactResult :type Hit%20Result%20Structure%20%28by%20ref%29))
  (CallFunction|ServerSetReadyforActivation true)
  (CallFunction|ShowActivationIcon))

(event Custom|Client_SetActivationIconVisibility
  (params (New%20Visibility :type Boolean))
  (Rendering|SetVisibility (Variables|Default|GetActivationIcon) New%20Visibility false))

(event Custom|Server_SetReadyForActivation
  (params (ReadyForActivation :type Boolean))
  (Variables|Default|SetReadyForActivation ReadyForActivation))

(event EventBeginPlay
  (|CallParentFunction)
  (bind _asghost_interaction_prompt_wbp (Utilities|Casting|CastToGhostInteractionPrompt_WBP (UserInterface|GetUserWidgetObject (Variables|Default|GetActivationIcon))))
  (Default|SetIconImage _asghost_interaction_prompt_wbp (Variables|/Game/Blueprints/Abilities/BaseAbility.BaseAbility_C|GetDisplayIcon (Variables|Default|GetOwningAbility))))

(fn ConstructionScript
  (|CallParentFunction))

(fn ShowActivationIcon
  (bind _activationicon (Variables|Default|GetActivationIcon))
  (if (Pawn|IsLocallyControlled (Variables|Default|GetOwningCharacter))
    (Class|ActorComponent|SetIsReplicated _activationicon false)
    (Rendering|SetVisibility _activationicon true false)
    (else
      (CallFunction|ClientSetActivationIconVisibility true))))

(fn HideActivationIcon
  (bind _activationicon (Variables|Default|GetActivationIcon))
  (if (Pawn|IsLocallyControlled (Variables|Default|GetOwningCharacter))
    (Class|ActorComponent|SetIsReplicated _activationicon false)
    (Rendering|SetVisibility _activationicon false false)
    (else
      (CallFunction|ClientSetActivationIconVisibility false))))

(fn Activate)

(fn Select
  (bind _asghost_interaction_prompt_wbp (Utilities|Casting|CastToGhostInteractionPrompt_WBP (UserInterface|GetUserWidgetObject (Variables|Default|GetActivationIcon))))
  (Default|SetBackgroundOpacity _asghost_interaction_prompt_wbp 0.8))

(fn Deselect
  (bind _asghost_interaction_prompt_wbp (Utilities|Casting|CastToGhostInteractionPrompt_WBP (UserInterface|GetUserWidgetObject (Variables|Default|GetActivationIcon))))
  (Default|SetBackgroundOpacity _asghost_interaction_prompt_wbp 0.3))