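; Thrown teleporter projectile for the ghost teleport ability that, once ready, teleports the owning character to just above itself.
; On landing it shows its activation icon and the owner's range decal, then notifies the ability, as it does when the owner enters or leaves TeleportationRange.
; Prepare and unprepare functions set server-side readiness and, along with deselection, adjust prompt opacity.
; Activation teleports through a server event, then has the ability destroy the teleporters.
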(event OnProjectileStop(ProjectileMovement)
  (params (ImpactResult :type Hit%20Result%20Structure%20%28by%20ref%29))
  (bind _decal (Variables|Default|GetDecal))
  (CallFunction|ShowActivationIcon)
  (Default|UpdateTeleporterPreperation (Variables|Default|GetOwningGhostTeleporterAbility))
  (if (Pawn|IsLocallyControlled (Variables|Default|GetOwningCharacter))
    (Class|ActorComponent|SetIsReplicated _decal false)
    (Rendering|SetVisibility _decal true false)
    (else
      (CallFunction|ClientSetDecalVisibility true))))

(event OnComponentBeginOverlap(TeleportationRange)
  (params (OverlappedComponent :type Primitive%20Component%20Object%20Reference) (OtherActor :type Actor%20Object%20Reference) (OtherComp :type Primitive%20Component%20Object%20Reference) (OtherBodyIndex :type Integer) (bFromSweep :type Boolean) (SweepResult :type Hit%20Result%20Structure%20%28by%20ref%29))
  (if (== OtherActor (Variables|Default|GetOwningCharacter))
    (Variables|Default|SetPlayerInside true)
    (Default|UpdateTeleporterPreperation (Variables|Default|GetOwningGhostTeleporterAbility))))

(event OnComponentEndOverlap(TeleportationRange)
  (params (OverlappedComponent :type Primitive%20Component%20Object%20Reference) (OtherActor :type Actor%20Object%20Reference) (OtherComp :type Primitive%20Component%20Object%20Reference) (OtherBodyIndex :type Integer))
  (if (== OtherActor (Variables|Default|GetOwningCharacter))
    (Variables|Default|SetPlayerInside false)
    (Default|UpdateTeleporterPreperation (Variables|Default|GetOwningGhostTeleporterAbility))))

(event Custom|Server_TeleportPlayer
  (bind _box (Variables|Default|GetBox))
  (bind _returnvalue (Transformation|GetWorldTransform _box))
  (Transformation|Teleport (Variables|Default|GetOwningCharacter) (+ (.location _returnvalue) "0,0,80.000000") (.rotation _returnvalue))
  (Default|DestroyTeleporters (Variables|Default|GetOwningGhostTeleporterAbility)))

(event Custom|Client_SetDecalVisibility
  (params (New%20Visibility :type Boolean))
  (Rendering|SetVisibility (Variables|Default|GetDecal) New%20Visibility false))

(event EventBeginPlay
  (|CallParentFunction)
  (bind _asghost_teleport_ability_bp (Utilities|Casting|CastToGhostTeleportAbility_BP (Variables|Default|GetOwningAbility)))
  (Variables|Default|SetOwningGhostTeleporterAbility _asghost_teleport_ability_bp))

(fn ConstructionScript
  (|CallParentFunction))

(fn PrepareTeleporter
  (CallFunction|ServerSetReadyforActivation true)
  (bind _asghost_interaction_prompt_wbp (Utilities|Casting|CastToGhostInteractionPrompt_WBP (UserInterface|GetUserWidgetObject (Variables|Default|GetActivationIcon))))
  (if (Variables|Default|GetSelected)
    (Default|SetBackgroundOpacity _asghost_interaction_prompt_wbp 0.3)
    (else
      (Default|SetBackgroundOpacity _asghost_interaction_prompt_wbp 0.8))))

(fn UnprepareTeleporter
  (CallFunction|ServerSetReadyforActivation false)
  (bind _asghost_interaction_prompt_wbp (Utilities|Casting|CastToGhostInteractionPrompt_WBP (UserInterface|GetUserWidgetObject (Variables|Default|GetActivationIcon))))
  (Default|SetBackgroundOpacity _asghost_interaction_prompt_wbp 0.05))

(fn Activate
  (if (Variables|Default|GetReadyForActivation)
    (|CallParentFunction)
    (CallFunction|ServerTeleportPlayer)))

(fn Deselect
  (Variables|Default|SetSelected false)
  (bind _asghost_interaction_prompt_wbp (Utilities|Casting|CastToGhostInteractionPrompt_WBP (UserInterface|GetUserWidgetObject (Variables|Default|GetActivationIcon))))
  (if (Variables|Default|GetReadyForActivation)
    (Default|SetBackgroundOpacity _asghost_interaction_prompt_wbp 0.3)
    (else
      (Default|SetBackgroundOpacity _asghost_interaction_prompt_wbp 0.05))))

(fn Select
  (Variables|Default|SetSelected true)
  (|CallParentFunction))