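; HookMolotov is a timed area hazard that sets enemy characters inside it on fire, then destroys itself after its Duration.
; Sphere overlaps track characters on a different team from the owning character, with the team check made on authority.
; Every tick, a server event reapplies a status effect for the burning duration to each tracked character, crediting the owner's controller.
; The GenerateEffects hook called on BeginPlay is empty here.
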(event OnComponentBeginOverlap(Sphere)
  (params (OverlappedComponent :type Primitive%20Component%20Object%20Reference) (OtherActor :type Actor%20Object%20Reference) (OtherComp :type Primitive%20Component%20Object%20Reference) (OtherBodyIndex :type Integer) (bFromSweep :type Boolean) (SweepResult :type Hit%20Result%20Structure%20%28by%20ref%29))
  (bind _asbase_character_bp (Utilities|Casting|CastToBaseCharacter_BP OtherActor))
  (bind _isenemy (CallFunction|CheckifEnemy _asbase_character_bp))
  (if _isenemy
    (Utilities|Array|Add (Variables|Default|GetPlayersInside) _asbase_character_bp)))

(event OnComponentEndOverlap(Sphere)
  (params (OverlappedComponent :type Primitive%20Component%20Object%20Reference) (OtherActor :type Actor%20Object%20Reference) (OtherComp :type Primitive%20Component%20Object%20Reference) (OtherBodyIndex :type Integer))
  (bind _asbase_character_bp (Utilities|Casting|CastToBaseCharacter_BP OtherActor))
  (Utilities|Array|RemoveItem (Variables|Default|GetPlayersInside) _asbase_character_bp))

(event Custom|Server_IgnitePlayersInside
  (for _array_element (Variables|Default|GetPlayersInside)
    (Utilities|IsValid _array_element
      (:Is%20Valid
        (Default|InflictStatusEffect _array_element "NewEnumerator2" (Variables|Default|GetBurningDuration) (Utilities|Struct|MakeDamageInstigator false (Default|GetPlayerControllerReference (Variables|Default|GetOwningCharacter))))))))

(event EventBeginPlay
  (CallFunction|GenerateEffects)
  (Utilities|FlowControl|Delay (Variables|Default|GetDuration))
  (Actor|DestroyActor))

(event EventTick
  (params (DeltaSeconds :type Float%20%28single-precision%29))
  (CallFunction|ServerIgnitePlayersInside))

(fn ConstructionScript)

(fn GenerateEffects)

(fn CheckifEnemy
  (params (BaseCharacter :type Base%20Character%20BP%20Object%20Reference))
  (Networking|SwitchHasAuthority
    (:Authority
      (bind _team (Default|GetPlayerTeam (Variables|/Game/Blueprints/Player/BaseCharacter_BP.BaseCharacter_BP_C|GetPlayerStateReference BaseCharacter)))
      (bind _team_2 (Default|GetPlayerTeam (Variables|/Game/Blueprints/Player/BaseCharacter_BP.BaseCharacter_BP_C|GetPlayerStateReference (Variables|Default|GetOwningCharacter))))
      (return (!= _team _team_2)))))