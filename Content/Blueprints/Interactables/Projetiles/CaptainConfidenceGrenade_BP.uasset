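; Captain Confidence's grenade, a projectile that inflicts a timed status effect (apparently "Watched") on nearby enemy characters when it stops.
; A range sphere tracks overlapping characters, and on detonation the server applies the effect to valid targets and plays a replicated sound.
; The target check excludes teammates and requires a line-of-sight trace to the character's camera.
; A multicast reveals the blast sphere before the grenade is destroyed after a short delay.
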(event OnProjectileStop(ProjectileMovement)
  (params (ImpactResult :type Hit%20Result%20Structure%20%28by%20ref%29))
  (CallFunction|ServerExplode)
  (Utilities|FlowControl|Delay 0.5)
  (CallFunction|DestroyThrowable))

(event OnComponentBeginOverlap(RangeCollider)
  (params (OverlappedComponent :type Primitive%20Component%20Object%20Reference) (OtherActor :type Actor%20Object%20Reference) (OtherComp :type Primitive%20Component%20Object%20Reference) (OtherBodyIndex :type Integer) (bFromSweep :type Boolean) (SweepResult :type Hit%20Result%20Structure%20%28by%20ref%29))
  (bind _asbase_character_bp (Utilities|Casting|CastToBaseCharacter_BP OtherActor))
  (Utilities|Array|AddUnique (Variables|Default|GetPlayersInRange) _asbase_character_bp))

(event OnComponentEndOverlap(RangeCollider)
  (params (OverlappedComponent :type Primitive%20Component%20Object%20Reference) (OtherActor :type Actor%20Object%20Reference) (OtherComp :type Primitive%20Component%20Object%20Reference) (OtherBodyIndex :type Integer))
  (bind _asbase_character_bp (Utilities|Casting|CastToBaseCharacter_BP OtherActor))
  (Utilities|Array|RemoveItem (Variables|Default|GetPlayersInRange) _asbase_character_bp))

(event Custom|Server_Explode
  (for _array_element (Variables|Default|GetPlayersInRange)
    (Utilities|IsValid _array_element
      (:Is%20Valid
        (bind _istarget (CallFunction|IsValidTarget _array_element))
        (if _istarget
          (Default|InflictStatusEffect _array_element "NewEnumerator3" (Variables|Default|GetWatchedDuration) (Utilities|Struct|MakeDamageInstigator false (Variables|/Game/Blueprints/Player/BaseCharacter_BP.BaseCharacter_BP_C|GetPlayerControllerReference (Variables|Default|GetOwningCharacter))))))))
  (CallFunction|ServerPlayReplicatedSound (Variables|Default|GetDetonationSound) (Transformation|GetWorldLocation (Variables|Default|GetBox)))
  (CallFunction|MulticastShowEffects))

(event Custom|Multicast_ShowEffects
  (Rendering|SetVisibility (Variables|Default|GetSphere) true false))

(event EventBeginPlay
  (|CallParentFunction)
  (Components|Sphere|SetSphereRadius (Variables|Default|GetRangeCollider) (Variables|Default|GetRange) true)
  (Rendering|SetVisibility (Variables|Default|GetSphere) false false))

(event EventTick
  (params (DeltaSeconds :type Float%20%28single-precision%29)))

(fn ConstructionScript
  (|CallParentFunction))

(fn CheckifTarget
  (params (OtherChracter :type Base%20Character%20BP%20Object%20Reference))
  (bind _sameteam (Default|CheckifonSameTeam OtherChracter (Variables|Default|GetOwningCharacter)))
  (if _sameteam
    (return false)
    (else
      (bind _outhit (Collision|LineTraceByChannel (Transformation|GetWorldLocation (Variables|Default|GetBox)) (.location (Transformation|GetWorldTransform (Variables|/Game/Blueprints/Player/BaseCharacter_BP.BaseCharacter_BP_C|GetCamera OtherChracter))) "TraceTypeQuery2" false 0 "None"))
      (if (== OtherChracter (.HitActor (Collision|BreakHitResult _outhit)))
        (return true)
        (else
          (return false))))))