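; GhostFakeThrowable_BP is a throwable projectile that deploys a GhostFake_BP actor when activated.
; Its Activate override calls the parent, then a server spawn event that creates the fake at the Box component's location and rotation.
; The owning character is passed as owner, instigator and PlayerCharacter, and the throwable destroys itself after spawning.
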(event Custom|Server_SpawnFake
  (bind _owningcharacter (Variables|Default|GetOwningCharacter))
  (bind _box (Variables|Default|GetBox))
  (Game|SpawnActorfromClass "/Game/Blueprints/Interactables/GhostFake_BP.GhostFake_BP_C" (Math|Transform|MakeTransform (Transformation|GetWorldLocation _box) (Transformation|GetWorldRotation _box) "1.000000,1.000000,1.000000") "Undefined" _owningcharacter _owningcharacter _owningcharacter)
  (CallFunction|DestroyThrowable))

(event EventBeginPlay
  (|CallParentFunction) ; This node is disabled and will not be called.\nDrag off pins to build functionality.
)

(event Collision|EventActorBeginOverlap
  (params (OtherActor :type Actor%20Object%20Reference)))

(event EventTick
  (params (DeltaSeconds :type Float%20%28single-precision%29)))

(fn ConstructionScript
  (|CallParentFunction))

(fn Activate
  (|CallParentFunction)
  (CallFunction|ServerSpawnFake))